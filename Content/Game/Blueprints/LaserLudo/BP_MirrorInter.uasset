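; BP_MirrorInter is a mirror pillar in LaserLudo that a Cidara player or a Spectre can focus on.
; Overlapping ZoneProximite registers it as that character's focused mirror; leaving clears the reference only if it still points to this mirror.
; SetFocus and SetEndFocus both write IsFocused and toggle OutlinePilier visibility with opposite polarity.
; Neither is called here, and the mirror contains no rotation or laser logic.
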(event OnComponentBeginOverlap(ZoneProximite)
  (params (OverlappedComponent :type Primitive%20Component%20Object%20Reference) (OtherActor :type Actor%20Object%20Reference) (OtherComp :type Primitive%20Component%20Object%20Reference) (OtherBodyIndex :type Integer) (bFromSweep :type Boolean) (SweepResult :type Hit%20Result%20Structure%20%28by%20ref%29))
  (bind _asbp_player_cidara (Utilities|Casting|CastToBP_PlayerCidara OtherActor)
    (:then
      (Variables|/Game/Game/Blueprints/Characters/Cidara/BP_PlayerCidara.BP_PlayerCidara_C|SetMiroirFocusCidara _asbp_player_cidara self))
    (:CastFailed
      (bind _asbp_spectre (Utilities|Casting|CastToBP_Spectre OtherActor))
      (Variables|/Game/Game/Blueprints/Characters/Spectre/BP_Spectre.BP_Spectre_C|SetMiroirFocusSpectrre _asbp_spectre self))))

(event OnComponentEndOverlap(ZoneProximite)
  (params (OverlappedComponent :type Primitive%20Component%20Object%20Reference) (OtherActor :type Actor%20Object%20Reference) (OtherComp :type Primitive%20Component%20Object%20Reference) (OtherBodyIndex :type Integer))
  (bind _asbp_player_cidara (Utilities|Casting|CastToBP_PlayerCidara OtherActor)
    (:then
      (if (== (Variables|/Game/Game/Blueprints/Characters/Cidara/BP_PlayerCidara.BP_PlayerCidara_C|GetMiroirFocusCidara _asbp_player_cidara) self)
        (Variables|/Game/Game/Blueprints/Characters/Cidara/BP_PlayerCidara.BP_PlayerCidara_C|SetMiroirFocusCidara _asbp_player_cidara 0)))
    (:CastFailed
      (bind _asbp_spectre (Utilities|Casting|CastToBP_Spectre OtherActor))
      (if (== (Variables|/Game/Game/Blueprints/Characters/Spectre/BP_Spectre.BP_Spectre_C|GetMiroirFocusSpectrre _asbp_spectre) self)
        (Variables|/Game/Game/Blueprints/Characters/Spectre/BP_Spectre.BP_Spectre_C|SetMiroirFocusSpectrre _asbp_spectre 0)))))

(event EventBeginPlay
  (|CallParentFunction) ; This node is disabled and will not be called.\nDrag off pins to build functionality.
)

(event Collision|EventActorBeginOverlap
  (params (OtherActor :type Actor%20Object%20Reference)))

(event EventTick
  (params (DeltaSeconds :type Float%20%28single-precision%29)))

(event EventSetFocus
  (params (Focused :type Boolean) (Investigator :type Actor%20Object%20Reference))
  (bind _output_get (Variables|Default|SetIsFocused Focused))
  (if _output_get
    (Rendering|SetVisibility (Variables|Default|GetOutlinePilier) true false)
    (else
      (Rendering|SetVisibility (Variables|Default|GetOutlinePilier) false false))))

(event EventSetEndFocus
  (params (EndFocus :type Boolean))
  (bind _output_get (Variables|Default|SetIsFocused EndFocus))
  (if _output_get
    (Rendering|SetVisibility (Variables|Default|GetOutlinePilier) false false)
    (else
      (Rendering|SetVisibility (Variables|Default|GetOutlinePilier) true false))))

(fn ConstructionScript
  (|CallParentFunction))