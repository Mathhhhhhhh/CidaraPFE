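; BP_LaserReceiver is the receiver for a laser puzzle, reacting when laser contact is received or lost.
; Each received event increments a counter, which a lost event resets to zero.
; Once the counter reaches ten, it only prints a debug message.
; Calls to open the laser door and advance the laser manager to the next room exist but are disconnected, so they never run.
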(event Custom|OnLaserReceived
  (bind _output_get (Variables|Default|SetTimeFake (+ (Variables|Default|GetTimeFake) 1)))
  (if (>= _output_get 10)
    (Development|PrintString "je capte")))

(event Custom|OnLaserLost
  (Variables|Default|SetTimeFake 0))

(event EventBeginPlay)

(event EventTick
  (params (DeltaSeconds :type Float%20%28single-precision%29)))

(fn ConstructionScript)