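; BP_MirrorBig is a large rotatable mirror element in the LaserLudo folder, turned in 45-degree yaw steps.
; Each TurnMirrorBig call increments a counter, and reaching the Seuil threshold resets it and triggers a turn.
; A timeline lerps the Pilier component's relative rotation, with a sound at the start.
; A Rotating flag blocks overlapping turns, though the counter still resets when a turn is blocked.
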(event OnComponentBeginOverlap(CapteurTest)
  (params (OverlappedComponent :type Primitive%20Component%20Object%20Reference) (OtherActor :type Actor%20Object%20Reference) (OtherComp :type Primitive%20Component%20Object%20Reference) (OtherBodyIndex :type Integer) (bFromSweep :type Boolean) (SweepResult :type Hit%20Result%20Structure%20%28by%20ref%29)))

(event Custom|TurnMirrorBig
  (bind _pilier (Variables|Default|GetPilier))
  (bind _relativerotation (Variables|/Script/Engine.SceneComponent|GetRelativeRotation _pilier))
  (bind (_roll _pitch _yaw) (Math|Rotator|BreakRotator _relativerotation))
  (bind _output_get (Variables|Default|SetInteractNumber (+ (Variables|Default|GetInteractNumber) 1)))
  (if (== _output_get (Variables|Default|GetSeuil))
    (Variables|Default|SetInteractNumber 0)
    ;[0.15 0.15 0.15 0.5] Est ce qu il est deja en train de rotate
    (if (not (Variables|Default|GetbRotating))
      (Variables|Default|SetbRotating true)
      (Variables|Default|SetStartRotation _relativerotation)
      (Variables|Default|SetTargetRotation (Math|Rotator|MakeRotator _roll _pitch (+ _yaw 45.0)))
      (Audio|PlaySoundatLocation "/Game/Game/Sounds/Lasers/SC_Rotation.SC_Rotation" (Transformation|GetActorLocation) "0, 0, 0" 1.0 1.0 0.0 0 0 0 0)
      (bind _alpha (Timeline|Timeline_0 PlayFromStart)
        (:Update
          (Transformation|SetRelativeRotation (Variables|Default|GetPilier) (Math|Rotator|Lerp(Rotator) (Variables|Default|GetStartRotation) (Variables|Default|GetTargetRotation) _alpha) false true))
        (:Finished
          (Variables|Default|SetbRotating false))))))

(event EventBeginPlay
  (|CallParentFunction))

(event Collision|EventActorBeginOverlap
  (params (OtherActor :type Actor%20Object%20Reference)))

(event EventTick
  (params (DeltaSeconds :type Float%20%28single-precision%29)))

(fn ConstructionScript
  (|CallParentFunction))