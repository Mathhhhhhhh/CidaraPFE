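; Laser emitter for a mirror puzzle that casts a bouncing beam to laser receivers.
; While active, a looping timer recursively line-traces, deriving each bounce from the mirror's own orientation and trace channel, up to MaxBounces.
; Segments reuse skin-specific Niagara beams, deactivating extras.
; Hit receivers learn whether a big mirror was involved; UpdateReceiver compares the active list to itself, so OnLaserLost never fires.
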(event Custom|LaserUpdate
  (bind _directionvector (Variables|Default|GetDirectionVector))
  (if (Variables|Default|GetbLaserActive)
    (Utilities|Array|Clear (Variables|Default|GetHitReceiverActifs))
    (bind _segmentindex (CallFunction|TracerLaser (Transformation|GetWorldLocation _directionvector) (Math|Vector|GetForwardVector _directionvector) 0 0 "TraceTypeQuery1" false))
    (bind _output_get (Variables|Default|SetSegment%20Index _segmentindex))
    (CallFunction|CleanBeam _output_get)
    (CallFunction|UpdateReceiver)))

(event EventBeginPlay
  (Utilities|Time|SetTimerbyEvent (delegate Custom|LaserUpdate) 0.01 true))

(fn ConstructionScript)

(fn TracerLaser
  (params (StartPos :type Vector) (Direction :type Vector) (BounceCount :type Integer) (ActorsToIgnore :type Array%20of%20Actor%20Object%20References) (TraceChannelType :type ETraceTypeQuery%20Enum :default "TraceTypeQuery1") (BigMirrorWasHit :type Boolean))
  (Variables|Default|SetActors%20to%20Ignore ActorsToIgnore)
  (bind _output_get (LocalVariables|SetBounce%20Count BounceCount))
  (bind _output_get_2 (LocalVariables|SetDirect Direction))
  (bind _output_get_3 (LocalVariables|SetStartPosition StartPos))
  (bind _output_get_4 (LocalVariables|SetEndCalcul (+ _output_get_3 (* _output_get_2 (Variables|Default|GetLaserLenght)))))
  (if (>= _output_get (Variables|Default|GetMaxBounces))
    (return (LocalVariables|GetBounce%20Count) BigMirrorWasHit)
    (else
      (bind (_outhit _returnvalue) (Collision|LineTraceByChannel _output_get_3 _output_get_4 TraceChannelType false (Variables|Default|GetActors%20to%20Ignore) "ForDuration" true "(R=1.000000,G=0.000000,B=0.000000,A=1.000000)" "(R=0.000000,G=1.000000,B=0.000000,A=1.000000)" 1.0))
      (LocalVariables|SetImpactNormal (.ImpactNormal (Collision|BreakHitResult _outhit)))
      (LocalVariables|SetImpactPoint (.ImpactPoint (Collision|BreakHitResult _outhit)))
      (LocalVariables|SetHitActor (.HitActor (Collision|BreakHitResult _outhit)))
      (if _returnvalue
        (CallFunction|BeamSegment (LocalVariables|GetStartPosition) (LocalVariables|GetImpactPoint) (LocalVariables|GetBounce%20Count))
        (bind _asbp_laser_receiver (Utilities|Casting|CastToBP_LaserReceiver (LocalVariables|GetHitActor))
          (:then
            (Utilities|Array|Add (Variables|Default|GetHitReceiverActifs) _asbp_laser_receiver)
            (Default|OnLaserReceived _asbp_laser_receiver self BigMirrorWasHit)
            (return (LocalVariables|GetBounce%20Count) BigMirrorWasHit))
          (:CastFailed
            (bind _asbp_mirror (Utilities|Casting|CastToBP_Mirror (LocalVariables|GetHitActor))
              (:then
                (bind (_segmentindex _hashitbigmirror) (CallFunction|TracerLaser (+ (* (LocalVariables|GetImpactNormal) 1) (LocalVariables|GetImpactPoint)) (Math|Vector|GetReflectionVector (* (Math|Vector|GetForwardVector (Variables|/Game/Game/Blueprints/LaserLudo/Elements/BP_Mirror.BP_Mirror_C|GetDirectArrow _asbp_mirror)) -1.0) (Math|Vector|GetForwardVector (Variables|/Game/Game/Blueprints/LaserLudo/Elements/BP_Mirror.BP_Mirror_C|GetBox _asbp_mirror))) (+ (LocalVariables|GetBounce%20Count) 1) (Utilities|Array|MakeArray (LocalVariables|GetHitActor)) (Variables|/Game/Game/Blueprints/LaserLudo/Elements/BP_Mirror.BP_Mirror_C|GetTraceChannel _asbp_mirror) (or (== (Utilities|GetClass _asbp_mirror) "/Game/Game/Blueprints/LaserLudo/Elements/BP_MirrorBig.BP_MirrorBig_C") BigMirrorWasHit)))
                (return _segmentindex (or _hashitbigmirror BigMirrorWasHit)))
              (:CastFailed
                (return (LocalVariables|GetBounce%20Count) BigMirrorWasHit)))))
        (else
          (CallFunction|BeamSegment (LocalVariables|GetStartPosition) (LocalVariables|GetEndCalcul) (LocalVariables|GetBounce%20Count))
          (return (LocalVariables|GetBounce%20Count) BigMirrorWasHit))))))

(fn BeamSegment
  (params (Start :type Vector) (End :type Vector) (Index :type Integer))
  (bind _beamsystem (Variables|Default|GetBeamSystem))
  (bind _output (Utilities|Array|Get(acopy) _beamsystem Index))
  (Utilities|IsValid _output
    (:Is%20Valid
      (LocalVariables|SetNiagaraRef _output)
      (Niagara|SetNiagaraVariable(Vector3) (LocalVariables|GetNiagaraRef) "User.BeamStart" Start)
      (Niagara|SetNiagaraVariable(Vector3) (LocalVariables|GetNiagaraRef) "User.BeamEnd" End)
      (Components|Activation|Activate (LocalVariables|GetNiagaraRef) true))
    (:Is%20Not%20Valid
      (switch Utilities|FlowControl|Switch|SwitchonE_SkinLaser (Variables|Default|GetSkin)
        (:NewEnumerator0
          (Variables|Default|SetNiagaraSkin "/Game/Game/Blueprints/LaserLudo/NS_LaserBeam.NS_LaserBeam"))
        (:NewEnumerator1
          (Variables|Default|SetNiagaraSkin "/Game/Game/Blueprints/LaserLudo/NS_LaserBeamPurple.NS_LaserBeamPurple")))
      (bind _returnvalue (Niagara|SpawnSystematLocation (Variables|Default|GetNiagaraSkin) Start "0, 0, 0" "1.000000,1.000000,1.000000" false false))
      (bind _output_get (LocalVariables|SetNiagaraRef _returnvalue))
      (Utilities|Array|SetArrayElem (Variables|Default|GetBeamSystem) Index _output_get true)
      (Niagara|SetNiagaraVariable(Vector3) (LocalVariables|GetNiagaraRef) "User.BeamStart" Start)
      (Niagara|SetNiagaraVariable(Vector3) (LocalVariables|GetNiagaraRef) "User.BeamEnd" End)
      (Components|Activation|Activate (LocalVariables|GetNiagaraRef) true))))

(fn UpdateReceiver
  (for _array_element (Variables|Default|GetHitReceiverActifs)
    (if (not (Utilities|Array|ContainsItem (Variables|Default|GetHitReceiverActifs) _array_element))
      (bind _asbp_laser_receiver (Utilities|Casting|CastToBP_LaserReceiver _array_element))
      (Default|OnLaserLost _asbp_laser_receiver)))
  (Variables|Default|SetHitReceiverPrecedents (Variables|Default|GetHitReceiverActifs)))

(fn CleanBeam
  (params (LastIndex :type Integer))
  (for (_array_element _array_index) (Variables|Default|GetBeamSystem)
    (if (> _array_index LastIndex)
      (Components|Activation|Deactivate _array_element))))

(fn Activate
  (Variables|Default|SetbLaserActive true))

(fn Deactivate
  (Variables|Default|SetbLaserActive false)
  (CallFunction|CleanBeam -1)
  (CallFunction|UpdateReceiver))

(fn UpdateMirrorBig
  (for _array_element (Variables|Default|GetHitReceiverPrecedents)
    (if (not (Utilities|Array|ContainsItem (Variables|Default|GetHitReceiverActifs) _array_element))
      (Utilities|Casting|CastToBP_LaserReceiver _array_element)))
  (Variables|Default|SetHitReceiverPrecedents (Variables|Default|GetHitReceiverActifs)))