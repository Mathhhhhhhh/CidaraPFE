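; BP_LaserReceiver is a laser puzzle target that triggers an action once a beam has held on it.
; Repeated hit calls increment a counter, reset on laser loss; past a threshold, the receiver type decides the outcome.
; It activates linked emitters, opens a door and advances the laser manager's room, or validates Level 1 by emitter skin and big-mirror hit.
; The construction script sets the material from the receiver's skin.
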(event Custom|OnLaserReceived
  (params (EmitterInst :type BP%20Laser%20Emitter%20Object%20Reference) (HitBigMirror :type Boolean))
  (Variables|Default|SetEmitter%20Inst EmitterInst)
  (Variables|Default|SetHit%20Big%20Mirror HitBigMirror)
  (bind _output_get (Variables|Default|SetTimeFake (+ (Variables|Default|GetTimeFake) 1)))
  (if (>= _output_get 10)
    (switch Utilities|FlowControl|Switch|SwitchonE_Receiver (Variables|Default|GetE_ReceiverType)
      (:NewEnumerator0
        (for _array_element (Variables|Default|GetBP_Emitter)
          (Variables|/Game/Game/Blueprints/LaserLudo/Elements/BP_LaserEmitter.BP_LaserEmitter_C|SetbLaserActive _array_element true))
        (Utilities|FlowControl|DoOnce false
          (:Completed
            (Audio|PlaySoundatLocation "/Game/Game/Sounds/Lasers/LaserActivation.LaserActivation" (Transformation|GetActorLocation) "0, 0, 0" 1.0 1.0 0.0 0 0 0 0))))
      (:NewEnumerator1
        (if (and (Utilities|Enum|Equal(Enum) (Variables|/Game/Game/Blueprints/LaserLudo/Elements/BP_LaserEmitter.BP_LaserEmitter_C|GetSkin (Variables|Default|GetEmitter%20Inst)) (Variables|Default|GetE_SkinReceiver)) (Variables|Default|GetHit%20Big%20Mirror))
          (Utilities|FlowControl|DoOnce false
            (:Completed
              (Variables|Default|SetCompteur (+ (Variables|Default|GetCompteur) 1))
              (if (== (Variables|Default|GetCompteur) 2)
                (Audio|PlaySoundatLocation "/Game/StarterContent/Audio/Starter_Music_Cue.Starter_Music_Cue" (Transformation|GetActorLocation) "0, 0, 0" 1.0 1.0 0.0 0 0 0 0)
                (else
                  (Audio|PlaySoundatLocation "/Game/Game/Sounds/Lasers/LaserActivation.LaserActivation" (Transformation|GetActorLocation) "0, 0, 0" 1.0 1.0 0.0 0 0 0 0)))))
          (else
            (Development|PrintString "pqs win" true true "(R=0.640625,G=0.013394,B=0.000000,A=1.000000)"))))
      (:NewEnumerator2
        (Default|OpenDoor (Variables|Default|GetBP_DoorLaser))
        (Default|NextRoom (Variables|Default|GetBP_LaserManager))))))

(event Custom|OnLaserLost
  (Variables|Default|SetTimeFake 0))

(event EventBeginPlay)

(event EventTick
  (params (DeltaSeconds :type Float%20%28single-precision%29)))

(fn ConstructionScript
  (switch Utilities|FlowControl|Switch|SwitchonE_SkinLaser (Variables|Default|GetE_SkinReceiver)
    (:NewEnumerator0
      (Rendering|Material|SetMaterial (Variables|Default|GetReceiver) 0 "/Game/Game/Blueprints/LaserLudo/Mode/Material_002.Material_002"))
    (:NewEnumerator1
      (Rendering|Material|SetMaterial (Variables|Default|GetReceiver) 0 "/Game/Game/Blueprints/LaserLudo/Mode/Material_003.Material_003"))
    (:NewEnumerator2
      (Rendering|Material|SetMaterial (Variables|Default|GetReceiver) 0 "/Game/Game/Blueprints/LaserLudo/Mode/Cheval/Material_001.Material_001"))))