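; Mirror pillar actor for the laser puzzle, with its pillar material set by a Skin choice in the construction script.
; BeginPlay caches the player, then snaps to the first PointPosition and gathers all BP_MirrorBig actors if points exist.
; MoveMirror offsets the pillar by a fixed step along camera-yaw-relative axes.
; Interaction events are empty, handled in BP_MirrorInter; older point-to-point slide and 90-degree rotation timelines remain disconnected.
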(event Custom|OnLaserDetected
  ;[0 0 0 0.5] OFF, interractions in BP_MirrorInter
)

(event EventBeginPlay
  (bind _asbp_player_cidara (Utilities|Casting|CastToBP_PlayerCidara (Game|GetPlayerCharacter 0)))
  (Variables|Default|SetAs%20BP%20Player%20Cidara _asbp_player_cidara)
  (if (> (Utilities|Array|Length (Variables|DeplacementMiroir|GetPointPosition)) 0)
    (Variables|DeplacementMiroir|SetCurrentIndex 0)
    (Transformation|SetActorLocation (Utilities|Array|Get(acopy) (Variables|DeplacementMiroir|GetPointPosition)) false false)
    (bind _outactors (Actor|GetAllActorsOfClass "/Game/Game/Blueprints/LaserLudo/Elements/BP_MirrorBig.BP_MirrorBig_C"))
    (Variables|Default|SetBP_MirrorBig _outactors)))

(event EventInteract
  (params (Investigator :type Actor%20Object%20Reference))
  ;[0 0 0 0.5] OFF, interractions in BP_MirrorInter
)

(event EventLongPressed
  (params (Look%20Direction%20Player :type Vector :default "0, 0, 0") (Investigator :type Actor%20Object%20Reference))
  ;[0 0 0 0.5] OFF, interractions in BP_MirrorInter
)

(fn ConstructionScript
  (bind _pilier (Variables|Default|GetPilier))
  (switch Utilities|FlowControl|Switch|SwitchonE_SkinLaser (Variables|Default|GetSkin)
    (:NewEnumerator0
      (Rendering|Material|SetMaterial _pilier 0 "/Game/Game/Blueprints/LaserLudo/Mode/MM_PillarCidara.MM_PillarCidara"))
    (:NewEnumerator1
      (Rendering|Material|SetMaterial _pilier 0 "/Game/Game/Blueprints/LaserLudo/Mode/MM_PillarSpectre.MM_PillarSpectre"))
    (:NewEnumerator2
      (Rendering|Material|SetMaterial _pilier 0 "/Game/Game/Blueprints/LaserLudo/Mode/MM_PillarFixed.MM_PillarFixed"))))

(fn MoveMirror
  (params (Direction :type Vector%202D%20Structure))
  (bind _returnvalue (Game|GetPlayerController 0))
  (bind _returnvalue_2 (Pawn|GetControlRotation _returnvalue :!class /Script/Engine.Controller))
  (bind _yaw (Math|Rotator|BreakRotator _returnvalue_2))
  (bind _returnvalue_3 (Math|Rotator|MakeRotator 0.0 0.0 _yaw))
  (Transformation|SetActorLocation (+ (Transformation|GetActorLocation) (+ (* (* (Math|Float|Round (.x Direction)) (Math|Vector|GetRightVector _returnvalue_3)) (Variables|Default|GetDéplacementPilier)) (* (* (Math|Float|Round (.y Direction)) (Math|Vector|GetForwardVector _returnvalue_3)) (Variables|Default|GetDéplacementPilier)))) false false))