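; Interactive puzzle mirror that BP_PlayerCidara or BP_Spectre can rotate and push, driving linked BP_MirrorBig actors.
; Its proximity zone registers it as that character's focused mirror, and focus events toggle the pillar outline.
; Interact turns the focused pillar 90° by timeline, then turns big mirrors with matching tags; its distance check compares its own location to itself.
; Long press slides it to the preset point best aligned with the look direction.
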(event OnComponentBeginOverlap(ZoneProximite)
  (params (OverlappedComponent :type Primitive%20Component%20Object%20Reference) (OtherActor :type Actor%20Object%20Reference) (OtherComp :type Primitive%20Component%20Object%20Reference) (OtherBodyIndex :type Integer) (bFromSweep :type Boolean) (SweepResult :type Hit%20Result%20Structure%20%28by%20ref%29))
  ;[0.15 0.15 0.15 0.5] Outline
  (bind _asbp_player_cidara (Utilities|Casting|CastToBP_PlayerCidara OtherActor)
    (:then
      (Variables|/Game/Game/Blueprints/Characters/Cidara/BP_PlayerCidara.BP_PlayerCidara_C|SetMiroirFocusCidara _asbp_player_cidara self))
    (:CastFailed
      (bind _asbp_spectre (Utilities|Casting|CastToBP_Spectre OtherActor))
      (Variables|/Game/Game/Blueprints/Characters/Spectre/BP_Spectre.BP_Spectre_C|SetMiroirFocusSpectrre _asbp_spectre self))))

(event OnComponentEndOverlap(ZoneProximite)
  (params (OverlappedComponent :type Primitive%20Component%20Object%20Reference) (OtherActor :type Actor%20Object%20Reference) (OtherComp :type Primitive%20Component%20Object%20Reference) (OtherBodyIndex :type Integer))
  ;[0.15 0.15 0.15 0.5] Outline
  (bind _asbp_player_cidara (Utilities|Casting|CastToBP_PlayerCidara OtherActor)
    (:then
      (if (== (Variables|/Game/Game/Blueprints/Characters/Cidara/BP_PlayerCidara.BP_PlayerCidara_C|GetMiroirFocusCidara _asbp_player_cidara) self)
        (Variables|/Game/Game/Blueprints/Characters/Cidara/BP_PlayerCidara.BP_PlayerCidara_C|SetMiroirFocusCidara _asbp_player_cidara 0)))
    (:CastFailed
      (bind _asbp_spectre (Utilities|Casting|CastToBP_Spectre OtherActor))
      (if (== (Variables|/Game/Game/Blueprints/Characters/Spectre/BP_Spectre.BP_Spectre_C|GetMiroirFocusSpectrre _asbp_spectre) self)
        (Variables|/Game/Game/Blueprints/Characters/Spectre/BP_Spectre.BP_Spectre_C|SetMiroirFocusSpectrre _asbp_spectre 0)))))

(event EventBeginPlay
  (|CallParentFunction)
  (bind _outactors (Actor|GetAllActorsOfClass "/Game/Game/Blueprints/LaserLudo/Elements/BP_MirrorBig.BP_MirrorBig_C"))
  (Variables|Default|SetBP_MirrorBig_0 _outactors))

(event EventInteract
  (params (Investigator :type Actor%20Object%20Reference))
  (bind _pilier (Variables|Default|GetPilier))
  (bind _relativerotation (Variables|/Script/Engine.SceneComponent|GetRelativeRotation _pilier))
  (bind (_roll _pitch _yaw) (Math|Rotator|BreakRotator _relativerotation))
  ;[0.15 0.15 0.15 0.5] Interractions
  ;;[0.15 0.15 0.15 0.5] Verif distance
  (if (< (Math|Vector|Distance(Vector) (Transformation|GetActorLocation) (Transformation|GetActorLocation)) 4e+02)
    ;;[0.15 0.15 0.15 0.5] Est ce que le joueur focus ce laser
    (if (Variables|Default|GetIsFocused)
      ;;[0.15 0.15 0.15 0.5] Est ce qu il est deja en train de rotate
      (if (not (Variables|Default|GetbRotating))
        (bind _asbp_player_cidara (Utilities|Casting|CastToBP_PlayerCidara Investigator)
          (:then
            (Variables|/Game/Game/Blueprints/Characters/Cidara/Anims/ABP_Cidara.ABP_Cidara_C|SetDoTurnMirror (Variables|/Game/Game/Blueprints/Characters/Cidara/BP_PlayerCidara.BP_PlayerCidara_C|GetABP_Cidara _asbp_player_cidara) true))
          (:CastFailed
            _))
        (Variables|Default|SetbRotating true)
        (Variables|Default|SetStartRotation _relativerotation)
        (Variables|Default|SetTargetRotation (Math|Rotator|MakeRotator _roll _pitch (+ _yaw 9e+01)))
        (Audio|PlaySoundatLocation "/Game/Game/Blueprints/LaserLudo/SoundEffect/SC_Rotation.SC_Rotation" (Transformation|GetActorLocation) "0, 0, 0" 1.0 1.0 0.0 "/Game/Game/Blueprints/LaserLudo/SoundEffect/SM_Mirror.SM_Mirror" 0 0 0)
        (bind _alpha (Timeline|Timeline_0 PlayFromStart)
          (:Update
            (Transformation|SetRelativeRotation (Variables|Default|GetPilier) (Math|Rotator|Lerp(Rotator) (Variables|Default|GetStartRotation) (Variables|Default|GetTargetRotation) _alpha) false true))
          (:Finished
            (Variables|Default|SetbRotating false)
            (for _array_element (Variables|Default|GetBP_MirrorBig_0)
              (if (Utilities|Enum|Equal(Enum) (Variables|/Game/Game/Blueprints/LaserLudo/Elements/BP_MirrorBig.BP_MirrorBig_C|GetTagBig _array_element) (Variables|Default|GetTag))
                (Default|TurnMirrorBig _array_element)
                (else
                  (Development|PrintString "falseeeeee" true true "(R=0.750000,G=0.000000,B=0.035780,A=1.000000)"))))))))))

(event EventLongPressed
  (params (Look%20Direction%20Player :type Vector :default "0, 0, 0") (Investigator :type Actor%20Object%20Reference))
  ;[0.15 0.15 0.15 0.5] Interractions
  (bind _asbp_player_cidara (Utilities|Casting|CastToBP_PlayerCidara Investigator)
    (:then
      (Variables|/Game/Game/Blueprints/Characters/Cidara/Anims/ABP_Cidara.ABP_Cidara_C|SetDoPushMirror (Variables|/Game/Game/Blueprints/Characters/Cidara/BP_PlayerCidara.BP_PlayerCidara_C|GetABP_Cidara _asbp_player_cidara) true))
    (:CastFailed
      _))
  (Variables|Default|SetPlayer%20Look%20Direction Look%20Direction%20Player)
  (Variables|Default|SetBestDot 0.5)
  (Variables|Default|SetBestIndex -1)
  (for (_array_element _array_index) (Variables|Default|GetPointPosition)
    (if (not (== _array_index (Variables|Default|GetCurrentIndex)))
      (if (> (Math|Vector|DotProduct (Math|Vector|Normalize (- _array_element (Transformation|GetActorLocation))) (Variables|Default|GetPlayer%20Look%20Direction)) (Variables|Default|GetBestDot))
        (Variables|Default|SetBestDot (Math|Vector|DotProduct (Math|Vector|Normalize (- _array_element (Transformation|GetActorLocation))) (Variables|Default|GetPlayer%20Look%20Direction)))
        (Variables|Default|SetBestIndex _array_index))))
  (if (!= (Variables|Default|GetBestIndex) -1)
    (Variables|Default|SetCurrentIndex (Variables|Default|GetBestIndex))
    (Variables|Default|SetTragetPosition (Utilities|Array|Get(acopy) (Variables|Default|GetPointPosition) (Variables|Default|GetBestIndex)))
    (Variables|Default|SetStartLocation (Transformation|GetActorLocation))
    (Audio|PlaySoundatLocation "/Game/Game/Blueprints/LaserLudo/SoundEffect/SC_MirrorPush.SC_MirrorPush" (Transformation|GetActorLocation) "0, 0, 0" 1.0 1.0 0.0 0 0 0 0)
    (bind _alpha (Timeline|Timeline_1 PlayFromStart)
      (:Update
        (Transformation|SetActorLocation (Math|Vector|Lerp(Vector) (Variables|Default|GetStartLocation) (Variables|Default|GetTragetPosition) _alpha) false false)))))

(event EventSetFocus
  (params (Focused :type Boolean) (Investigator :type Actor%20Object%20Reference))
  ;[0.15 0.15 0.15 0.5] Outline
  (bind _output_get (Variables|Default|SetIsFocused Focused))
  (if _output_get
    (Rendering|SetVisibility (Variables|Default|GetOutlinePilier) true false)
    (else
      (Rendering|SetVisibility (Variables|Default|GetOutlinePilier) false false))))

(event EventSetEndFocus
  (params (EndFocus :type Boolean))
  ;[0.15 0.15 0.15 0.5] Outline
  (bind _output_get (Variables|Default|SetIsFocused EndFocus))
  (if _output_get
    (Rendering|SetVisibility (Variables|Default|GetOutlinePilier) false false)
    (else
      (Rendering|SetVisibility (Variables|Default|GetOutlinePilier) true false))))

(event Collision|EventActorBeginOverlap
  (params (OtherActor :type Actor%20Object%20Reference)))

(event EventTick
  (params (DeltaSeconds :type Float%20%28single-precision%29)))

(fn ConstructionScript
  (|CallParentFunction))