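; BP_ObeliskPuzzle is the controller actor for an obelisk-and-laser puzzle, though it holds no solving logic yet.
; On BeginPlay it registers itself with the GI_Cidara game instance, then caches every BP_Obelix and BP_ObeliskLaser actor in the world.
; ApplyStatefromManager switches on the incoming state, but none of its branches are implemented.
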(event EventBeginPlay
  (|CallParentFunction)
  (Utilities|FlowControl|Sequence
    (:then_0
      (bind _asgi_cidara (Utilities|Casting|CastToGI_Cidara (Game|GetGameInstance)))
      (bind _output_get (Variables|Default|SetGameInstanceRef _asgi_cidara))
      (if (Utilities|IsValid _output_get)
        (CallFunction|GetPuzzleName (Variables|Default|GetPuzzleId))
        (Default|RegisterPuzzle _output_get self)))
    (:then_1
      (bind _outactors (Actor|GetAllActorsOfClass "/Game/Game/Blueprints/Puzzle/PuzzleObelisk/BP_Obelix.BP_Obelix_C"))
      (Variables|Default|SetObeliskRef _outactors))
    (:then_2
      (bind _outactors_2 (Actor|GetAllActorsOfClass "/Game/Game/Blueprints/Puzzle/PuzzleObelisk/BP_ObeliskLaser.BP_ObeliskLaser_C"))
      (Variables|Default|SetObeliskLaserRef _outactors_2))))

(event Collision|EventActorBeginOverlap
  (params (OtherActor :type Actor%20Object%20Reference))
  (|CallParentFunction OtherActor) ; This node is disabled and will not be called.\nDrag off pins to build functionality.
)

(event EventTick
  (params (DeltaSeconds :type Float%20%28single-precision%29))
  (|CallParentFunction DeltaSeconds) ; This node is disabled and will not be called.\nDrag off pins to build functionality.
)

(event EventApplyStatefromManager
  (params (NewState :type E_PuzzleState%20Enum :default "NewEnumerator0"))
  (switch Utilities|FlowControl|Switch|SwitchonE_PuzzleState NewState))

(fn ConstructionScript
  (|CallParentFunction))