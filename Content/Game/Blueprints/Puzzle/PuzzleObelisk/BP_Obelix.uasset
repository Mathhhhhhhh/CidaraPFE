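; BP_Obelix is a puzzle obelisk that switches on a laser beam when the level's BP_Spectre actor enters its ActivationSphere.
; BeginPlay caches the Spectre for the overlap check and also looks up BP_TempleDoor, though that result is unused.
; ActivateObelisk sets IsActivated, reveals the laser mesh and plays a timeline that stretches its Z scale to extend the beam.
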(event OnComponentBeginOverlap(ActivationSphere)
  (params (OverlappedComponent :type Primitive%20Component%20Object%20Reference) (OtherActor :type Actor%20Object%20Reference) (OtherComp :type Primitive%20Component%20Object%20Reference) (OtherBodyIndex :type Integer) (bFromSweep :type Boolean) (SweepResult :type Hit%20Result%20Structure%20%28by%20ref%29))
  (if (== OtherActor (Variables|Default|GetSpectreRef))
    (CallFunction|ActivateObelisk)))

(event Custom|ActivateObelisk
  (bind _laser (Variables|Default|GetLaser))
  (bind _laser_mesh (Variables|/Game/Game/Blueprints/Puzzle/PuzzleObelisk/BP_ObeliskLaser.BP_ObeliskLaser_C|GetLaser_Mesh _laser))
  (Variables|Default|SetIsActivated true)
  (Rendering|SetVisibility _laser_mesh true false)
  (bind _alpha (Timeline|TL_ScaleLaser Play)
    (:Update
      (Transformation|SetRelativeScale3D _laser_mesh (Math|Vector|MakeVector 0.035 0.035 (Math|Float|Lerp 0.01 1e+03 _alpha))))))

(event Collision|EventActorBeginOverlap
  (params (OtherActor :type Actor%20Object%20Reference)))

(event EventTick
  (params (DeltaSeconds :type Float%20%28single-precision%29)))

(event EventBeginPlay
  (Utilities|FlowControl|Sequence
    (:then_0
      (bind _returnvalue (Actor|GetActorOfClass "/Game/Game/Blueprints/Characters/Spectre/BP_Spectre.BP_Spectre_C"))
      (Variables|Default|SetSpectreRef _returnvalue))
    (:then_1
      (Actor|GetActorOfClass "/Game/Game/Blueprints/Puzzle/TempleDoor/BP_TempleDoor.BP_TempleDoor_C"))))

(fn ConstructionScript)