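; Collectible piece for the tutorial elevator puzzle, which the player picks up by interacting within range once it is revealed.
; Collection notifies BP_PuzzleElevatorTuto, then timelines raise the piece and oscillate its scale before a delay releases it.
; Tick then flies it toward the player until it is close enough to stop its reveal and destroy itself.
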(event Custom|CollectAnimation
  (bind _scale (Variables|Default|GetScale))
  (bind _startlocation (Variables|Default|GetStartLocation))
  (bind _alpha (Timeline|TL_MoveUp Play)
    (:Update
      (Transformation|SetActorLocation (Math|Vector|Lerp(Vector) _startlocation (+ _startlocation (Math|Vector|MakeVector 0.0 0.0 (Variables|Default|GetTargetHeight))) _alpha) false false))
    (:Finished
      (bind _alpha_2 (Timeline|TL_ScaleOscil Play)
        (:Update
          (Transformation|SetActorScale3D (Math|Vector|Lerp(Vector) (Variables|Default|GetScale) (+ _scale (* _scale (Variables|Default|GetScaleIntensity))) _alpha_2))
          (Utilities|FlowControl|Delay 2.0)
          (Utilities|FlowControl|Sequence
            (:then_0
              (Timeline|TL_ScaleOscil Stop))
            (:then_1
              (Variables|Default|SetCanGo? true))))))))

(event EventBeginPlay
  (Utilities|FlowControl|Sequence
    (:then_0
      (|CallParentFunction))
    (:then_1
      (bind _returnvalue (Actor|GetActorOfClass "/Game/Game/Blueprints/Puzzle/PuzzleTuto/PuzzleElevator/BP_PuzzleElevatorTuto.BP_PuzzleElevatorTuto_C"))
      (Variables|Default|SetPuzzleRef _returnvalue))
    (:then_2
      (Variables|Default|SetStartLocation (Transformation|GetActorLocation)))
    (:then_3
      (Variables|Default|SetScale (Variables|/Script/Engine.SceneComponent|GetRelativeScale3D (Variables|Default|GetStaticMesh))))))

(event EventTick
  (params (DeltaSeconds :type Float%20%28single-precision%29))
  (if (Variables|Default|GetCanGo?)
    (bind _output_get (Variables|Default|SetDirection (Math|Vector|Normalize (- (Transformation|GetActorLocation (Game|GetPlayerCharacter 0)) (Transformation|GetActorLocation)))))
    (Transformation|SetActorLocation (+ (Transformation|GetActorLocation) (* (* _output_get (Variables|Default|GetFlySpeed)) (Variables|Default|GetDeltaSecond))) false false)
    (if (<= (Math|Vector|Distance(Vector) (Transformation|GetActorLocation (Game|GetPlayerCharacter 0)) (Transformation|GetActorLocation)) (Variables|Default|GetDisapearRange))
      (Utilities|FlowControl|DoOnce false
        (:Completed
          (CallFunction|StopReveal)
          (Utilities|FlowControl|Delay 0.5)
          (Actor|DestroyActor))))))

(event EventInteract
  (bind _puzzleref (Variables|Default|GetPuzzleRef))
  (if (and (and (not (Variables|Default|GetIsCollected)) (Variables|Default|GetIsRevealed?)) (<= (Math|Vector|Distance(Vector) (Transformation|GetActorLocation (Game|GetPlayerCharacter 0)) (Transformation|GetActorLocation)) (Variables|Default|GetCollectRange)))
    (Variables|Default|SetIsCollected true)
    (CallFunction|CollectAnimation)
    (if (Utilities|IsValid _puzzleref)
      (Default|OnPiecesCollected _puzzleref self))))

(fn ConstructionScript
  (|CallParentFunction))