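; Puzzle tutorial elevator actor that moves from a start point to an end point when the player interacts with it.
; Interact activates it only if CanBeActivated is set and the player character is within ActivateRange of the root component.
; A timeline then lerps the actor, with sweep, between the Start and End world locations cached at BeginPlay.
; The graph only plays the timeline forward, with no reverse move.
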(event Custom|ActivateElevator
  (bind _alpha (Timeline|Tl_MoveUp Play)
    (:Update
      (Transformation|SetActorLocation (Math|Vector|Lerp(Vector) (Variables|Default|GetStartLocation) (Variables|Default|GetEndLocation) _alpha) true false))))

(event EventBeginPlay
  (Variables|Default|SetStartLocation (Transformation|GetWorldLocation (Variables|Default|GetStart)))
  (Variables|Default|SetEndLocation (Transformation|GetWorldLocation (Variables|Default|GetEnd))))

(event Collision|EventActorBeginOverlap
  (params (OtherActor :type Actor%20Object%20Reference)))

(event EventInteract
  (if (and (Variables|Default|GetCanBeActivated?) (<= (Math|Vector|Distance(Vector) (Transformation|GetActorLocation (Game|GetPlayerCharacter 0)) (Transformation|GetWorldLocation (Variables|Default|GetDefaultSceneRoot))) (Variables|Default|GetActivateRange)))
    (CallFunction|ActivateElevator)))

(fn ConstructionScript)