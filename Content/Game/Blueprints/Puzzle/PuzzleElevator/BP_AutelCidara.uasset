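; Cidara's altar in the elevator puzzle, which also triggers the level's closing cinematic.
; When Cidara enters its box with the linked altar active, a timeline moves a Niagara effect to the crystal, turns it blue and arms the cinematic flag.
; Cidara entering CinBox plays the sequence, activates the elevator and loads the elven village behind a loading screen.
; The checks for both characters, the flag and puzzle completion are disconnected and never run.
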(event OnComponentBeginOverlap(Box)
  (params (OverlappedComponent :type Primitive%20Component%20Object%20Reference) (OtherActor :type Actor%20Object%20Reference) (OtherComp :type Primitive%20Component%20Object%20Reference) (OtherBodyIndex :type Integer) (bFromSweep :type Boolean) (SweepResult :type Hit%20Result%20Structure%20%28by%20ref%29))
  (bind _returnvalue (Transformation|GetActorLocation))
  (Utilities|Casting|CastToBP_PlayerCidara OtherActor)
  (Variables|Default|SetIsActive true)
  (if (Variables|/Game/Game/Blueprints/Puzzle/PuzzleElevator/BP_AutelSpectre.BP_AutelSpectre_C|GetIsActive (Variables|Default|GetAutelRef))
    (bind _returnvalue_2 (Niagara|SpawnSystematLocation "/Game/Basic_VFX/Niagara/NS_Basic_16.NS_Basic_16" _returnvalue))
    (Utilities|FlowControl|Sequence
      (:then_0
        (bind _alpha (Timeline|Timeline Play)
          (:Update
            (Transformation|SetWorldLocation _returnvalue_2 (Math|Vector|Lerp(Vector) _returnvalue (Transformation|GetActorLocation (Variables|Default|GetCristalRef)) _alpha) false false))
          (:Finished
            (Components|DestroyComponent _returnvalue_2)
            (Rendering|Material|SetMaterial (Variables|/Game/Game/Blueprints/Puzzle/PuzzleElevator/BP_ElevatorCrystal.BP_ElevatorCrystal_C|GetStaticMesh (Variables|Default|GetCristalRef)) 0 "/Game/DreamscapeSeries/DreamscapeTower/Materials/Crystals/MI_CrystaGroup_01_Blue.MI_CrystaGroup_01_Blue")
            (Variables|Default|SetCinCanBeActivated true)
            (Utilities|FlowControl|Delay 1.0))))
      (:then_1
        (Utilities|FlowControl|DoOnce false
          (:Completed
            (Audio|PlaySound2D "/Game/Game/Sounds/Feedback/AutelsActivations_Cue.AutelsActivations_Cue" 1.0 1.0 0.0 0 0)))))))

(event OnComponentBeginOverlap(CinBox)
  (params (OverlappedComponent :type Primitive%20Component%20Object%20Reference) (OtherActor :type Actor%20Object%20Reference) (OtherComp :type Primitive%20Component%20Object%20Reference) (OtherBodyIndex :type Integer) (bFromSweep :type Boolean) (SweepResult :type Hit%20Result%20Structure%20%28by%20ref%29))
  (Utilities|Casting|CastToBP_PlayerCidara OtherActor)
  (CallFunction|PlayFinal)
  (Utilities|FlowControl|Delay 17.3)
  (Default|ActivateElevator (Variables|Default|GetElevatorRef))
  (Utilities|FlowControl|Delay 5.7)
  (bind _asgi_cidara (Utilities|Casting|CastToGI_Cidara (Game|GetGameInstance)))
  (Variables|/Game/Game/Blueprints/Manager/GI_Cidara.GI_Cidara_C|SetbIsMenuMode _asgi_cidara false)
  (bind _returnvalue (UserInterface|CreateWidget "/Game/Game/Blueprints/Widget/WBP_LoadingScreen.WBP_LoadingScreen_C"))
  (UserInterface|Viewport|AddtoViewport _returnvalue 0)
  (Default|LoadingFadein _returnvalue)
  (Game|OpenLevel(byObjectReference) "/Game/Game/Maps/L_VillageElfique.L_VillageElfique"))

(event OnComponentEndOverlap(CinBox)
  (params (OverlappedComponent :type Primitive%20Component%20Object%20Reference) (OtherActor :type Actor%20Object%20Reference) (OtherComp :type Primitive%20Component%20Object%20Reference) (OtherBodyIndex :type Integer))
  (Utilities|Casting|CastToBP_Spectre OtherActor
    (:then
      (Variables|Default|SetSpectreIn false))
    (:CastFailed
      (Variables|Default|SetCidaraIn false))))

(event EventBeginPlay)

(event Collision|EventActorBeginOverlap
  (params (OtherActor :type Actor%20Object%20Reference)))

(event EventTick
  (params (DeltaSeconds :type Float%20%28single-precision%29)))

(fn ConstructionScript)

(fn PlayFinal
  (bind _returnvalue (Game|GetPlayerController 0))
  (bind _returnvalue_2 (Actor|GetActorOfClass "/Game/Game/Blueprints/Characters/Cidara/BP_PlayerCidara.BP_PlayerCidara_C"))
  (Rendering|SetActorHiddenInGame _returnvalue_2 true)
  (bind _returnvalue_3 (Actor|GetActorOfClass "/Game/Game/Blueprints/Characters/Spectre/BP_Spectre.BP_Spectre_C"))
  (Rendering|SetActorHiddenInGame _returnvalue_3 true)
  (Viewport|RemoveAllWidgets)
  (Input|DisableInput (Pawn|GetControlledPawn _returnvalue) _returnvalue)
  (Sequencer|Player|Play (Variables|/Script/LevelSequence.LevelSequenceActor|GetSequencePlayer (Variables|Default|GetLevelSequence)) :!class /Script/MovieScene.MovieSceneSequencePlayer))