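; BP_Elevator is a puzzle elevator that rises from a Start point to an End point when its Detection volume is overlapped.
; The overlap, gated by CanBeActivated, starts the elevator and calls EndLoopMessage on the BP_FixLoop actor found at BeginPlay.
; Activation triggers the player pawn's ElevatorShake and a door sound, then after a delay a timeline lerps the actor between the cached locations with sweep.
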(event OnComponentBeginOverlap(Detection)
  (params (OverlappedComponent :type Primitive%20Component%20Object%20Reference) (OtherActor :type Actor%20Object%20Reference) (OtherComp :type Primitive%20Component%20Object%20Reference) (OtherBodyIndex :type Integer) (bFromSweep :type Boolean) (SweepResult :type Hit%20Result%20Structure%20%28by%20ref%29))
  (if (Variables|Default|GetCanBeActivated?)
    (CallFunction|ActivateElevator)
    (Class|BPIEndLoop|EndLoop(Message) (Variables|Default|GetFixLoopRef))))

(event Custom|ActivateElevator
  (bind _asbp_player_cidara (Utilities|Casting|CastToBP_PlayerCidara (Game|Player|GetPlayerPawn 0)))
  (Default|ElevatorShake _asbp_player_cidara)
  (Audio|PlaySound2D "/Game/Game/Sounds/Environment/DoorOpening.DoorOpening" 1.0 1.0 0.0 0 0 false)
  (Utilities|FlowControl|Delay 3.0)
  (bind _alpha (Timeline|Tl_MoveUp Play)
    (:Update
      (Transformation|SetActorLocation (Math|Vector|Lerp(Vector) (Variables|Default|GetStartLocation) (Variables|Default|GetEndLocation) _alpha) true false))))

(event EventBeginPlay
  (Utilities|FlowControl|Sequence
    (:then_0
      (Variables|Default|SetStartLocation (Transformation|GetWorldLocation (Variables|Default|GetStart)))
      (Variables|Default|SetEndLocation (Transformation|GetWorldLocation (Variables|Default|GetEnd))))
    (:then_1
      (bind _returnvalue (Actor|GetActorOfClass "/Game/Game/Blueprints/Characters/BP_PlayerCidara.BP_PlayerCidara_C"))
      (Variables|Default|SetPlayerRef _returnvalue))
    (:then_2
      (bind _returnvalue_2 (Actor|GetActorOfClass "/Game/Game/Blueprints/Puzzle/PuzzleElevator/BP_FixLoop.BP_FixLoop_C"))
      (Variables|Default|SetFixLoopRef _returnvalue_2))))

(fn ConstructionScript)