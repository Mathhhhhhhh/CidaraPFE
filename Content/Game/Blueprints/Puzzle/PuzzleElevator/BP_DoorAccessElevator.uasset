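; Elevator access double door for a puzzle, swung open once through OpenDoor with a short camera cutscene.
; After a delay, it removes player input mapping and blends the view to its own camera.
; A timeline rotates both leaves in yaw, the left toward absolute zero and the right by a relative offset, with a one-shot sound.
; On finish, it returns the view to Cidara, restores input and exits Spectre mode.
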(event Custom|OpenDoor
  (bind _as_pc_cidara (Variables|Default|GetAs%20PC%20Cidara))
  (bind _as_pc_cidara_2 (Variables|Default|GetAs%20PC%20Cidara))
  (if (not (Variables|Default|GetIsDoorOpen))
    (Utilities|FlowControl|Delay 2.0)
    (Default|RemoveMapping _as_pc_cidara_2)
    (Game|Player|SetViewTargetwithBlend _as_pc_cidara_2 (Variables|Default|GetCamera) 2.0 "VTBlend_Cubic" 2.0 false)
    (Variables|Default|SetIsDoorOpen true)
    (bind (_direction _doorleftalpha _doorrightalpha) (Timeline|TL_Open PlayFromStart)
      (:Update
        (Utilities|FlowControl|Sequence
          (:then_0
            (Transformation|SetWorldRotation (Variables|Default|GetStaticMesh) (Math|Rotator|MakeRotator 0.0 0.0 (Math|Float|Lerp (Variables|Default|GetBaseRotA) 0.0 _doorleftalpha)) false false)
            (Transformation|SetWorldRotation (Variables|Default|GetStaticMesh1) (Math|Rotator|MakeRotator 0.0 0.0 (Math|Float|Lerp (Variables|Default|GetBaseRotB) (Variables|Default|GetTargetRotB) _doorrightalpha)) false false))
          (:then_1
            (Utilities|FlowControl|DoOnce false
              (:Completed
                (Audio|PlaySound2D "/Game/Game/Blueprints/Bridge/SC_BridgeUp.SC_BridgeUp" 1.0 1.0 0.0 0 0))))))
      (:Finished
        (Game|Player|SetViewTargetwithBlend _as_pc_cidara (Variables|Default|GetCidara) 0.0 "VTBlend_Cubic" 1.0 false)
        (Utilities|FlowControl|Delay 0.2)
        (Default|AddMapping _as_pc_cidara)
        (Default|ExitSpectreMode _as_pc_cidara)))))

(event EventBeginPlay
  (bind _aspc_cidara (Utilities|Casting|CastToPC_Cidara (Game|GetPlayerController 0)))
  (Variables|Default|SetAs%20PC%20Cidara _aspc_cidara)
  (bind _output_get (Variables|Default|SetBaseRotA (.yaw (Transformation|GetWorldRotation (Variables|Default|GetStaticMesh)))))
  (Variables|Default|SetTargetRotA (+ _output_get 8e+01))
  (bind _output_get_2 (Variables|Default|SetBaseRotB (.yaw (Transformation|GetWorldRotation (Variables|Default|GetStaticMesh1)))))
  (Variables|Default|SetTargetRotB (- _output_get_2 8e+01))
  (bind _returnvalue (Actor|GetActorOfClass "/Game/Game/Blueprints/Characters/Cidara/BP_PlayerCidara.BP_PlayerCidara_C"))
  (Variables|Default|SetCidara _returnvalue))

(fn ConstructionScript)