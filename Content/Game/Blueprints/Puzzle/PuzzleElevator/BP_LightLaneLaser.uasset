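; BP_LightLaneLaser is a light lane laser for the elevator puzzle, switching a rect light and box collision on or off together.
; BeginPlay caches the light's intensity and attenuation radius, then fades in or out based on IsActive.
; One timeline, played forward or reversed, scales both values from zero.
; Its direction sets Box collision during the fade and IsActive when finished.
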(event Custom|FAdeoutLigth
  (bind _rectlight (Variables|Default|GetRectLight))
  (bind _box (Variables|Default|GetBox))
  (bind (_direction _alpha) (Timeline|TL_FadeLigth ReverseFromEnd)
    (:Update
      (Rendering|Components|Light|SetIntensity _rectlight (Math|Float|Lerp 0.0 (Variables|Default|GetIntensity) _alpha))
      (Rendering|Lighting|SetAttenuationRadius _rectlight (Math|Float|Lerp 0.0 (Variables|Default|GetAttenuation%20Radius) _alpha))
      (switch Utilities|FlowControl|Switch|SwitchonETimelineDirection _direction
        (:Forward
          (Collision|SetCollisionEnabled _box "QueryAndPhysics"))
        (:Backward
          (Collision|SetCollisionEnabled _box "NoCollision"))))
    (:Finished
      (switch Utilities|FlowControl|Switch|SwitchonETimelineDirection _direction
        (:Forward
          (Variables|Default|SetIsActive true))
        (:Backward
          (Variables|Default|SetIsActive false))))))

(event Custom|FAdeInLigth
  (bind _rectlight (Variables|Default|GetRectLight))
  (bind _box (Variables|Default|GetBox))
  (bind (_direction _alpha) (Timeline|TL_FadeLigth PlayFromStart)
    (:Update
      (Rendering|Components|Light|SetIntensity _rectlight (Math|Float|Lerp 0.0 (Variables|Default|GetIntensity) _alpha))
      (Rendering|Lighting|SetAttenuationRadius _rectlight (Math|Float|Lerp 0.0 (Variables|Default|GetAttenuation%20Radius) _alpha))
      (switch Utilities|FlowControl|Switch|SwitchonETimelineDirection _direction
        (:Forward
          (Collision|SetCollisionEnabled _box "QueryAndPhysics"))
        (:Backward
          (Collision|SetCollisionEnabled _box "NoCollision"))))
    (:Finished
      (switch Utilities|FlowControl|Switch|SwitchonETimelineDirection _direction
        (:Forward
          (Variables|Default|SetIsActive true))
        (:Backward
          (Variables|Default|SetIsActive false))))))

(event EventBeginPlay
  (bind _rectlight (Variables|Default|GetRectLight))
  (Variables|Default|SetIntensity (Variables|/Script/Engine.LightComponentBase|GetIntensity _rectlight))
  (Variables|Default|SetAttenuation%20Radius (Variables|/Script/Engine.LocalLightComponent|GetAttenuationRadius _rectlight))
  (if (Variables|Default|GetIsActive)
    (CallFunction|FAdeinLigth)
    (else
      (CallFunction|FAdeoutLigth))))

(event Collision|EventActorBeginOverlap
  (params (OtherActor :type Actor%20Object%20Reference)))

(event EventTick
  (params (DeltaSeconds :type Float%20%28single-precision%29)))

(fn ConstructionScript)