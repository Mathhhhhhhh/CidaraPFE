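; BP_Conduit is an interactable elevator-puzzle conduit that switches between active and inactive states.
; When BP_PlayerCidara interacts, it toggles itself and sets its linked ConduitRef to the opposite state, then ignores further interaction during a short cooldown.
; Each state change plays or reverses a timeline driving emissive intensity on a dynamic material and fades the associated light lane in or out.
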(event Custom|SetActive
  (bind _alpha (Timeline|TL_Active Play)
    (:Update
      (Rendering|Material|SetScalarParameterValue (Variables|Default|GetDynamicMatRef) "Emissive Intensity" (Math|Float|Lerp 0.0 2.0 _alpha) :!class /Script/Engine.MaterialInstanceDynamic))))

(event Custom|Deactive
  (bind _alpha (Timeline|TL_Active Reverse)
    (:Update
      (Rendering|Material|SetScalarParameterValue (Variables|Default|GetDynamicMatRef) "Emissive Intensity" (Math|Float|Lerp 0.0 2.0 _alpha) :!class /Script/Engine.MaterialInstanceDynamic))))

(event Custom|DeactiveConduit
  (CallFunction|Deactive)
  (Variables|Default|SetIsActive false)
  (Default|FAdeoutLigth (Variables|Default|GetAssociedLigthLane)))

(event Custom|ActivateConduit
  (CallFunction|SetActive)
  (Variables|Default|SetIsActive true)
  (Default|FAdeinLigth (Variables|Default|GetAssociedLigthLane)))

(event EventBeginPlay
  (bind _mesh (Variables|Default|GetMesh))
  (Utilities|FlowControl|Sequence
    (:then_0
      (bind _returnvalue (Rendering|Material|CreateDynamicMaterialInstance _mesh 2 (Rendering|Material|GetMaterial _mesh 2) "None" :!class /Script/Engine.PrimitiveComponent))
      (Variables|Default|SetDynamicMatRef _returnvalue)
      (if (Variables|Default|GetIsActive)
        (CallFunction|SetActive)
        (else
          (CallFunction|Deactive))))
    (:then_1
      (Actor|GetActorOfClass "/Game/Game/Blueprints/Characters/Cidara/BP_PlayerCidara.BP_PlayerCidara_C"))))

(event EventInterract
  (params (Investigator :type Actor%20Object%20Reference))
  (bind _conduitref (Variables|Default|GetConduitRef))
  (Utilities|Casting|CastToBP_PlayerCidara Investigator)
  (if (Variables|Default|GetCanInterract)
    (Variables|Default|SetCanInterract false)
    (if (Variables|Default|GetIsActive)
      (CallFunction|DeactiveConduit)
      (CallFunction|ActivateConduit _conduitref)
      (else
        (CallFunction|ActivateConduit)
        (CallFunction|DeactiveConduit _conduitref)))
    (Utilities|FlowControl|Delay 4.0)
    (Variables|Default|SetCanInterract true)))

(fn ConstructionScript)