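; Spectre altar for the elevator puzzle that activates while a BP_Spectre stands in its box, sending a particle to a linked crystal and turning it purple.
; The first activation plays a timeline-driven cutscene, locking input while the camera shows a door moving amid dust and pans with the particle.
; On exit, the particle returns and the crystal turns red, unless the paired altar is still active.
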(event OnComponentBeginOverlap(Box)
  (params (OverlappedComponent :type Primitive%20Component%20Object%20Reference) (OtherActor :type Actor%20Object%20Reference) (OtherComp :type Primitive%20Component%20Object%20Reference) (OtherBodyIndex :type Integer) (bFromSweep :type Boolean) (SweepResult :type Hit%20Result%20Structure%20%28by%20ref%29))
  (bind _returnvalue (Transformation|GetActorLocation))
  (bind _returnvalue_2 (Game|GetPlayerController 0))
  (bind _returnvalue_3 (Game|GetPlayerController 0))
  (bind _doorref (Variables|Default|GetDoorRef))
  (bind _baselocation (Variables|/Game/Game/Blueprints/Puzzle/PuzzleElevator/BP_DoorElevator.BP_DoorElevator_C|GetBaseLocation _doorref))
  (Utilities|Casting|CastToBP_Spectre OtherActor)
  (Variables|Default|SetIsActive true)
  (Utilities|FlowControl|Sequence
    (:then_0
      (if (Variables|Default|GetDoOnce)
        (Utilities|FlowControl|DoOnce false
          (:Completed
            (Game|Player|SetViewTargetwithBlend _returnvalue_2 (Variables|Default|GetCamera) 1.0 "VTBlend_Cubic" 1.0 false)
            (Input|DisableInput _returnvalue_2 _returnvalue_2)
            (bind _alpha (Timeline|Timeline Play)
              (:Update
                (Transformation|SetActorLocation _doorref (Math|Vector|Lerp(Vector) _baselocation (Variables|/Game/Game/Blueprints/Puzzle/PuzzleElevator/BP_DoorElevator.BP_DoorElevator_C|GetTargetLocation _doorref) _alpha) false false)
                (Utilities|FlowControl|DoOnce false
                  (:Completed
                    (bind _returnvalue_4 (Niagara|SpawnSystematLocation "/Game/Basic_VFX/Niagara/NS_Dust.NS_Dust" _baselocation "0.000000,90.000000,0.000000" "5.000000,1.500000,1.000000")))))
              (:Finished
                (Components|DestroyComponent _returnvalue_4 :!label _label)
                (bind _returnvalue_5 (Niagara|SpawnSystematLocation "/Game/Basic_VFX/Niagara/NS_Basic_14.NS_Basic_14" _returnvalue))
                (bind _alpha_2 (Timeline|Timeline_0 Play)
                  (:Update
                    (Transformation|SetWorldLocation _returnvalue_5 (Math|Vector|Lerp(Vector) _returnvalue (Transformation|GetActorLocation (Variables|Default|GetCrystalRef)) _alpha_2) false false)
                    (Transformation|SetActorLocation (Variables|Default|GetCamera) (Math|Vector|Lerp(Vector) (Variables|Default|GetBaseLocationCam) (Variables|Default|GetTargetLocationCam) _alpha_2) false false))
                  (:Finished
                    (Components|DestroyComponent _returnvalue_5)
                    (Rendering|Material|SetMaterial (Variables|/Game/Game/Blueprints/Puzzle/PuzzleElevator/BP_ElevatorCrystal.BP_ElevatorCrystal_C|GetStaticMesh (Variables|Default|GetCrystalRef)) 0 "/Game/DreamscapeSeries/DreamscapeTower/Materials/Crystals/MI_CrystaGroup_01_Purple.MI_CrystaGroup_01_Purple")
                    (Utilities|FlowControl|DoOnce false
                      (:Completed
                        (Game|Player|SetViewTargetwithBlend _returnvalue_3 (Variables|Default|GetCameraZoneRef) 1.0 "VTBlend_Cubic" 1.0 false)
                        (Input|EnableInput _returnvalue_3 _returnvalue_3)
                        (Variables|Default|SetDoOnce false)))))))))
        (else
          (goto _label))))))

(event OnComponentEndOverlap(Box)
  (params (OverlappedComponent :type Primitive%20Component%20Object%20Reference) (OtherActor :type Actor%20Object%20Reference) (OtherComp :type Primitive%20Component%20Object%20Reference) (OtherBodyIndex :type Integer))
  (bind _crystalref (Variables|Default|GetCrystalRef))
  (bind _returnvalue (Transformation|GetActorLocation _crystalref))
  (Utilities|Casting|CastToBP_Spectre OtherActor)
  (Variables|Default|SetIsActive false)
  (if (not (Variables|/Game/Game/Blueprints/Puzzle/PuzzleElevator/BP_AutelCidara.BP_AutelCidara_C|GetIsActive (Variables|Default|GetAutelRef)))
    (bind _returnvalue_2 (Niagara|SpawnSystematLocation "/Game/Basic_VFX/Niagara/NS_Basic_14.NS_Basic_14" _returnvalue))
    (bind _alpha (Timeline|Timeline_1 Play)
      (:Update
        (Transformation|SetWorldLocation _returnvalue_2 (Math|Vector|Lerp(Vector) _returnvalue (Transformation|GetActorLocation) _alpha) false false))
      (:Finished
        (Rendering|Material|SetMaterial (Variables|/Game/Game/Blueprints/Puzzle/PuzzleElevator/BP_ElevatorCrystal.BP_ElevatorCrystal_C|GetStaticMesh (Variables|Default|GetCrystalRef)) 0 "/Game/DreamscapeSeries/DreamscapeTower/Materials/Crystals/MI_CrystaGroup_02_Red.MI_CrystaGroup_02_Red")
        (Utilities|FlowControl|Delay 0.2)
        (Components|DestroyComponent _returnvalue_2)))))

(event EventBeginPlay
  (bind _output_get (Variables|Default|SetBaseLocationCam (Transformation|GetActorLocation (Variables|Default|GetCamera))))
  (Variables|Default|SetTargetLocationCam (+ _output_get "-1000.000000,0.000000,-100.000000")))

(event Collision|EventActorBeginOverlap
  (params (OtherActor :type Actor%20Object%20Reference)))

(fn ConstructionScript)