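; Tutorial shadow stone for the puzzle elevator: an outlined interactable that triggers a one-time cutscene revealing a dynamic shadow.
; Interacting within range turns off the player's point light, disables input and blends to a set camera.
; Parallel timelines move a sphere from the player's reveal halo to the stone's scene point and scale it, enabling the shadow partway through.
; The scale timeline's end destroys the blocker box, then restores view and input.
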(event EventBeginPlay
  (bind _returnvalue (Actor|GetActorOfClass "/Game/Game/Blueprints/Characters/Cidara/BP_PlayerCidara.BP_PlayerCidara_C"))
  (Variables|Default|SetPlayerRef _returnvalue))

(event Collision|EventActorBeginOverlap
  (params (OtherActor :type Actor%20Object%20Reference)))

(event EventTick
  (params (DeltaSeconds :type Float%20%28single-precision%29)))

(event EventInterract
  (params (Investigator :type Actor%20Object%20Reference))
  (bind _returnvalue (Game|GetPlayerController 0))
  (bind _returnvalue_2 (Game|GetPlayerController 0))
  (bind _returnvalue_3 (Game|GetPlayerController 0))
  (bind _playerref (Variables|Default|GetPlayerRef))
  (bind _sphere (Variables|Default|GetSphere))
  (bind _dynamicshadowref (Variables|Default|GetDynamicShadowRef))
  (if (and (< (Math|Vector|VectorLength (- (Transformation|GetActorLocation _playerref) (Transformation|GetWorldLocation (Variables|Default|GetStaticMesh)))) 4e+02) (Variables|Default|GetCanInterract))
    (Variables|Default|SetCanInterract false)
    (Default|PointLightOff _playerref)
    (Input|DisableInput _returnvalue_3 _returnvalue_3)
    (Game|Player|SetViewTargetwithBlend _returnvalue_3 (Variables|Default|GetCameraRef) 0.0 "VTBlend_EaseOut" 0.0 false)
    (bind _output_get (Variables|Default|SetRevealHaloLoc (Transformation|GetWorldLocation (Variables|/Game/Game/Blueprints/Characters/Cidara/BP_PlayerCidara.BP_PlayerCidara_C|GetRevealHalo (Variables|Default|GetPlayerRef)))))
    (Utilities|FlowControl|Sequence
      (:then_0
        (bind _alpha (Timeline|TL_Animation PlayFromStart)
          (:Update
            (Transformation|SetWorldLocation (Variables|Default|GetSphere) (Math|Vector|Lerp(Vector) _output_get (Transformation|GetWorldLocation (Variables|Default|GetScene)) _alpha) false false))))
      (:then_1
        (bind _alpha_2 (Timeline|Timeline PlayFromStart)
          (:Update
            (Transformation|SetWorldScale3D _sphere (Math|Vector|Lerp(Vector) (Transformation|GetWorldScale _sphere) (Variables|Default|GetScaleTarget) _alpha_2))
            (if (>= _alpha_2 0.25)
              (Utilities|FlowControl|Delay 0.2)
              (Utilities|FlowControl|DoOnce false
                (:Completed
                  (Default|ShadowAppear _dynamicshadowref)
                  (Default|SetEnabled _dynamicshadowref true)))))
          (:Finished
            (Actor|DestroyActor (Variables|Default|GetBlockerBox))
            (Utilities|FlowControl|Delay 1.0)
            (Game|Player|SetViewTargetwithBlend _returnvalue_2 (Pawn|GetControlledPawn _returnvalue_2) 0.0 "VTBlend_EaseOut" 0.0 false)
            (Utilities|FlowControl|Delay 0.4)
            (Input|EnableInput _returnvalue _returnvalue)))))))

(event EventSetFocus
  (params (Focused :type Boolean) (Investigator :type Actor%20Object%20Reference))
  (if Focused
    (Rendering|Material|SetOverlayMaterial (Variables|Default|GetStaticMesh) "/Game/Game/Materials/VFX/MI_InteractableOutline.MI_InteractableOutline" :!class /Script/Engine.MeshComponent)
    (else
      (Rendering|Material|SetOverlayMaterial (Variables|Default|GetStaticMesh) 0 :!class /Script/Engine.MeshComponent))))

(fn ConstructionScript)