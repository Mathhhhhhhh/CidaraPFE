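; Tutorial elevator puzzle that counts collected pieces and enables the elevator once all are gathered.
; On BeginPlay it registers with GI_Cidara and caches the elevator, pieces and access-elevator actors from the level.
; Reaching the piece total reports Completed to the game instance.
; State handling is separate: applying Not Started resets progress, while Completed fills the count, allows elevator activation and calls MovingPlatform on the access elevators.
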(event EventBeginPlay
  (|CallParentFunction)
  (Utilities|FlowControl|Sequence
    (:then_0
      (bind _returnvalue (Actor|GetActorOfClass "/Game/Game/Blueprints/Puzzle/PuzzleElevator/BP_ElevatorPieces.BP_ElevatorPieces_C"))
      (Variables|Default|SetElevatorPiecesRef _returnvalue))
    (:then_1
      (bind _asgi_cidara (Utilities|Casting|CastToGI_Cidara (Game|GetGameInstance)))
      (bind _output_get (Variables|Default|SetGameInstance _asgi_cidara))
      (if (Utilities|IsValid _output_get)
        (CallFunction|GetPuzzleName (Variables|Default|GetPuzzle%20Id))
        (Default|RegisterPuzzle _output_get self)))
    (:then_2
      (bind _returnvalue_2 (Actor|GetActorOfClass "/Game/Game/Blueprints/Puzzle/PuzzleElevator/BP_Elevator.BP_Elevator_C"))
      (Variables|Default|SetElevatorRef _returnvalue_2))
    (:then_3
      (bind _outactors (Actor|GetAllActorsOfClass "/Game/Game/Blueprints/Plateforms/BP_AccesElevators.BP_AccesElevators_C"))
      (Variables|Default|SetAcces%20Elevators _outactors))))

(event Collision|EventActorBeginOverlap
  (params (OtherActor :type Actor%20Object%20Reference))
  (|CallParentFunction OtherActor) ; This node is disabled and will not be called.\nDrag off pins to build functionality.
)

(event EventTick
  (params (DeltaSeconds :type Float%20%28single-precision%29))
  (|CallParentFunction DeltaSeconds) ; This node is disabled and will not be called.\nDrag off pins to build functionality.
)

(event EventApplyStatefromManager
  (params (NewState :type E_PuzzleState%20Enum :default "NewEnumerator0"))
  (bind _elevatorref (Variables|Default|GetElevatorRef))
  (switch Utilities|FlowControl|Switch|SwitchonE_PuzzleState NewState
    (:NewEnumerator0
      (Variables|Default|SetPiecesCollected 0)
      (Variables|Default|SetIsActivated? false))
    (:NewEnumerator2
      (Variables|Default|SetPiecesCollected (Variables|Default|GetTotalPieces))
      (Variables|Default|SetIsActivated? true)
      (Utilities|FlowControl|Sequence
        (:then_0
          (if (Utilities|IsValid _elevatorref)
            (Variables|/Game/Game/Blueprints/Puzzle/PuzzleElevator/BP_Elevator.BP_Elevator_C|SetCanBeActivated? _elevatorref true)))
        (:then_1
          (Default|MovingPlatform (Variables|Default|GetAcces%20Elevators)))))))

(fn ConstructionScript
  (|CallParentFunction))

(fn OnPiecesCollected
  (params (ElevatorPieces :type BP%20Elevator%20Pieces%20Object%20Reference))
  (bind _output_get (Variables|Default|SetPiecesCollected (+ (Variables|Default|GetPiecesCollected) 1)))
  (if (>= _output_get (Variables|Default|GetTotalPieces))
    (Variables|Default|SetIsActivated? true)
    (Default|SetPuzzleState (Variables|Default|GetGameInstance) (Variables|Default|GetPuzzle%20Id) "NewEnumerator2" true)
    (Development|PrintString "Ciompleted")
    (return)
    (else
      (return))))

(fn GetPuzzleName
  (params (PuzzleId :type Name :default "None"))
  (return (Variables|Default|GetPuzzle%20Id)))