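; BP_ElevatorPieces is a collectible piece for the tutorial elevator puzzle, picked up by interacting once revealed and within range.
; Collecting plays a sound, notifies BP_PuzzleElevatorTuto and runs timelines that raise, spin and scale the piece, with delayed destruction starting during the scale phase.
; When CanGo is set, Tick flies it toward the player, then stops the reveal, clears the player's target markers and destroys it.
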(event Custom|CollectAnimation
  (bind _scale (Variables|Default|GetScale))
  (bind _startlocation (Variables|Default|GetStartLocation))
  (bind _alpha (Timeline|TL_MoveUp PlayFromStart)
    (:Update
      (Transformation|SetActorLocation (Math|Vector|Lerp(Vector) _startlocation (+ _startlocation (Math|Vector|MakeVector 0.0 0.0 (Variables|Default|GetTargetHeight))) _alpha) false false)
      (Class|Actor|AddActorWorldRotation "0.000000,5.000000,0.000000"))
    (:Finished
      (bind _alpha_2 (Timeline|TL_ScaleOscil Play)
        (:Update
          (Transformation|SetActorScale3D (Math|Vector|Lerp(Vector) (Variables|Default|GetScale) (+ _scale (* _scale (Variables|Default|GetScaleIntensity))) _alpha_2))
          (Class|Actor|AddActorWorldRotation "0.000000,5.000000,0.000000")
          (Utilities|FlowControl|Delay 1.0)
          (Actor|DestroyActor))))))

(event EventBeginPlay
  (Utilities|FlowControl|Sequence
    (:then_0
      (|CallParentFunction))
    (:then_1
      (bind _returnvalue (Actor|GetActorOfClass "/Game/Game/Blueprints/Puzzle/PuzzleElevator/BP_PuzzleElevatorTuto.BP_PuzzleElevatorTuto_C"))
      (Variables|Default|SetPuzzleRef _returnvalue))
    (:then_2
      (Variables|Default|SetStartLocation (Transformation|GetActorLocation)))
    (:then_3
      (Variables|Default|SetScale (Variables|/Script/Engine.SceneComponent|GetRelativeScale3D (Variables|Default|GetStaticMesh))))
    (:then_4
      (bind _returnvalue_2 (Actor|GetActorOfClass "/Game/Game/Blueprints/Puzzle/PuzzleElevator/BP_PuzzleElevatorTuto.BP_PuzzleElevatorTuto_C"))
      (Variables|Default|SetPuzzleElevatorTuto _returnvalue_2))
    (:then_5
      (bind _returnvalue_3 (Actor|GetActorOfClass "/Game/Game/Blueprints/Characters/Cidara/BP_PlayerCidara.BP_PlayerCidara_C"))
      (Variables|Default|SetPlayerRef _returnvalue_3))))

(event EventInterract
  (params (Investigator :type Actor%20Object%20Reference))
  (bind _puzzleref (Variables|Default|GetPuzzleRef))
  (if (and (and (not (Variables|Default|GetIsCollected)) (Variables|Default|GetIsRevealed?)) (<= (Math|Vector|Distance(Vector) (Transformation|GetActorLocation Investigator) (Transformation|GetActorLocation)) (Variables|Default|GetCollectRange)))
    (Variables|Default|SetIsCollected true)
    (Audio|PlaySound2D "/Game/Game/Sounds/PickUp/SC_PickUp.SC_PickUp" 1.0 1.0 0.0 0 0)
    (CallFunction|CollectAnimation)
    (if (Utilities|IsValid _puzzleref)
      (Default|OnPiecesCollected _puzzleref self))))

(event EventTick
  (params (DeltaSeconds :type Float%20%28single-precision%29))
  (bind _playerref (Variables|Default|GetPlayerRef))
  (if (Variables|Default|GetCanGo?)
    (bind _output_get (Variables|Default|SetDirection (Math|Vector|Normalize (- (Transformation|GetActorLocation (Game|GetPlayerCharacter 0)) (Transformation|GetActorLocation)))))
    (Transformation|SetActorLocation (+ (Transformation|GetActorLocation) (* (* _output_get (Variables|Default|GetFlySpeed)) (Variables|Default|GetDeltaSecond))) false false)
    (if (<= (Math|Vector|Distance(Vector) (Transformation|GetActorLocation (Game|GetPlayerCharacter 0)) (Transformation|GetActorLocation)) (Variables|Default|GetDisapearRange))
      (Utilities|FlowControl|DoOnce false
        (:Completed
          (CallFunction|StopReveal)
          (Utilities|Array|Clear (Variables|/Game/Game/Blueprints/Characters/Cidara/BP_PlayerCidara.BP_PlayerCidara_C|GetTargetActors _playerref))
          (Utilities|Array|Clear (Variables|/Game/Game/Blueprints/Characters/Cidara/BP_PlayerCidara.BP_PlayerCidara_C|GetMarkerWidgets _playerref))
          (Utilities|FlowControl|Delay 0.5)
          (Actor|DestroyActor))))))

(fn ConstructionScript
  (|CallParentFunction))