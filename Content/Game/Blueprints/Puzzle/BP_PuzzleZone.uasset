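; BP_PuzzleZone is a box-bounded puzzle area that registers itself as the Cidara player controller's current puzzle zone when the player enters.
; Exiting clears that link and signals the exit unless Spectre mode is on.
; Activate, deactivate and complete functions set the state and fire notifications, with completion also ending Spectre mode.
; A Tick check that would end Spectre mode when the Spectre leaves the box is disabled.
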(event OnComponentBeginOverlap(Box)
  (params (OverlappedComponent :type Primitive%20Component%20Object%20Reference) (OtherActor :type Actor%20Object%20Reference) (OtherComp :type Primitive%20Component%20Object%20Reference) (OtherBodyIndex :type Integer) (bFromSweep :type Boolean) (SweepResult :type Hit%20Result%20Structure%20%28by%20ref%29))
  (Utilities|Casting|CastToBP_PlayerCidara OtherActor)
  (Development|PrintString "Hello")
  (bind _aspc_cidara (Utilities|Casting|CastToPC_Cidara (Game|GetPlayerController 0)))
  (Variables|/Game/Game/Blueprints/Manager/PC_Cidara.PC_Cidara_C|SetCurrentPuzzleZone _aspc_cidara self)
  (Development|PrintString "YES"))

(event OnComponentEndOverlap(Box)
  (params (OverlappedComponent :type Primitive%20Component%20Object%20Reference) (OtherActor :type Actor%20Object%20Reference) (OtherComp :type Primitive%20Component%20Object%20Reference) (OtherBodyIndex :type Integer))
  (if (== OtherActor "/Game/Game/Blueprints/Characters/Cidara/BP_PlayerCidara.BP_PlayerCidara")
    (bind _aspc_cidara (Utilities|Casting|CastToPC_Cidara (Game|GetPlayerController 0)))
    (if (== (Variables|/Game/Game/Blueprints/Manager/PC_Cidara.PC_Cidara_C|GetCurrentPuzzleZone _aspc_cidara) self)
      (if (== (Variables|/Game/Game/Blueprints/Manager/PC_Cidara.PC_Cidara_C|GetInSpectreMode _aspc_cidara) false)
        (Variables|/Game/Game/Blueprints/Manager/PC_Cidara.PC_Cidara_C|SetCurrentPuzzleZone _aspc_cidara 0)
        (Default|CallOnPlayerExitedZone)))))

(event EventTick
  (params (DeltaSeconds :type Float%20%28single-precision%29))
  (if (Math|Boolean|ANDBoolean (Variables|Default|GetIsActive) (Utilities|IsValid (Variables|Components|GetSpectre)) false)
    (if (== (Collision|IsOverlappingActor (Variables|Default|GetBox) (Variables|Components|GetSpectre) :!class /Script/Engine.PrimitiveComponent) false)
      (bind _aspc_cidara (Utilities|Casting|CastToPC_Cidara (Game|GetPlayerController 0)))
      (Default|ExitSpectreMode _aspc_cidara))))

(event EventBeginPlay
  (bind _returnvalue (Actor|GetActorOfClass "/Game/Game/Blueprints/Characters/Spectre/BP_Spectre.BP_Spectre_C"))
  (Variables|Components|SetSpectre _returnvalue))

(fn ConstructionScript)

(fn ActivatePuzzleZone
  (bind _spectre (Variables|Components|GetSpectre))
  (Variables|Default|SetState "NewEnumerator2")
  (Variables|Default|SetIsActive true)
  (Default|CallOnSpectreActivated _spectre)
  (return _spectre))

(fn DeactivatePuzzleZone
  (Variables|Default|SetState "NewEnumerator1")
  (Variables|Default|SetIsActive false)
  (Default|CallOnSpectreDeactivated))

(fn CompletePuzzle
  (Variables|Default|SetState "NewEnumerator3")
  (Default|CallOnPuzzleCompleted)
  (bind _aspc_cidara (Utilities|Casting|CastToPC_Cidara (Game|GetPlayerController 0)))
  (Default|ExitSpectreMode _aspc_cidara))