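; Base puzzle actor that tracks a puzzle's state, ID and progress, with empty update and completion hooks, presumably for child puzzles.
; On BeginPlay it caches the Cidara game instance and loads those values from the save game's single Puzzle entry.
; Start, complete and reset events switch the state enum, with completion also firing the completed hook.
; Saving writes the values back and triggers the game instance save.
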(event Custom|ResetPuzzle
  (Variables|Default|SetPuzzleState "NewEnumerator0"))

(event Custom|StartPuzzle
  (Variables|Default|SetPuzzleState "NewEnumerator1"))

(event Custom|CompletePuzzle
  (Variables|Default|SetPuzzleState "NewEnumerator2")
  (CallFunction|OnPuzzleCompletedEvent))

(event Custom|OnPuzzleCompletedEvent)

(event EventBeginPlay
  (bind _asgi_cidara (Utilities|Casting|CastToGI_Cidara (Game|GetGameInstance)))
  (Variables|Default|SetGameInstanceRef _asgi_cidara)
  (CallFunction|LoadSaveData))

(event Collision|EventActorBeginOverlap
  (params (OtherActor :type Actor%20Object%20Reference)))

(event EventTick
  (params (DeltaSeconds :type Float%20%28single-precision%29)))

(event EventSaveGameData
  (CallFunction|CreateSaveData)
  (Default|SaveGameData (Variables|Default|GetGameInstanceRef)))

(fn ConstructionScript)

(fn LoadSaveData
  (bind _gameinstanceref (Variables|Default|GetGameInstanceRef))
  (bind _save_game_ref (Variables|/Game/Game/Blueprints/Manager/GI_Cidara.GI_Cidara_C|GetSave%20Game%20Ref _gameinstanceref))
  (bind _puzzle (Variables|/Game/Game/Blueprints/Manager/SaveSystem/BP_SaveGame.BP_SaveGame_C|GetPuzzle _save_game_ref))
  (bind (_state _puzzleid _progress) (Utilities|Struct|BreakS_PuzzleSaveData _puzzle))
  (Variables|Default|SetPuzzleState _state)
  (Variables|Default|SetPuzzleId _puzzleid)
  (Variables|Default|SetProgress _progress)
  (return))

(fn CreateSaveData
  (|SetBy-RefVar (Variables|/Game/Game/Blueprints/Manager/SaveSystem/BP_SaveGame.BP_SaveGame_C|GetPuzzle (Variables|/Game/Game/Blueprints/Manager/GI_Cidara.GI_Cidara_C|GetSave%20Game%20Ref (Variables|Default|GetGameInstanceRef))) (Utilities|Struct|MakeS_PuzzleSaveData (Variables|Default|GetPuzzleState) (Variables|Default|GetPuzzleId) (Variables|Default|GetProgress) ""))
  (return))

(fn UpdatePuzzle)

(fn GetPuzzleId
  (params (PuzzleId :type Name))
  (bind _output_get (Variables|Default|SetPuzzleId PuzzleId))
  (return _output_get))

(fn GetInitialState
  (return "NewEnumerator0"))

(fn GetPuzzleName
  (params (PuzzleId :type Name :default "None"))
  (return "None"))