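; Game Instance for Cidara that manages save games, puzzle state and narrative collectible progress.
; Puzzles register by ID through BPI_Puzzle; state changes and slot loads push states to them, stashing pending states for unregistered ones.
; AutoSave rotates through slots on puzzle state changes, though SaveToSlot writes SaveGameRef instead of the save object it fills.
; Collectible fragments are counted toward required totals, with completion calling an empty TriggerEcho stub.
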(event EventSaveGameData
  (SaveGame|SaveGametoSlot (Variables|Default|GetSave%20Game%20Ref) (Variables|Default|GetGameSlotName)))

(event EventLoadGameData
  (bind _returnvalue (SaveGame|DoesSaveGameExist (Variables|Default|GetGameSlotName)))
  (if _returnvalue
    (Variables|Default|SetShouldLoad? true)
    (bind _returnvalue_2 (SaveGame|LoadGamefromSlot (Variables|Default|GetGameSlotName)))
    (bind _asbp_save_game (Utilities|Casting|CastToBP_SaveGame _returnvalue_2))
    (Variables|Default|SetSave%20Game%20Ref _asbp_save_game)
    (else
      (bind _returnvalue_3 (SaveGame|CreateSaveGameObject "/Game/Game/Blueprints/Manager/SaveSystem/BP_SaveGame.BP_SaveGame_C"))
      (Variables|Default|SetSave%20Game%20Ref _returnvalue_3))))

(event EventInit
  (CallFunction|LoadGameData))

(fn SaveAllPuzzle
  (bind _gameslotname (Variables|Default|GetGameSlotName))
  (bind _returnvalue (SaveGame|CreateSaveGameObject "/Game/Game/Blueprints/Manager/SaveSystem/BP_SaveGame.BP_SaveGame_C"))
  (bind _output_get (LocalVariables|SetSaveGameL _returnvalue))
  (bind _keys (Utilities|Map|Keys (Variables|/Game/Game/Blueprints/Manager/SaveSystem/BP_SaveGame.BP_SaveGame_C|GetPuzzleState _output_get)))
  (for _array_element _keys
    (Utilities|Map|Add (Variables|Default|GetPendingSaveStates) _array_element (.Value (Utilities|Map|Find (Variables|/Game/Game/Blueprints/Manager/SaveSystem/BP_SaveGame.BP_SaveGame_C|GetPuzzleState _output_get) _array_element))))
  (bind _returnvalue_2 (SaveGame|SaveGametoSlot (LocalVariables|GetSaveGameL) _gameslotname))
  (if _returnvalue_2
    (Development|PrintString "SaveAllPuzzleOK")
    (else
      (Development|PrintString "Save ALl puzzle fail")))
  (Development|PrintString _gameslotname))

(fn GetPuzzleState
  (params (PuzzleId :type Name))
  (if (Utilities|Map|Contains (Variables|Default|GetRegisterPuzzleData) PuzzleId)
    (return (.Value (Utilities|Map|Find (Variables|Default|GetPendingSaveStates) PuzzleId)))
    (else
      (return "NewEnumerator0"))))

(fn LoadAllPuzzle
  (bind _returnvalue (SaveGame|DoesSaveGameExist (Variables|Default|GetGameSlotName)))
  (if _returnvalue
    (bind _returnvalue_2 (SaveGame|LoadGamefromSlot (Variables|Default|GetGameSlotName)))
    (bind _asbp_save_game (Utilities|Casting|CastToBP_SaveGame _returnvalue_2))
    (bind _output_get (LocalVariables|SetSaveGameL _asbp_save_game))
    (bind _keys (Utilities|Map|Keys (Variables|/Game/Game/Blueprints/Manager/SaveSystem/BP_SaveGame.BP_SaveGame_C|GetPuzzleState _output_get)))
    (for _array_element _keys
      (Utilities|Map|Add (Variables|Default|GetPendingSaveStates) _array_element (.Value (Utilities|Map|Find (Variables|/Game/Game/Blueprints/Manager/SaveSystem/BP_SaveGame.BP_SaveGame_C|GetPuzzleState _output_get) _array_element)))
      (if (Utilities|Map|Contains (Variables|Default|GetRegisterPuzzleInstance) _array_element)
        (Default|ApplyStatefromManager (.Value (Utilities|Map|Find (Variables|Default|GetRegisterPuzzleInstance) _array_element)) (.Value (Utilities|Map|Find (Variables|/Game/Game/Blueprints/Manager/SaveSystem/BP_SaveGame.BP_SaveGame_C|GetPuzzleState _output_get) _array_element)))
        (else
          (Utilities|Map|Add (Variables|Default|GetPendingSaveStates) _array_element (.Value (Utilities|Map|Find (Variables|/Game/Game/Blueprints/Manager/SaveSystem/BP_SaveGame.BP_SaveGame_C|GetPuzzleState _output_get) _array_element))))))
    (else
      (Utilities|Map|Clear (Variables|Default|GetPendingSaveStates))
      (Development|PrintString "NoSaveFound")
      (return))))

(fn SavetoSlot
  (params (SlotName :type String))
  (if (Utilities|Array|IsEmpty SlotName)
    (LocalVariables|SetLSlotName (Variables|Default|GetGameSlotName))
    (else
      (LocalVariables|SetLSlotName SlotName)))
  (bind _returnvalue (SaveGame|CreateSaveGameObject "/Game/Game/Blueprints/Manager/SaveSystem/BP_SaveGame.BP_SaveGame_C"))
  (bind _output_get (LocalVariables|SetSG _returnvalue))
  (bind _keys (Utilities|Map|Keys (Variables|Default|GetRegisterPuzzleData)))
  (for _array_element _keys
    (Utilities|Map|Add (Variables|/Game/Game/Blueprints/Manager/SaveSystem/BP_SaveGame.BP_SaveGame_C|GetPuzzleState _output_get) _array_element (.State (Utilities|Struct|BreakS_PuzzleSaveData (.Value (Utilities|Map|Find (Variables|Default|GetRegisterPuzzleData) _array_element))))))
  (bind _returnvalue_2 (SaveGame|SaveGametoSlot (Variables|Default|GetSave%20Game%20Ref) (LocalVariables|GetLSlotName)))
  (if _returnvalue_2
    (Development|PrintString "Save OK")
    (Development|PrintString (LocalVariables|GetLSlotName))
    (return)
    (else
      (Development|PrintString "SAve FAiled")
      (Development|PrintString (LocalVariables|GetLSlotName))
      (return))))

(fn LoadfromSlot
  (params (SlotName :type String))
  (if (Utilities|Array|IsEmpty SlotName)
    (LocalVariables|SetLSlotName (Variables|Default|GetGameSlotName))
    (else
      (LocalVariables|SetLSlotName SlotName)))
  (bind _returnvalue (SaveGame|DoesSaveGameExist (LocalVariables|GetLSlotName)))
  (if _returnvalue
    (bind _returnvalue_2 (SaveGame|LoadGamefromSlot (LocalVariables|GetLSlotName)))
    (bind _asbp_save_game (Utilities|Casting|CastToBP_SaveGame _returnvalue_2))
    (bind _output_get (LocalVariables|SetSG _asbp_save_game))
    (bind _keys (Utilities|Map|Keys (Variables|/Game/Game/Blueprints/Manager/SaveSystem/BP_SaveGame.BP_SaveGame_C|GetPuzzleState _output_get)))
    (for _array_element _keys
      (if (Utilities|Map|Contains (Variables|Default|GetRegisterPuzzleData) _array_element)
        (Puzzle|SetPuzzleState _array_element (.Value (Utilities|Map|Find (Variables|/Game/Game/Blueprints/Manager/SaveSystem/BP_SaveGame.BP_SaveGame_C|GetPuzzleState _output_get) _array_element)) false)
        (else
          (Utilities|Map|Add (Variables|Default|GetPendingSaveStates) _array_element (.Value (Utilities|Map|Find (Variables|/Game/Game/Blueprints/Manager/SaveSystem/BP_SaveGame.BP_SaveGame_C|GetPuzzleState _output_get) _array_element)))
          (Development|PrintString "LoadFromSlot: Stashed")
          (Development|PrintString (Utilities|String|ToString(Name) _array_element)))))
    (Development|PrintString "Load complete")
    (Development|PrintString (LocalVariables|GetLSlotName))
    (return)
    (else
      (Development|PrintString "NoSave")
      (return))))

(fn SetPuzzleState
  (params (PuzzleId :type Name) (NewState :type E_PuzzleState%20Enum :default "NewEnumerator0") (FromPuzzle? :type Boolean))
  (bind _registerpuzzledata (Variables|Default|GetRegisterPuzzleData))
  (Development|PrintString (Utilities|String|ToString(Name) PuzzleId))
  (LocalVariables|SetLPuzzleId PuzzleId)
  (LocalVariables|SetLNewState NewState)
  (if (Utilities|Map|Contains _registerpuzzledata (LocalVariables|GetLPuzzleId))
    (bind _structout (Utilities|Struct|SetmembersinS_PuzzleSaveData (.Value (Utilities|Map|Find _registerpuzzledata (LocalVariables|GetLPuzzleId)))))
    (Utilities|Map|Add (Variables|Default|GetRegisterPuzzleData) (LocalVariables|GetLPuzzleId) _structout)
    (if (and (Variables|Default|GetAutoSaveCompleted?) (Utilities|Enum|Equal(Enum) (LocalVariables|GetLNewState) "NewEnumerator2"))
      (Default|ApplyStatefromManager (.Value (Utilities|Map|Find (Variables|Default|GetRegisterPuzzleInstance) (LocalVariables|GetLPuzzleId))) (LocalVariables|GetLNewState))
      (Development|PrintString (Utilities|String|EnumtoString (LocalVariables|GetLNewState)))
      (Save|AutoSave)
      (return))
    (else
      (Utilities|Map|Add (Variables|Default|GetPendingSaveStates) (LocalVariables|GetLPuzzleId) (LocalVariables|GetLNewState))
      (if (Utilities|Map|Contains (Variables|Default|GetRegisterPuzzleInstance) (LocalVariables|GetLPuzzleId))
        (Default|ApplyStatefromManager (.Value (Utilities|Map|Find (Variables|Default|GetRegisterPuzzleInstance) (LocalVariables|GetLPuzzleId))) (LocalVariables|GetLNewState))
        (Default|CallOnPuzzleStateChanged (LocalVariables|GetLPuzzleId) (LocalVariables|GetLNewState))
        (if (and (Variables|Default|GetAutoSaveCompleted?) (and (Utilities|Enum|Equal(Enum) (LocalVariables|GetLNewState) "NewEnumerator2") FromPuzzle?))
          (Save|AutoSave)
          (Development|PrintString "SetPuzzleState")
          (Development|PrintString (Utilities|String|ToString(Name) (LocalVariables|GetLPuzzleId)))
          (Development|PrintString (Utilities|String|EnumtoString (LocalVariables|GetLNewState)))
          (return))))))

(fn AutoSave
  (Save|SavetoSlot (Utilities|Array|Get(acopy) (Variables|Default|GetAutoSaveSlot) (Variables|Default|GetAutoSaveIndex)))
  (Variables|Default|SetAutoSaveIndex (Math|Integer|%(Integer) (+ (Variables|Default|GetAutoSaveIndex) 1) (Utilities|Array|Length (Variables|Default|GetAutoSaveSlot))))
  (return))

(fn UnregisterPuzzle
  (params (PuzzleActor :type BP%20Puzzle%20Base%20Object%20Reference))
  (if (Utilities|IsValid PuzzleActor)
    (if (Utilities|DoesObjectImplementInterface PuzzleActor "/Game/Game/Blueprints/Interface/BPI_Puzzle.BPI_Puzzle_C")
      (bind _name (Default|GetPuzzleName PuzzleActor "None"))
      (Utilities|Map|Remove (Variables|Default|GetRegisterPuzzleInstance) _name)
      (return))))

(fn RegisterPuzzle
  (params (PuzzleRef :type BP%20Puzzle%20Base%20Object%20Reference))
  (bind _output_get (LocalVariables|SetLPuzzleRef PuzzleRef))
  (if (Utilities|IsValid _output_get)
    (if (Utilities|DoesObjectImplementInterface _output_get "/Game/Game/Blueprints/Interface/BPI_Puzzle.BPI_Puzzle_C")
      (bind _name (Default|GetPuzzleName (LocalVariables|GetLPuzzleRef) (Variables|/Game/Game/Blueprints/Puzzle/PuzzleSystemBase/BP_PuzzleBase.BP_PuzzleBase_C|GetPuzzleId (LocalVariables|GetLPuzzleRef))))
      (bind _output_get_2 (LocalVariables|SetLPuzzleId _name))
      (if (or (== _output_get_2 "") (== _output_get_2 ""))
        (Development|PrintString "RegisterPuzzle : Empty ID")
        (return)
        (elif (not (Utilities|Map|Contains (Variables|Default|GetRegisterPuzzleData) (LocalVariables|GetLPuzzleId)))
          (Utilities|Map|Add (Variables|Default|GetRegisterPuzzleData) (LocalVariables|GetLPuzzleId) (Utilities|Struct|MakeS_PuzzleSaveData "NewEnumerator0" (LocalVariables|GetLPuzzleId)))
          (Utilities|Map|Add (Variables|Default|GetRegisterPuzzleInstance) (LocalVariables|GetLPuzzleId) (LocalVariables|GetLPuzzleRef))
          (if (Utilities|Map|Contains (Variables|Default|GetPendingSaveStates) (LocalVariables|GetLPuzzleId))
            (CallFunction|ApplyStatefromManager (.State (Utilities|Struct|BreakS_PuzzleSaveData (.Value (Utilities|Map|Find (Variables|Default|GetRegisterPuzzleData) (LocalVariables|GetLPuzzleId))))))
            (else
              (bind _structout (Utilities|Struct|SetmembersinS_PuzzleSaveData (.Value (Utilities|Map|Find (Variables|Default|GetRegisterPuzzleData) (LocalVariables|GetLPuzzleId))) (.Value (Utilities|Map|Find (Variables|Default|GetPendingSaveStates) (LocalVariables|GetLPuzzleId)))))
              (Utilities|Map|Add (Variables|Default|GetRegisterPuzzleData) (LocalVariables|GetLPuzzleId) _structout)
              (Default|ApplyStatefromManager (LocalVariables|GetLPuzzleRef) (.Value (Utilities|Map|Find (Variables|Default|GetPendingSaveStates) (LocalVariables|GetLPuzzleId))))
              (Utilities|Map|Remove (Variables|Default|GetPendingSaveStates) (LocalVariables|GetLPuzzleId))
              (Development|PrintString "Hello")
              (return)))))
      (else
        (Development|PrintString "RegisterPuzzle : Missing interface")
        (return)))
    (else
      (Development|PrintString "RegisterPuzzle : Invalid actor")
      (return))))

(fn RegisterFragementCollected
  (params (CollectibleID :type Name))
  (bind _collectiblesstate (Variables|Default|GetCollectiblesState))
  (bind (_value _returnvalue) (Utilities|Map|Find _collectiblesstate CollectibleID))
  (bind (_collectibleid _fragmentcollected _fragmentrequired) (Utilities|Struct|BreakS_NarrativeCollectiblesState _value))
  (if _returnvalue
    (bind _result (Math|Integer|IncrementInt _fragmentcollected)
      (:%20%20
        (if (>= (.fragmentcollected (Utilities|Struct|MakeS_NarrativeCollectiblesState _collectibleid _result _fragmentrequired false)) (.fragmentrequired (Utilities|Struct|MakeS_NarrativeCollectiblesState _collectibleid _result _fragmentrequired false)))
          (Utilities|Map|Add (Variables|Default|GetCollectiblesState) CollectibleID (Utilities|Struct|MakeS_NarrativeCollectiblesState CollectibleID (.fragmentcollected (Utilities|Struct|MakeS_NarrativeCollectiblesState _collectibleid _result _fragmentrequired false)) (.fragmentrequired (Utilities|Struct|MakeS_NarrativeCollectiblesState _collectibleid _result _fragmentrequired false)) true))
          (Collectibles|TriggerEcho CollectibleID)
          (return)
          (else
            (Utilities|Map|Add (Variables|Default|GetCollectiblesState) CollectibleID (Utilities|Struct|MakeS_NarrativeCollectiblesState (.collectibleid (Utilities|Struct|MakeS_NarrativeCollectiblesState _collectibleid _result _fragmentrequired false)) (.fragmentcollected (Utilities|Struct|MakeS_NarrativeCollectiblesState _collectibleid _result _fragmentrequired false)) (.fragmentrequired (Utilities|Struct|MakeS_NarrativeCollectiblesState _collectibleid _result _fragmentrequired false)) false))
            (return)))))))

(fn RegisterCollectiblePlan
  (params (CollectibleID :type Name) (FragmentsRequired :type Integer))
  (if (Utilities|Map|Contains (Variables|Default|GetCollectiblesState) CollectibleID)
    (return)
    (else
      (Utilities|Map|Add (Variables|Default|GetCollectiblesState) CollectibleID (Utilities|Struct|MakeS_NarrativeCollectiblesState CollectibleID 0 FragmentsRequired false))
      (return))))

(fn TriggerEcho
  (params (CollectibleID :type Name)))

(fn GetInitialState
  (return "NewEnumerator0"))

(fn GetPuzzleName
  (params (PuzzleId :type Name :default "None"))
  (return "None"))