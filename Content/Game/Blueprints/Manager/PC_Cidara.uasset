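; Player controller that switches control between Cidara and a Spectre while a current puzzle zone is set.
; Switch input activates the zone and possesses the Spectre it returns; cancel repossesses Cidara and deactivates the zone.
; Each switch swaps Enhanced Input contexts and resets the view target after possession for an eased camera blend between Cidara and the zone.
; Helper functions add or remove both mapping contexts together.
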(event Input|EnhancedActionEvents|EnhancedInputActionIA_SwitchCidaraSpectre
  (params (ActionValue :type Boolean) (ElapsedSeconds :type Float%20%28double-precision%29) (TriggeredSeconds :type Float%20%28double-precision%29) (InputAction :type Input%20Action%20Object%20Reference :default "/Game/Game/Input/Actions/IA_SwitchCidaraSpectre.IA_SwitchCidaraSpectre"))
  (if (and (not (Variables|Default|GetInSpectreMode)) (Utilities|IsValid (Variables|Default|GetCurrentPuzzleZone)))
    (CallFunction|EnterSpectreMode)))

(event Input|EnhancedActionEvents|EnhancedInputActionIA_SpectreCancel
  (params (ActionValue :type Boolean) (ElapsedSeconds :type Float%20%28double-precision%29) (TriggeredSeconds :type Float%20%28double-precision%29) (InputAction :type Input%20Action%20Object%20Reference :default "/Game/Game/Input/Actions/Spectre/IA_SpectreCancel.IA_SpectreCancel"))
  (if (Variables|Default|GetInSpectreMode)
    (CallFunction|ExitSpectreMode)))

(event EventBeginPlay
  (Utilities|FlowControl|Sequence
    (:then_0
      (bind _asbp_player_cidara (Utilities|Casting|CastToBP_PlayerCidara (Pawn|GetControlledPawn)))
      (Variables|Default|SetCidaraRef _asbp_player_cidara)
      (Input|AddMappingContext (PlayerController|LocalPlayerSubsystems|GetEnhancedInputLocalPlayerSubsystem) "/Game/Game/Input/IMC_Cidara.IMC_Cidara" 0 "(bIgnoreAllPressedKeysUntilRelease=True,bForceImmediately=False,bNotifyUserSettings=False)"))
    (:then_1
      (bind _returnvalue (Actor|GetActorOfClass "/Game/Game/Blueprints/Characters/Spectre/BP_Spectre.BP_Spectre_C"))
      (Variables|Default|SetSpectre _returnvalue))))

(fn ConstructionScript)

(fn SwapMappingContext
  (params (IMC%20To%20Add :type Input%20Mapping%20Context%20Object%20Reference) (IMC%20To%20Remove :type Input%20Mapping%20Context%20Object%20Reference))
  (bind _returnvalue (PlayerController|LocalPlayerSubsystems|GetEnhancedInputLocalPlayerSubsystem))
  (Input|RemoveMappingContext _returnvalue IMC%20To%20Remove "(bIgnoreAllPressedKeysUntilRelease=True,bForceImmediately=False,bNotifyUserSettings=False)")
  (Input|AddMappingContext _returnvalue IMC%20To%20Add 0 "(bIgnoreAllPressedKeysUntilRelease=True,bForceImmediately=False,bNotifyUserSettings=False)"))

(fn ExitSpectreMode
  (if (Variables|Default|GetInSpectreMode)
    (Pawn|Possess (Variables|Default|GetCidaraRef))
    (Game|Player|SetViewTargetwithBlend (Variables|Default|GetCurrentPuzzleZone) 0.0 "VTBlend_Linear" 0.0 false)
    (Game|Player|SetViewTargetwithBlend (Variables|Default|GetCidaraRef) 1.2 "VTBlend_EaseInOut" 2.0 true)
    (CallFunction|SwapMappingContext "/Game/Game/Input/IMC_Cidara.IMC_Cidara" "/Game/Game/Input/IMC_Spectre.IMC_Spectre")
    (Default|DeactivatePuzzleZone (Variables|Default|GetCurrentPuzzleZone))
    (Variables|Default|SetInSpectreMode false)))

(fn EnterSpectreMode
  (bind _currentpuzzlezone (Variables|Default|GetCurrentPuzzleZone))
  (if (Utilities|IsValid _currentpuzzlezone)
    (bind _spectre (Default|ActivatePuzzleZone _currentpuzzlezone))
    (bind _output_get (Variables|Default|SetSpectre _spectre))
    (Pawn|Possess _output_get)
    (Game|Player|SetViewTargetwithBlend (Variables|Default|GetCidaraRef) 0.0 "VTBlend_Linear" 0.0 false)
    (Game|Player|SetViewTargetwithBlend (Variables|Default|GetCurrentPuzzleZone) 1.2 "VTBlend_EaseInOut" 2.0 true)
    (CallFunction|SwapMappingContext "/Game/Game/Input/IMC_Spectre.IMC_Spectre" "/Game/Game/Input/IMC_Cidara.IMC_Cidara")
    (Variables|Default|SetInSpectreMode true)))

(fn RemoveMapping
  (bind _returnvalue (PlayerController|LocalPlayerSubsystems|GetEnhancedInputLocalPlayerSubsystem))
  (Input|RemoveMappingContext _returnvalue "/Game/Game/Input/IMC_Spectre.IMC_Spectre" "(bIgnoreAllPressedKeysUntilRelease=True,bForceImmediately=False,bNotifyUserSettings=False)")
  (Input|RemoveMappingContext _returnvalue "/Game/Game/Input/IMC_Cidara.IMC_Cidara" (Utilities|Struct|MakeModifyContextOptions true false false)))

(fn AddMapping
  (bind _returnvalue (PlayerController|LocalPlayerSubsystems|GetEnhancedInputLocalPlayerSubsystem))
  (Input|AddMappingContext _returnvalue "/Game/Game/Input/IMC_Cidara.IMC_Cidara" 1 (Utilities|Struct|MakeModifyContextOptions true true false))
  (Development|PrintString (Utilities|GetDisplayName _returnvalue))
  (Input|AddMappingContext _returnvalue "/Game/Game/Input/IMC_Spectre.IMC_Spectre" 0 "(bIgnoreAllPressedKeysUntilRelease=True,bForceImmediately=False,bNotifyUserSettings=False)"))