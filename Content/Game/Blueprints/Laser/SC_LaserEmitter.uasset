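; Scene component that emits an outgoing laser from its owner when the owner is hit by one, or the reverse when the system is inverted.
; It caches the owner's BPC_LaserHandler, then spawns and attaches a BP_Laser carrying range, color and previous-laser chain, with the last laser as Owner.
; Deactivation calls LaserStopHitting on the attached laser.
; Parallel functions handle a BP_CidaraLaser variant, with no callers here.
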(event EventBeginPlay
  (bind _returnvalue (Components|GetOwner))
  (bind _returnvalue_2 (Actor|GetComponentbyClass _returnvalue "/Game/Game/Blueprints/Laser/BPC_LaserHandler.BPC_LaserHandler_C"))
  (Utilities|IsValid _returnvalue_2
    (:Is%20Valid
      (Variables|Default|SetOwningHandler _returnvalue_2))))

(event EventLaserStartHitting
  (params (Input :type BP%20Laser%20Object%20Reference) (Hit%20info :type Hit%20Result%20Structure))
  (if (Utilities|IsSystemInverted)
    (CallFunction|DesactivateLaser)
    (else
      (CallFunction|ActivateLaser))))

(event EventLaserStopHitting
  (params (Input :type BP%20Laser%20Object%20Reference))
  (if (Utilities|IsSystemInverted)
    (CallFunction|ActivateLaser)
    (else
      (CallFunction|DesactivateLaser))))

(fn ActivateLaser
  (bind _outputpin (Utilities|GetFilteredLasers))
  (if (Utilities|Array|IsNotEmpty _outputpin)
    _
    (else
      _))
  (bind _returnvalue (Game|SpawnActorfromClass "/Game/Game/Blueprints/Laser/BP_Laser.BP_Laser_C" (Transformation|GetWorldTransform) "Undefined" "OverrideRootScale" (Utilities|Array|Get(acopy) _outputpin (Utilities|Array|LastIndex _outputpin)) (Variables|Default|GetMaxRange) (Utilities|GetFilteredLasers) (Variables|Default|GetOwningHandler) (Variables|Default|GetCurrentColor) (Utilities|Array|MakeArray (Components|GetOwner)) 0))
  (bind _output_get (Variables|Default|SetAttachedLaser _returnvalue))
  (Transformation|AttachComponentToComponent _output_get self "None" "KeepWorld" "KeepWorld" "KeepWorld" false))

(fn DesactivateLaser
  (bind _attachedlaser (Variables|Default|GetAttachedLaser)
    (:then
      (Default|LaserStopHitting _attachedlaser))
    (:else)))

(fn OnRepOwningHandler)

(fn ActivateCidaraLaser
  (bind _outputpin (Utilities|GetFilteredLasers))
  (if (Utilities|Array|IsNotEmpty _outputpin)
    _
    (else
      _))
  (bind _returnvalue (Game|SpawnActorfromClass "/Game/Game/Blueprints/Laser/BP_CidaraLaser.BP_CidaraLaser_C" (Transformation|GetWorldTransform) "Undefined" "OverrideRootScale" (Utilities|Array|Get(acopy) _outputpin (Utilities|Array|LastIndex _outputpin)) (Variables|Default|GetMaxRange) (Utilities|GetFilteredLasers) (Variables|Default|GetOwningHandler) (Variables|Default|GetCurrentColor) (Utilities|Array|MakeArray (Components|GetOwner)) 0))
  (bind _output_get (Variables|Default|SetAttachedLaser _returnvalue))
  (Transformation|AttachComponentToComponent _output_get self "None" "KeepWorld" "KeepWorld" "KeepWorld" false))

(fn DesactivateCidaraLaser
  (bind _attachedlaser (Variables|Default|GetAttachedLaser)
    (:then
      (Default|LaserStopHitting _attachedlaser))
    (:else)))