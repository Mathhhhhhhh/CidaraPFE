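; BP_Laser is a laser beam actor that stretches its mesh to blocking hits and notifies the BPC_Handler components it hits.
; Each tick it multi-traces forward, diffing current and previous handler sets to send start, update and stop messages.
; A recursive check through PreviousLasers skips handlers owning upstream lasers, preventing loops in laser chains.
; LaserStopHitting notifies previously hit handlers, then destroys the actor.
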(event EventBeginPlay
  (bind _returnvalue (Rendering|Material|CreateDynamicMaterialInstance "/Game/Game/Materials/Laser/MI_Laser.MI_Laser" "None" "None" :!class /Script/Engine.KismetMaterialLibrary))
  (Variables|Default|SetMaterial%20Instance _returnvalue)
  (Rendering|Material|SetMaterial (Variables|Default|GetLaser_Mesh) 0 (Variables|Default|GetMaterial%20Instance))
  (CallFunction|ChangeLaserColor (Variables|Exposed|GetColor%20Override)))

(event EventTick
  (params (DeltaSeconds :type Float%20%28single-precision%29))
  (bind _returnvalue (Transformation|GetActorLocation))
  (bind (_outhits _returnvalue_2) (Collision|MultiLineTraceByChannel _returnvalue (+ _returnvalue (* (Transformation|GetActorForwardVector) (Variables|Exposed|GetRange))) "TraceTypeQuery3" false (Variables|Exposed|GetActors%20To%20Ignore) "ForOneFrame"))
  (if _returnvalue_2
    (for _array_element _outhits
      (Utilities|FlowControl|Sequence
        (:then_0
          (if (.bBlockingHit (Collision|BreakHitResult _array_element))
            (CallFunction|UpdateLenght (.Distance (Collision|BreakHitResult _array_element)))))
        (:then_1
          (CallFunction|HandleHitActors _array_element))))
    (bind _result (Utilities|Set|Difference (Variables|Default|GetPreviously%20Hit%20Handlers) (Variables|Default|GetCurrent%20Hit%20Handlers)))
    (bind _result_2 (Utilities|Set|ToArray _result))
    (for _array_element_2 _result_2
      (Class|BPILasers|LaserStopHitting(Message) _array_element_2 self)
      (Utilities|Map|Remove (Variables|Exposed|GetHitting%20Handlers) _array_element_2))
    (Variables|Default|SetPreviously%20Hit%20Handlers (Variables|Default|GetCurrent%20Hit%20Handlers))
    (Utilities|Set|Clear (Variables|Default|GetCurrent%20Hit%20Handlers))))

(event EventLaserStopHitting
  (params (Input :type BP%20Laser%20Object%20Reference))
  (Utilities|FlowControl|Sequence
    (:then_0
      (bind _result (Utilities|Set|ToArray (Variables|Default|GetPreviously%20Hit%20Handlers)))
      (for _array_element _result
        (Class|BPILasers|LaserStopHitting(Message) _array_element self)))
    (:then_1
      (Actor|DestroyActor))))

(fn ConstructionScript)

(fn ChangeLaserColor
  (params (Value :type Linear%20Color%20Structure))
  (Rendering|Material|SetVectorParameterValue (Variables|Default|GetMaterial%20Instance) "None" Value :!class /Script/Engine.MaterialInstanceDynamic))

(fn UpdateLenght
  (params (InputPin :type Float%20%28single-precision%29))
  (if (not (Math|Float|NearlyEqual(Float) InputPin (Variables|Exposed|GetPrevious%20Lenght) 2.0))
    (bind _output_get (Variables|Exposed|SetPrevious%20Lenght InputPin))
    (Transformation|SetWorldScale3D (Variables|Default|GetLaser_Mesh) (Math|Vector|MakeVector 0.1 0.1 (/ _output_get 1e+02)))))

(fn HandleHitActors
  (params (InputPin :type Hit%20Result%20Structure))
  (bind _hitactor (Collision|BreakHitResult InputPin))
  (bind _returnvalue (Actor|GetComponentbyClass _hitactor "/Game/Game/Blueprints/Laser/BPC_Handler.BPC_Handler_C"))
  (Utilities|IsValid _returnvalue
    (:Is%20Valid
      (LocalVariables|SetL-Handler _returnvalue)
      (if (CallFunction|IsNotonPath (LocalVariables|GetL-Handler))
        (Utilities|Map|Add (Variables|Exposed|GetHitting%20Handlers) (LocalVariables|GetL-Handler) InputPin)
        (if (Utilities|Set|Contains (Variables|Default|GetPreviously%20Hit%20Handlers) (LocalVariables|GetL-Handler))
          (Default|LaserUpdateHitting (LocalVariables|GetL-Handler) self InputPin)
          (else
            (Class|BPILasers|LaserStartHitting(Message) (LocalVariables|GetL-Handler) self InputPin)))
        (Utilities|Set|Add (Variables|Default|GetCurrent%20Hit%20Handlers) (LocalVariables|GetL-Handler))))))

(fn IsNotonPath
  (params (Input%20Handler :type Actor%20Component%20Object%20Reference))
  (if (Utilities|Array|IsNotEmpty (Variables|Exposed|GetPrevious_Lasers))
    (for _array_element (Variables|Exposed|GetPrevious_Lasers)
      (bind _output_get (LocalVariables|SetL-CurrentLaser _array_element))
      (if (== (Variables|BP_Laser_C|GetOwning%20Handler _output_get) Input%20Handler)
        (return false)
        (elif (not (CallFunction|IsNotonPath (LocalVariables|GetL-CurrentLaser) Input%20Handler))
          (return false))))
    (return true)
    (else
      (return true))))