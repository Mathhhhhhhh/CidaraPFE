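; BP_CidaraLaser is a laser actor that line-traces forward every tick and tracks the handlers it hits.
; A blocking hit updates the laser's length, and every hit is passed to HandleHitActors.
; A set difference between previous and current handlers finds those the beam has left and sends them a stop-hitting message.
; LaserStopHitting sends that message to all previously hit handlers, then destroys the laser.
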(event EventBeginPlay
  (|CallParentFunction) ; This node is disabled and will not be called.\nDrag off pins to build functionality.
)

(event EventTick
  (params (DeltaSeconds :type Float%20%28single-precision%29))
  (bind _returnvalue (Transformation|GetActorLocation))
  (bind (_outhits _returnvalue_2) (Collision|MultiLineTraceByChannel _returnvalue (+ _returnvalue (* (Transformation|GetActorForwardVector) (Variables|Default|GetRange))) "TraceTypeQuery3" false (Variables|Default|GetActors%20To%20Ignore) "None"))
  ;[0.15 0.15 0.15 0.5] ICI capte si laser hit qqc
  (if _returnvalue_2
    (for _array_element _outhits
      (Utilities|FlowControl|Sequence
        (:then_0
          (if (.bBlockingHit (Collision|BreakHitResult _array_element))
            (CallFunction|UpdateLenght (.Distance (Collision|BreakHitResult _array_element)))))
        (:then_1
          (CallFunction|HandleHitActors _array_element))))
    (bind _result (Utilities|Set|Difference (Variables|Default|GetPreviously%20Hit%20Handlers) (Variables|Default|GetCurrent%20Hit%20Handlers)))
    (bind _result_2 (Utilities|Set|ToArray _result))
    (for _array_element_2 _result_2
      (Class|BPILasers|LaserStopHitting(Message) _array_element_2 self)
      (Utilities|Map|Remove (Variables|Default|GetHitting%20Handlers) _array_element_2))
    (Variables|Default|SetPreviously%20Hit%20Handlers (Variables|Default|GetCurrent%20Hit%20Handlers))
    (Utilities|Set|Clear (Variables|Default|GetCurrent%20Hit%20Handlers))))

(event EventLaserStopHitting
  (params (Input :type BP%20Laser%20Object%20Reference))
  (Utilities|FlowControl|Sequence
    (:then_0
      (bind _result (Utilities|Set|ToArray (Variables|Default|GetPreviously%20Hit%20Handlers)))
      (for _array_element _result
        (Class|BPILasers|LaserStopHitting(Message) _array_element self)))
    (:then_1
      (Actor|DestroyActor))))

(event Collision|EventActorBeginOverlap
  (params (OtherActor :type Actor%20Object%20Reference)))

(fn ConstructionScript
  (|CallParentFunction))