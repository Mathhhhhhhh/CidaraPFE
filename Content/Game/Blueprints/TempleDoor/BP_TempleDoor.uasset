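; BP_TempleDoor is a temple door actor that slides from a start point to an end point when interacted with.
; BeginPlay caches the world locations of its Start and End components, so the targets stay fixed as the actor moves.
; Interract calls ActivateElevator, which plays the Tl_MoveUp timeline to lerp the actor between those locations with sweep enabled.
; The graph has no reverse or closing logic.
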(event Custom|ActivateElevator
  (bind _alpha (Timeline|Tl_MoveUp Play)
    (:Update
      (Transformation|SetActorLocation (Math|Vector|Lerp(Vector) (Variables|Default|GetStartLocation) (Variables|Default|GetEndLocation) _alpha) true false))))

(event EventBeginPlay
  (Variables|Default|SetStartLocation (Transformation|GetWorldLocation (Variables|Default|GetStart)))
  (Variables|Default|SetEndLocation (Transformation|GetWorldLocation (Variables|Default|GetEnd))))

(event Collision|EventActorBeginOverlap
  (params (OtherActor :type Actor%20Object%20Reference)))

(event EventInterract
  (CallFunction|ActivateElevator))

(fn ConstructionScript)