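; BP_BoxAndCam is a possessable zone with a trigger box, through which the player controls the Spectre, likely from the zone's camera.
; Cidara entering the box gains the ability to possess and registers the zone in her BoxCams list; leaving reverses both.
; While possessed, it forwards move and climb input to the Spectre found at BeginPlay.
; A key hands possession back to Cidara and switches her HUD animation.
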(event OnComponentBeginOverlap(Box)
  (params (OverlappedComponent :type Primitive%20Component%20Object%20Reference) (OtherActor :type Actor%20Object%20Reference) (OtherComp :type Primitive%20Component%20Object%20Reference) (OtherBodyIndex :type Integer) (bFromSweep :type Boolean) (SweepResult :type Hit%20Result%20Structure%20%28by%20ref%29))
  ;[0.15 0.15 0.15 0.5] si le joueur se trouve dans la box, il peut posseder spectre
  (bind _asbp_player_cidara (Utilities|Casting|CastToBP_PlayerCidara OtherActor))
  (Variables|/Game/Game/Blueprints/Characters/BP_PlayerCidara.BP_PlayerCidara_C|SetCanPossess? _asbp_player_cidara true)
  (Utilities|Array|Add (Variables|/Game/Game/Blueprints/Characters/BP_PlayerCidara.BP_PlayerCidara_C|GetBoxCams _asbp_player_cidara) self))

(event OnComponentEndOverlap(Box)
  (params (OverlappedComponent :type Primitive%20Component%20Object%20Reference) (OtherActor :type Actor%20Object%20Reference) (OtherComp :type Primitive%20Component%20Object%20Reference) (OtherBodyIndex :type Integer))
  ;[0.15 0.15 0.15 0.5] si le joueur se trouve dans la box, il peut posseder spectre
  (bind _asbp_player_cidara (Utilities|Casting|CastToBP_PlayerCidara OtherActor))
  (Variables|/Game/Game/Blueprints/Characters/BP_PlayerCidara.BP_PlayerCidara_C|SetCanPossess? _asbp_player_cidara false)
  (Utilities|Array|RemoveItem (Variables|/Game/Game/Blueprints/Characters/BP_PlayerCidara.BP_PlayerCidara_C|GetBoxCams _asbp_player_cidara) self))

(event Input|EnhancedActionEvents|EnhancedInputActionIA_Move
  (params (ActionValue :type Vector%202D%20Structure) (ElapsedSeconds :type Float%20%28double-precision%29) (TriggeredSeconds :type Float%20%28double-precision%29) (InputAction :type Input%20Action%20Object%20Reference :default "/Game/Game/Input/Actions/IA_Move.IA_Move"))
  ;[0.15 0.15 0.15 0.5] bouge spectre
  (Default|MoveSpectre (Variables|Default|GetSpectre) (.x ActionValue) (.y ActionValue)))

(event EventBeginPlay
  (Utilities|FlowControl|Sequence
    (:then_0
      (bind _returnvalue (Actor|GetActorOfClass "/Game/Game/Blueprints/Characters/Spectre/BP_Spectre.BP_Spectre_C"))
      (Variables|Default|SetSpectre _returnvalue))
    (:then_1
      (bind _returnvalue_2 (Actor|GetActorOfClass "/Game/Game/Blueprints/Characters/BP_PlayerCidara.BP_PlayerCidara_C"))
      (Variables|Default|SetCidara _returnvalue_2))))

(event EventTick
  (params (DeltaSeconds :type Float%20%28single-precision%29)))

(event Input|KeyboardEvents|A
  (params (Key :type Key%20Structure :default "None"))
  (bind _cidara (Variables|Default|GetCidara))
  (bind _spectre (Variables|Default|GetSpectre))
  ;[0.15 0.15 0.15 0.5] possess cidara
  (:Pressed
    (if (Variables|/Game/Game/Blueprints/Characters/Spectre/BP_Spectre.BP_Spectre_C|GetisPossess? _spectre)
      (Variables|/Game/Game/Blueprints/Characters/Spectre/BP_Spectre.BP_Spectre_C|SetisPossess? _spectre false)
      (Pawn|Possess (Pawn|GetController) _cidara)
      (Default|SwitchHUDAnim _cidara)
      (Development|PrintString "je possede cidara"))))

(event Input|KeyboardEvents|R
  (params (Key :type Key%20Structure :default "None"))
  (bind _spectre (Variables|Default|GetSpectre))
  ;[0.1458 0.1458 0.1458] Start Climb
  (:Pressed
    (if (not (Variables|/Game/Game/Blueprints/Characters/Spectre/BP_Spectre.BP_Spectre_C|GetisClimbing? _spectre))
      (Default|SpectreClimb _spectre)
      (else
        (Default|StopClimbing _spectre)))))

(event Input|KeyboardEvents|W
  (params (Key :type Key%20Structure :default "None"))
  (:Pressed
    (Default|PlayAnimChangeFace (Variables|Default|GetWBP_HUD))))

(fn ConstructionScript)