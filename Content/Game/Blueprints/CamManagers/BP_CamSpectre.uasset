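; BP_CamSpectre is the controlled camera actor through which player input drives the Spectre.
; On BeginPlay it finds and caches the Spectre and the Cidara player by class.
; It forwards IA_Move to the Spectre's movement and toggles its climbing on R.
; A hands the controller's possession to Cidara while the Spectre's IsPossess flag is set.
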(event Input|EnhancedActionEvents|EnhancedInputActionIA_Move
  (params (ActionValue :type Vector%202D%20Structure) (ElapsedSeconds :type Float%20%28double-precision%29) (TriggeredSeconds :type Float%20%28double-precision%29) (InputAction :type Input%20Action%20Object%20Reference :default "/Game/Game/Input/Actions/IA_Move.IA_Move"))
  (Default|MoveSpectre (Variables|Default|GetSpectre) (.x ActionValue) (.y ActionValue)))

(event EventBeginPlay
  (Utilities|FlowControl|Sequence
    (:then_0
      (bind _returnvalue (Actor|GetActorOfClass "/Game/Game/Blueprints/Characters/Spectre/BP_Spectre.BP_Spectre_C"))
      (Variables|Default|SetSpectre _returnvalue))
    (:then_1
      (bind _returnvalue_2 (Actor|GetActorOfClass "/Game/Game/Blueprints/Characters/BP_PlayerCidara.BP_PlayerCidara_C"))
      (Variables|Default|SetCidara _returnvalue_2))))

(event Input|KeyboardEvents|R
  (params (Key :type Key%20Structure :default "None"))
  (bind _spectre (Variables|Default|GetSpectre))
  ;[1 1 1] Start Climb
  (:Pressed
    (if (not (Variables|/Game/Game/Blueprints/Characters/Spectre/BP_Spectre.BP_Spectre_C|GetisClimbing? _spectre))
      (Default|SpectreClimb _spectre)
      (else
        (Default|StopClimbing _spectre)))))

(event Input|KeyboardEvents|A
  (params (Key :type Key%20Structure :default "None"))
  (:Pressed
    (if (Variables|/Game/Game/Blueprints/Characters/Spectre/BP_Spectre.BP_Spectre_C|GetisPossess? (Variables|Default|GetSpectre))
      (Pawn|Possess (Pawn|GetController) (Variables|Default|GetCidara)))))

(fn ConstructionScript)