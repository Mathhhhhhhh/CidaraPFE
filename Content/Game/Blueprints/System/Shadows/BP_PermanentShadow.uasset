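; BP_PermanentShadow is a shadow volume actor that marks a permanent shadow zone for the spectre character.
; Entering or leaving its ShadowBox registers or unregisters the volume with the BP_Spectre's shadow detection component.
; On entry it also activates its associated spawner, if set, and then deactivates a linked checkpoint, apparently advancing the respawn point.
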(event OnComponentBeginOverlap(ShadowBox)
  (params (OverlappedComponent :type Primitive%20Component%20Object%20Reference) (OtherActor :type Actor%20Object%20Reference) (OtherComp :type Primitive%20Component%20Object%20Reference) (OtherBodyIndex :type Integer) (bFromSweep :type Boolean) (SweepResult :type Hit%20Result%20Structure%20%28by%20ref%29))
  (CallFunction|HandleBeginOverlap OtherActor))

(event OnComponentEndOverlap(ShadowBox)
  (params (OverlappedComponent :type Primitive%20Component%20Object%20Reference) (OtherActor :type Actor%20Object%20Reference) (OtherComp :type Primitive%20Component%20Object%20Reference) (OtherBodyIndex :type Integer))
  (CallFunction|HandleEndOverlap OtherActor))

(event Custom|HandleEndOverlap
  (params (OtherActor :type Actor%20Object%20Reference))
  (bind _asbp_spectre (Utilities|Casting|CastToBP_Spectre OtherActor))
  (if (Utilities|IsValid _asbp_spectre)
    (Default|UnregisterPermanentVolume (Variables|/Game/Game/Blueprints/Characters/Spectre/BP_Spectre.BP_Spectre_C|GetBPC_ShadowDetection _asbp_spectre) self)))

(event Custom|HandleBeginOverlap
  (params (OtherActor :type Actor%20Object%20Reference))
  (bind _spawnerassocied (Variables|Default|GetSpawnerAssocied))
  (bind _checkpointdeactivate (Variables|Default|GetCheckPointDeactivate))
  (bind _asbp_spectre (Utilities|Casting|CastToBP_Spectre OtherActor))
  (if (Utilities|IsValid _asbp_spectre)
    (Default|RegisterPermanentVolume (Variables|/Game/Game/Blueprints/Characters/Spectre/BP_Spectre.BP_Spectre_C|GetBPC_ShadowDetection _asbp_spectre) self)
    (if (Utilities|IsValid _spawnerassocied)
      (Variables|/Game/Game/Blueprints/Characters/Spectre/BP_SafeSpawn.BP_SafeSpawn_C|SetIsActive _spawnerassocied true)
      (if (Utilities|IsValid _checkpointdeactivate)
        (Variables|/Game/Game/Blueprints/Characters/Spectre/BP_SafeSpawn.BP_SafeSpawn_C|SetIsActive _checkpointdeactivate false)))))

(event EventBeginPlay)

(event Collision|EventActorBeginOverlap
  (params (OtherActor :type Actor%20Object%20Reference)))

(event EventTick
  (params (DeltaSeconds :type Float%20%28single-precision%29)))

(fn ConstructionScript)