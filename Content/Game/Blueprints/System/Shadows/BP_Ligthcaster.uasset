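; Light caster actor for the shadow system, exposing a spherical area of influence that can be switched on and off.
; Activate and Deactivate play a timeline forward or in reverse to grow or shrink the sphere radius, firing OnActivated or OnDeactivated when finished.
; Sphere overlaps register the caster with other actors' BPC_ShadowDetection component while active, and unregister it when overlap ends.
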(event Custom|HandleBeginOverlap
  (params (OverlappedComponent :type Primitive%20Component%20Object%20Reference) (OtherActor :type Actor%20Object%20Reference) (OtherComp :type Primitive%20Component%20Object%20Reference) (OtherBodyIndex :type Integer) (bFromSweep :type Boolean) (SweepResult :type Hit%20Result%20Structure%20%28by%20ref%29))
  (bind _returnvalue (Actor|GetComponentbyClass OtherActor "/Game/Game/Blueprints/System/Shadows/BPC_ShadowDetection.BPC_ShadowDetection_C"))
  (if (Variables|Default|GetActive)
    (if (Utilities|IsValid _returnvalue)
      (Default|RegisterLigthcaster _returnvalue self))))

(event Custom|HandleEndOverlap
  (params (OverlappedComponent :type Primitive%20Component%20Object%20Reference) (OtherActor :type Actor%20Object%20Reference) (OtherComp :type Primitive%20Component%20Object%20Reference) (OtherBodyIndex :type Integer))
  (bind _returnvalue (Actor|GetComponentbyClass OtherActor "/Game/Game/Blueprints/System/Shadows/BPC_ShadowDetection.BPC_ShadowDetection_C"))
  (if (Utilities|IsValid _returnvalue)
    (Default|UnregisterLigthcaster _returnvalue self)))

(event Custom|Deactivate
  (if (Variables|Default|GetActive)
    (Variables|Default|SetActive false)
    (bind _alpha (Timeline|TL_Activation Reverse)
      (:Update
        (bind _output_get (Variables|Default|SetCurrentRadius (Math|Float|Lerp 0.0 (Variables|Default|GetRadius) _alpha)))
        (Components|Sphere|SetSphereRadius (Variables|Default|GetSphere) _output_get true))
      (:Finished
        (if (Variables|Default|GetActive)
          (Default|CallOnActivated)
          (else
            (Default|CallOnDeactivated)))))))

(event Custom|Activate
  (if (not (Variables|Default|GetActive))
    (Variables|Default|SetActive true)
    (bind _alpha (Timeline|TL_Activation PlayFromStart)
      (:Update
        (bind _output_get (Variables|Default|SetCurrentRadius (Math|Float|Lerp 0.0 (Variables|Default|GetRadius) _alpha)))
        (Components|Sphere|SetSphereRadius (Variables|Default|GetSphere) _output_get true))
      (:Finished
        (if (Variables|Default|GetActive)
          (Default|CallOnActivated)
          (else
            (Default|CallOnDeactivated)))))))

(event EventBeginPlay
  (bind _sphere (Variables|Default|GetSphere))
  (Components|Sphere|SetSphereRadius _sphere 0.0 true)
  (Collision|BindEventtoOnComponentBeginOverlap _sphere (EventDispatchers|CreateEvent :!event Custom|HandleBeginOverlap))
  (Collision|BindEventtoOnComponentEndOverlap _sphere (EventDispatchers|CreateEvent :!event Custom|HandleEndOverlap))
  (if (Variables|Default|GetActive)
    (CallFunction|Activate)))

(fn ConstructionScript)