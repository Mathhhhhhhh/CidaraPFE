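; BP_DynamicShadow is a toggleable shadow volume that reports itself to actors carrying a BPC_ShadowDetection component.
; ShadowBox overlaps register the volume on entry, only while enabled, and unregister it on exit.
; SetEnabled broadcasts a change and registers or unregisters the volume with actors already inside the box.
; ShadowAppear plays a timeline that drives the Reveal parameter of the Cube's dynamic material, created at BeginPlay.
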(event OnComponentBeginOverlap(ShadowBox)
  (params (OverlappedComponent :type Primitive%20Component%20Object%20Reference) (OtherActor :type Actor%20Object%20Reference) (OtherComp :type Primitive%20Component%20Object%20Reference) (OtherBodyIndex :type Integer) (bFromSweep :type Boolean) (SweepResult :type Hit%20Result%20Structure%20%28by%20ref%29))
  (CallFunction|HandleBeginOverlap OtherActor))

(event OnComponentEndOverlap(ShadowBox)
  (params (OverlappedComponent :type Primitive%20Component%20Object%20Reference) (OtherActor :type Actor%20Object%20Reference) (OtherComp :type Primitive%20Component%20Object%20Reference) (OtherBodyIndex :type Integer))
  (CallFunction|HandleEndOverlap OtherActor))

(event Custom|HandleEndOverlap
  (params (OtherActor :type Actor%20Object%20Reference))
  (bind _returnvalue (Actor|GetComponentbyClass OtherActor "/Game/Game/Blueprints/System/Shadows/BPC_ShadowDetection.BPC_ShadowDetection_C"))
  (if (Utilities|IsValid _returnvalue)
    (Default|UnRegisterDynamicVolume _returnvalue self)))

(event Custom|HandleBeginOverlap
  (params (OtherActor :type Actor%20Object%20Reference))
  (bind _returnvalue (Actor|GetComponentbyClass OtherActor "/Game/Game/Blueprints/System/Shadows/BPC_ShadowDetection.BPC_ShadowDetection_C"))
  (if (Utilities|IsValid _returnvalue)
    (if (Variables|Default|GetEnabled)
      (Default|RegisterDynamicVolume _returnvalue self))))

(event Custom|ShadowAppear
  (bind _alpha (Timeline|TL_Shadow Play)
    (:Update
      (Rendering|Material|SetScalarParameterValue (Variables|Default|GetMaterialref) "Reveal" (Math|Float|Lerp 0.0 1.0 _alpha) :!class /Script/Engine.MaterialInstanceDynamic))))

(event EventBeginPlay
  (bind _cube (Variables|Default|GetCube))
  (bind _returnvalue (Rendering|Material|CreateDynamicMaterialInstance _cube 0 (Rendering|Material|GetMaterial _cube 0) "None" :!class /Script/Engine.PrimitiveComponent))
  (Variables|Default|SetMaterialref _returnvalue))

(event Collision|EventActorBeginOverlap
  (params (OtherActor :type Actor%20Object%20Reference)))

(event EventTick
  (params (DeltaSeconds :type Float%20%28single-precision%29)))

(fn ConstructionScript)

(fn SetEnabled
  (params (bNew :type Boolean))
  (bind _shadowbox (Variables|Default|GetShadowBox))
  (bind _overlappingactors (Collision|GetOverlappingActors _shadowbox 0 :!class /Script/Engine.PrimitiveComponent))
  (if (not (== bNew (Variables|Default|GetEnabled)))
    (bind _output_get (Variables|Default|SetEnabled bNew))
    (Default|CallOnEnabledChange _output_get)
    (if bNew
      (for _array_element _overlappingactors
        (Utilities|IsValid (Actor|GetComponentbyClass _array_element "/Game/Game/Blueprints/System/Shadows/BPC_ShadowDetection.BPC_ShadowDetection_C")
          (:Is%20Valid
            (Default|RegisterDynamicVolume (Actor|GetComponentbyClass _array_element "/Game/Game/Blueprints/System/Shadows/BPC_ShadowDetection.BPC_ShadowDetection_C") self))))
      (else
        (for _array_element_2 _overlappingactors
          (Utilities|IsValid (Actor|GetComponentbyClass _array_element_2 "/Game/Game/Blueprints/System/Shadows/BPC_ShadowDetection.BPC_ShadowDetection_C")
            (:Is%20Valid
              (Default|UnRegisterDynamicVolume (Actor|GetComponentbyClass _array_element_2 "/Game/Game/Blueprints/System/Shadows/BPC_ShadowDetection.BPC_ShadowDetection_C") self))))))))