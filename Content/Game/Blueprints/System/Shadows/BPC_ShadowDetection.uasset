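; Actor component that tracks whether its owner is in shadow or sunlight and broadcasts state changes.
; A looping timer resolves state by priority: permanent shadow volumes, active light casters, enabled dynamic shadow volumes, then sun raycasts.
; The raycast fallback samples a grid of traces along the sun direction against a lit-ratio threshold, with early exit on unanimous light.
; Leaving shadow starts a cancellable grace period that broadcasts rising warning progress before declaring exposure.
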(event Custom|CancelGracePeriod
  (Variables|Default|SetInGracePeriod false)
  (Utilities|Time|ClearandInvalidateTimerbyHandle (Variables|Default|GetGraceTimerHandle))
  (Utilities|Time|ClearandInvalidateTimerbyHandle (Variables|Default|GetWarningTickHandler))
  (Variables|Default|SetCurrentShadowState "NewEnumerator0")
  (Default|CallOnShadowWarning 0.0)
  (Default|CallOnShadowStateChanged "NewEnumerator0"))

(event Custom|StartGracePeriod
  (Variables|Default|SetInGracePeriod true)
  (Variables|Default|SetCurrentShadowState "NewEnumerator2")
  (Variables|Default|SetPendingShadowState "NewEnumerator1")
  (Variables|Default|SetGraceStartTime (Utilities|Time|GetGameTimeinSeconds))
  (Default|CallOnShadowStateChanged "NewEnumerator2")
  (bind _returnvalue (Utilities|Time|SetTimerbyEvent (delegate Custom|OnGracePeriodElapsed) (Variables|Default|GetGracePeriodDuration)))
  (Variables|Default|SetGraceTimerHandle _returnvalue)
  (bind _returnvalue_2 (Utilities|Time|SetTimerbyEvent (delegate Custom|BroadcastWarningTick) 0.03 true))
  (Variables|Default|SetWarningTickHandler _returnvalue_2))

(event Custom|OnGracePeriodElapsed
  (Variables|Default|SetInGracePeriod false)
  (Utilities|Time|ClearandInvalidateTimerbyHandle (Variables|Default|GetWarningTickHandler))
  (Variables|Default|SetCurrentShadowState "NewEnumerator1")
  (Default|CallOnExitedShadow)
  (Default|CallOnShadowStateChanged "NewEnumerator1")
  (Default|CallOnShadowWarning 1.0))

(event Custom|BroadcastWarningTick
  (Default|CallOnShadowWarning (Math|Float|Clamp(Float) (/ (- (Utilities|Time|GetGameTimeinSeconds) (Variables|Default|GetGraceStartTime)) (Variables|Default|GetGracePeriodDuration)))))

(event Custom|CleanUpGraceTimer
  (if (Variables|Default|GetInGracePeriod)
    (Utilities|Time|ClearandInvalidateTimerbyHandle (Variables|Default|GetGraceTimerHandle))
    (Utilities|Time|ClearandInvalidateTimerbyHandle (Variables|Default|GetWarningTickHandler))
    (Variables|Default|SetInGracePeriod false)))

(event Custom|ResetShadowState)

(event EventBeginPlay
  (Utilities|FlowControl|Sequence
    (:then_0
      (bind _returnvalue (Actor|GetActorOfClass "/Game/Game/Blueprints/LightRune/BP_Sun.BP_Sun_C"))
      (Variables|Default|SetSunRef _returnvalue)
      (bind _returnvalue_2 (Utilities|Time|SetTimerbyFunctionName 0 "DetectionTick" (/ 1.0 (Variables|Default|GetDetectionTickRate)) true))
      (Variables|Default|SetTickTimerHandle _returnvalue_2))
    (:then_1
      (Variables|Default|SetSunTraceOffSet (Utilities|Array|MakeArray "0.000000,0.000000,50.000000" "0.000000,0.000000,-50.000000" "0.000000,50.000000,0.000000" "0.000000,-50.000000,0.000000")))))

(event EventTick
  (params (DeltaSeconds :type Float%20%28single-precision%29)))

(fn DetectionTick
  (bind _result (CallFunction|ResolveShadowState))
  (bind _output_get (LocalVariables|SetQueryResult _result))
  (if (.InShadow (Utilities|Struct|BreakS_ShadowQueryResult _output_get))
    (if (Variables|Default|GetInGracePeriod)
      (CallFunction|CancelGracePeriod)
      (elif (Utilities|Enum|NotEqual(Enum) (Variables|Default|GetCurrentShadowState) "NewEnumerator0")
        (Variables|Default|SetCurrentShadowState "NewEnumerator0")
        (Default|CallOnEnteredShadow)
        (Default|CallOnShadowStateChanged "NewEnumerator0")))
    (elif (and (Utilities|Enum|Equal(Enum) (Variables|Default|GetCurrentShadowState) "NewEnumerator0") (== (Variables|Default|GetInGracePeriod) false))
      (CallFunction|StartGracePeriod))))

(fn GetSunDirection
  (bind _sunref (Variables|Default|GetSunRef))
  (if (Utilities|IsValid _sunref)
    (return (Transformation|GetActorForwardVector _sunref))
    (else
      (return "0.000000,0.000000,-1.000000"))))

(fn PerformSingleRaycast
  (params (StratLocation :type Vector) (TraceDistance :type Float%20%28double-precision%29))
  (bind (_outhit _returnvalue) (Collision|LineTraceByChannel StratLocation (+ StratLocation (* (Math|Vector|NegateVector (CallFunction|GetSunDirection)) TraceDistance)) (Variables|Default|GetTraceChannel) true (Utilities|Array|MakeArray (Components|GetOwner)) "None" true "(R=1.000000,G=0.000000,B=0.000000,A=1.000000)" "(R=0.000000,G=1.000000,B=0.000000,A=1.000000)" 1.0))
  (return _returnvalue (.Location (Collision|BreakHitResult _outhit))))

(fn PerformShadowQuery
  (LocalVariables|SetOwner (Components|GetOwner))
  (bind _isinshadow (CallFunction|IsPointinShadowSamples (+ (Transformation|GetActorLocation (LocalVariables|GetOwner)) "0.000000,0.000000,-50.000000") (Variables|Default|GetGrid%20Yaxis) (Variables|Default|GetGrid%20XAxis)))
  (if _isinshadow
    (return (Utilities|Struct|MakeS_ShadowQueryResult true 1.0 "NewEnumerator0" (+ (Transformation|GetActorLocation (LocalVariables|GetOwner)) "0.000000,0.000000,-50.000000")))
    (else
      (return (Utilities|Struct|MakeS_ShadowQueryResult false 1.0 "NewEnumerator0" (+ (Transformation|GetActorLocation (LocalVariables|GetOwner)) "0.000000,0.000000,-50.000000"))))))

(fn RegisterPermanentVolume
  (params (Volume :type Actor%20Object%20Reference))
  (Utilities|Array|AddUnique (Variables|Default|GetOverlappingPermanentVolumes) Volume))

(fn UnregisterPermanentVolume
  (params (Volume :type Actor%20Object%20Reference))
  (Utilities|Array|RemoveItem (Variables|Default|GetOverlappingPermanentVolumes) Volume))

(fn RegisterDynamicVolume
  (params (Volume :type Actor%20Object%20Reference))
  (Utilities|Array|AddUnique (Variables|Default|GetOverlappingDynamicVolumes) Volume))

(fn UnRegisterDynamicVolume
  (params (Volume :type Actor%20Object%20Reference))
  (Utilities|Array|RemoveItem (Variables|Default|GetOverlappingDynamicVolumes) Volume))

(fn ResolveShadowState
  (bind _returnvalue (Components|GetOwner))
  (bind _returnvalue_2 (Transformation|GetActorLocation _returnvalue))
  (if (> (Utilities|Array|Length (Variables|Default|GetOverlappingPermanentVolumes)) 0)
    (return (Utilities|Struct|MakeS_ShadowQueryResult true 1.0 "NewEnumerator1" _returnvalue_2))
    (else
      (bind _array_element (Utilities|Array|ForEachLoopwithBreak (Variables|Default|GetOverlappingLightCasters) :!label _label)
        (:LoopBody
          (bind _asbp_ligthcaster (Utilities|Casting|CastToBP_Ligthcaster _array_element))
          (if (Variables|/Game/Game/Blueprints/System/Shadows/BP_Ligthcaster.BP_Ligthcaster_C|GetActive _asbp_ligthcaster)
            (LocalVariables|SetLResult (Utilities|Struct|MakeS_ShadowQueryResult false 1.0 "NewEnumerator3" _returnvalue_2))
            (goto _label Break)))
        (:Completed
          (if (or (.InShadow (Utilities|Struct|BreakS_ShadowQueryResult (LocalVariables|GetLResult))) (Utilities|Enum|Equal(Enum) (.Source (Utilities|Struct|BreakS_ShadowQueryResult (LocalVariables|GetLResult))) "NewEnumerator3"))
            (return (LocalVariables|GetLResult))
            (else
              (bind _array_element_2 (Utilities|Array|ForEachLoopwithBreak (Variables|Default|GetOverlappingDynamicVolumes) :!label _label_2)
                (:LoopBody
                  (bind _asbp_dynamic_shadow (Utilities|Casting|CastToBP_DynamicShadow _array_element_2))
                  (if (Variables|/Game/Game/Blueprints/System/Shadows/BP_DynamicShadow.BP_DynamicShadow_C|GetEnabled _asbp_dynamic_shadow)
                    (LocalVariables|SetLResult (Utilities|Struct|MakeS_ShadowQueryResult true 1.0 "NewEnumerator2" _returnvalue_2))
                    (goto _label_2 Break)))
                (:Completed
                  (if (.InShadow (Utilities|Struct|BreakS_ShadowQueryResult (LocalVariables|GetLResult)))
                    (return (LocalVariables|GetLResult))
                    (else
                      (bind _result (CallFunction|PerformShadowQuery))
                      (return _result))))))))))))

(fn RegisterLigthcaster
  (params (Volume :type Actor%20Object%20Reference))
  (Utilities|Array|AddUnique (Variables|Default|GetOverlappingLightCasters) Volume))

(fn UnregisterLigthcaster
  (params (Volume :type Actor%20Object%20Reference))
  (Utilities|Array|RemoveItem (Variables|Default|GetOverlappingLightCasters) Volume))

(fn IsPointinLigthSimple
  (params (Location%20 :type Vector))
  (Utilities|IsValid (Variables|Default|GetSunRef)
    (:Is%20Valid
      (bind _output_get (LocalVariables|SetRayStart (+ Location%20 (* (Math|Vector|NegateVector (CallFunction|GetSunDirection)) 5e+03))))
      (bind _returnvalue (Collision|LineTraceByChannel _output_get Location%20 "TraceTypeQuery5" false 0 "None" true "(R=0.000000,G=1.000000,B=0.193893,A=1.000000)" "(R=1.000000,G=0.000000,B=0.088168,A=1.000000)" 1.0))
      (bind _output_get_2 (LocalVariables|SetInLigth (not _returnvalue)))
      (return _output_get_2))
    (:Is%20Not%20Valid
      (LocalVariables|SetInLigth true))))

(fn IsPointinShadowSamples
  (params (CenterLocation :type Vector) (GridYaxis :type Vector :default "1.000000,0.000000,0.000000") (GridXAxis :type Vector :default "0.000000,1.000000,0.000000"))
  (bind _samplegridsize (Variables|Default|GetSampleGridSize))
  (bind _returnvalue (- _samplegridsize 1))
  (bind _returnvalue_2 (Math|Conversions|ToFloat(Integer) _returnvalue))
  (bind _returnvalue_3 (/ _returnvalue_2 2.0))
  (LocalVariables|SetLigthCount 0)
  (LocalVariables|SetShadowCount 0)
  (bind _output_get (LocalVariables|SetTotalSamples (Math|Float|Truncate (Math|Float|Square (Math|Conversions|ToFloat(Integer) (Variables|Default|GetSampleGridSize))))))
  (LocalVariables|SetLigthThreshold (* _output_get (Variables|Default|GetLigthThresholdRatio)))
  (LocalVariables|SetMaxIndex (- _output_get 1))
  (bind _output_get_2 (LocalVariables|SetGridIndex 0))
  (while (<= _output_get_2 (LocalVariables|GetMaxIndex))
    (bind _isinligth (CallFunction|IsPointinLigthSimple (+ (+ (* GridXAxis (* (- (Math|Conversions|ToFloat(Integer) (Math|Integer|%(Integer) (LocalVariables|GetGridIndex) _samplegridsize)) _returnvalue_3) (Variables|Default|GetSampleSpacing))) (* GridYaxis (* (- (Math|Conversions|ToFloat(Integer) (/ (LocalVariables|GetGridIndex) _samplegridsize)) _returnvalue_3) (Variables|Default|GetSampleSpacing)))) CenterLocation)))
    (if _isinligth
      (bind _result (Math|Integer|IncrementInt (LocalVariables|GetLigthCount))
        (:%20%20
          (if (and (>= _result (Variables|Default|GetEarlyExitUnanimousCount)) (== (LocalVariables|GetShadowCount) 0))
            (LocalVariables|SetResult false)
            (LocalVariables|SetGridIndex (+ (LocalVariables|GetMaxIndex) 1))
            (LocalVariables|SetDidEarlyExit true)
            (else
              (Math|Integer|IncrementInt (LocalVariables|GetGridIndex) :!label _label)))))
      (else
        (Math|Integer|IncrementInt (LocalVariables|GetShadowCount)
          (:%20%20
            (goto _label))))))
  (if (LocalVariables|GetDidEarlyExit)
    (return (LocalVariables|GetResult))
    (else
      (bind _output_get_3 (LocalVariables|SetResult (not (>= (LocalVariables|GetLigthCount) (LocalVariables|GetLigthThreshold)))))
      (return _output_get_3))))