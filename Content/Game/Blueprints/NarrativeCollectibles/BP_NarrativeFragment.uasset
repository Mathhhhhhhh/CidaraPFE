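; BP_NarrativeFragment is a narrative collectible that registers itself as collected when interacted with.
; It caches the GI_Cidara game instance on BeginPlay.
; Interract checks that the player character is within InterractRange, then passes CollectibleID to the game instance.
; After a short delay it calls EventFragment, which is empty in this Blueprint.
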(event Custom|EventFragment)

(event EventBeginPlay
  (bind _asgi_cidara (Utilities|Casting|CastToGI_Cidara (Game|GetGameInstance)))
  (Variables|Default|SetGIref _asgi_cidara))

(event EventInterract
  (if (<= (Math|Vector|Distance(Vector) (Transformation|GetActorLocation (Game|GetPlayerCharacter 0)) (Transformation|GetActorLocation)) (Variables|Default|GetInterractRange))
    (Default|RegisterFragementCollected (Variables|Default|GetGIref) (Variables|Default|GetCollectibleID))
    (Utilities|FlowControl|Delay 0.2)
    (CallFunction|EventFragment)))

(fn ConstructionScript)