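; BPC_DialogueComponent is an actor component that steps through dialogue stored in a DataTable.
; It looks up the row named after CurrentRowNumber and caches it as CurrentDialogueRow, which getters read for long text, character and timer.
; Rows chain through a NextRow index: ReadNextRow only updates the number, leaving the fetch to a separate call, and a negative index marks the dialogue as finished.
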(event EventBeginPlay)

(event EventTick
  (params (DeltaSeconds :type Float%20%28single-precision%29)))

(fn GetCurrentDialogueRowData
  (bind _returnvalue (Utilities|GetDataTableRow (Variables|Default|GetDataTable) (Utilities|String|StringToName (Utilities|String|ToString(Integer) (Variables|Default|GetCurrentRowNumber))))
    (:then
      (bind _output_get (Variables|Default|SetCurrentDialogueRow _returnvalue))
      (return _output_get))))

(fn GetDialogueLongfromCurrentRow
  (return (.TextLong (Utilities|Struct|BreakS_DialogueLine (Variables|Default|GetCurrentDialogueRow)))))

(fn GetCharacterfromCurrentRow
  (return (.Character (Utilities|Struct|BreakS_DialogueLine (Variables|Default|GetCurrentDialogueRow)))))

(fn IsDialogueFinished
  (return (<= (.NextRow (Utilities|Struct|BreakS_DialogueLine (Variables|Default|GetCurrentDialogueRow))) -1)))

(fn ReadNextRow
  (Variables|Default|SetCurrentRowNumber (.nextrow (Variables|Default|GetCurrentDialogueRow))))

(fn GetCurrentRowTimer
  (return (.Time (Utilities|Struct|BreakS_DialogueLine (Variables|Default|GetCurrentDialogueRow)))))