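; BP_Glyphe is a glyph decal that fades in or out depending on the player's proximity and light.
; It starts at zero opacity on a dynamic material instance.
; Box overlaps with the cached BP_PlayerCidara trigger UpdateVisibility, which fades in only if the player is in range with the point light active, otherwise out.
; One timeline drives opacity, playing forward for fade-out and reversing for fade-in.
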(event OnComponentBeginOverlap(Box)
  (params (OverlappedComponent :type Primitive%20Component%20Object%20Reference) (OtherActor :type Actor%20Object%20Reference) (OtherComp :type Primitive%20Component%20Object%20Reference) (OtherBodyIndex :type Integer) (bFromSweep :type Boolean) (SweepResult :type Hit%20Result%20Structure%20%28by%20ref%29))
  (if (== OtherActor (Variables|Default|GetPlayerRef))
    (Variables|Default|SetPlayerInRange true)
    (CallFunction|UpdateVisibility)))

(event OnComponentEndOverlap(Box)
  (params (OverlappedComponent :type Primitive%20Component%20Object%20Reference) (OtherActor :type Actor%20Object%20Reference) (OtherComp :type Primitive%20Component%20Object%20Reference) (OtherBodyIndex :type Integer))
  (if (== OtherActor (Variables|Default|GetPlayerRef))
    (Variables|Default|SetPlayerInRange false)
    (CallFunction|UpdateVisibility)))

(event Custom|GlypheFadeOut
  (bind _alpha (Timeline|TL_FadeGlyphe Play)
    (:Update
      (Rendering|Material|SetScalarParameterValue (Variables|Default|GetDynaMI) "Opacity" _alpha :!class /Script/Engine.MaterialInstanceDynamic))))

(event Custom|GlypheFadeIn
  (bind _alpha (Timeline|TL_FadeGlyphe Reverse)
    (:Update
      (Rendering|Material|SetScalarParameterValue (Variables|Default|GetDynaMI) "Opacity" _alpha :!class /Script/Engine.MaterialInstanceDynamic))))

(event EventBeginPlay
  (bind _asbp_player_cidara (Utilities|Casting|CastToBP_PlayerCidara (Game|Player|GetPlayerPawn 0)))
  (Variables|Default|SetPlayerRef _asbp_player_cidara)
  (bind _returnvalue (Rendering|Material|CreateDynamicMaterialInstance (Variables|Default|GetNew%20Decal%20Material) "None" "None" :!class /Script/Engine.KismetMaterialLibrary))
  (bind _output_get (Variables|Default|SetDynaMI _returnvalue))
  (Rendering|Components|Decal|SetDecalMaterial (Variables|Default|GetDecal) _output_get)
  (Rendering|Material|SetScalarParameterValue _output_get "Opacity" 0.0 :!class /Script/Engine.MaterialInstanceDynamic))

(fn ConstructionScript
  (Rendering|Components|Decal|SetDecalMaterial (Variables|Default|GetDecal) (Variables|Default|GetNew%20Decal%20Material)))

(fn UpdateVisibility
  (if (and (Variables|Default|GetPlayerInRange) (Variables|/Game/Game/Blueprints/Characters/Cidara/BP_PlayerCidara.BP_PlayerCidara_C|GetIsPointLightActive? (Variables|Default|GetPlayerRef)))
    (CallFunction|GlypheFadein)
    (else
      (CallFunction|GlypheFadeOut))))