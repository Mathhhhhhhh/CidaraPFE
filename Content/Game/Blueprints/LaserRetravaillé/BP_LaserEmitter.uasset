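; Laser emitter that traces a beam along its DirectionVector each tick while LaserActive is false, recursively reflecting off BP_Miroir up to MaxBounces.
; Each segment reuses or spawns a pooled Niagara beam, and CleanBeam deactivates those beyond the returned index.
; Hit BP_LaserReceivers get OnLaserReceived.
; UpdateReceiver targets OnLaserLost at previous receivers still in the active list, but clears the previous list every pass, leaving nothing to notify.
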(event EventTick
  (params (DeltaSeconds :type Float%20%28single-precision%29))
  (bind _directionvector (Variables|Default|GetDirectionVector))
  (if (not (Variables|Default|GetbLaserActive))
    (Utilities|Array|Clear (Variables|Default|GetHitReceiverActifs))
    (bind _segmentindex (CallFunction|TracerLaser (Transformation|GetWorldLocation _directionvector) (Math|Vector|GetForwardVector _directionvector)))
    (bind _output_get (Variables|Default|SetSegment%20Index _segmentindex))
    (CallFunction|CleanBeam _output_get)
    (CallFunction|UpdateReceiver)))

(fn ConstructionScript)

(fn TracerLaser
  (params (StartPos :type Vector) (Direction :type Vector) (BounceCount :type Integer))
  (bind _output_get (LocalVariables|SetBounce%20Count BounceCount))
  (bind _output_get_2 (LocalVariables|SetDirect Direction))
  (bind _output_get_3 (LocalVariables|SetStartPosition StartPos))
  (bind _output_get_4 (LocalVariables|SetEndCalcul (+ _output_get_3 (* _output_get_2 (Variables|Default|GetLaserLenght)))))
  (if (not (>= _output_get (Variables|Default|GetMaxBounces)))
    (bind (_outhit _returnvalue) (Collision|LineTraceByChannel _output_get_3 _output_get_4 "TraceTypeQuery1" false 0 "ForDuration" true "(R=1.000000,G=0.000000,B=0.000000,A=1.000000)" "(R=0.000000,G=1.000000,B=0.000000,A=1.000000)" 1.0))
    (LocalVariables|SetImpactNormal (.ImpactNormal (Collision|BreakHitResult _outhit)))
    (LocalVariables|SetImpactPoint (.ImpactPoint (Collision|BreakHitResult _outhit)))
    (LocalVariables|SetHitActor (.HitActor (Collision|BreakHitResult _outhit)))
    (if _returnvalue
      (CallFunction|BeamSegment (LocalVariables|GetStartPosition) (LocalVariables|GetImpactPoint) (LocalVariables|GetBounce%20Count))
      (bind _asbp_laser_receiver (Utilities|Casting|CastToBP_LaserReceiver (LocalVariables|GetHitActor))
        (:then
          (Utilities|Array|Add (Variables|Default|GetHitReceiverActifs) _asbp_laser_receiver)
          (Default|OnLaserReceived _asbp_laser_receiver))
        (:CastFailed
          (Utilities|Casting|CastToBP_Miroir (LocalVariables|GetHitActor))
          (bind _segmentindex (CallFunction|TracerLaser (+ (* (LocalVariables|GetImpactNormal) 2) (LocalVariables|GetImpactPoint)) (Math|Vector|GetReflectionVector (LocalVariables|GetDirect) (LocalVariables|GetImpactNormal)) (+ (LocalVariables|GetBounce%20Count) 1)))
          (return _segmentindex)))
      (else
        (CallFunction|BeamSegment (LocalVariables|GetStartPosition) (LocalVariables|GetImpactPoint) (LocalVariables|GetBounce%20Count))))))

(fn BeamSegment
  (params (Start :type Vector) (End :type Vector) (Index :type Integer))
  (bind _beamsystem (Variables|Default|GetBeamSystem))
  (bind _output (Utilities|Array|Get(acopy) _beamsystem Index))
  (Utilities|IsValid _output
    (:Is%20Valid
      (LocalVariables|SetNiagaraRef _output)
      (Niagara|SetNiagaraVariable(Vector3) (LocalVariables|GetNiagaraRef) "User.BeamStart" Start)
      (Niagara|SetNiagaraVariable(Vector3) (LocalVariables|GetNiagaraRef) "User.BeamEnd" End)
      (Components|Activation|Activate (LocalVariables|GetNiagaraRef) true))
    (:Is%20Not%20Valid
      (bind _returnvalue (Niagara|SpawnSystematLocation "/Game/Game/Blueprints/LaserRetravaillé/NS_LaserBeam.NS_LaserBeam" "0, 0, 0" "0, 0, 0" "1.000000,1.000000,1.000000" false))
      (bind _output_get (LocalVariables|SetNiagaraRef _returnvalue))
      (Utilities|Array|Add (Variables|Default|GetBeamSystem) _output_get)
      (Niagara|SetNiagaraVariable(Vector3) (LocalVariables|GetNiagaraRef) "User.BeamStart" Start)
      (Niagara|SetNiagaraVariable(Vector3) (LocalVariables|GetNiagaraRef) "User.BeamEnd" End)
      (Components|Activation|Activate (LocalVariables|GetNiagaraRef) true))))

(fn UpdateReceiver
  (for _array_element (Variables|Default|GetHitReceiverPrecedents)
    (if (Utilities|Array|ContainsItem (Variables|Default|GetHitReceiverActifs) _array_element)
      (bind _asbp_laser_receiver (Utilities|Casting|CastToBP_LaserReceiver _array_element))
      (Default|OnLaserLost _asbp_laser_receiver)))
  (bind _output_get (Variables|Default|SetHitReceiverPrecedents (Variables|Default|GetHitReceiverActifs)))
  (Utilities|Array|Clear _output_get))

(fn CleanBeam
  (params (LastIndex :type Integer))
  (for (_array_element _array_index) (Variables|Default|GetBeamSystem)
    (if (> _array_index LastIndex)
      (Components|Activation|Deactivate _array_element))))