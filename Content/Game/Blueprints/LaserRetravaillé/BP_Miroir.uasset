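; BP_Miroir is a mirror on a pillar, likely for a laser puzzle, that the player can rotate and move.
; Its proximity zone registers it as the player's MiroirFocus.
; Timelines animate fixed-step pillar yaw rotation and slides between preset PointPosition spots, with TryMove choosing the spot best aligned with the look direction by dot product.
; DéplacerMiroir separately offers instant step movement relative to camera yaw.
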(event OnComponentBeginOverlap(ZoneProximite)
  (params (OverlappedComponent :type Primitive%20Component%20Object%20Reference) (OtherActor :type Actor%20Object%20Reference) (OtherComp :type Primitive%20Component%20Object%20Reference) (OtherBodyIndex :type Integer) (bFromSweep :type Boolean) (SweepResult :type Hit%20Result%20Structure%20%28by%20ref%29))
  (if (Utilities|DoesObjectImplementInterface OtherActor "/Game/Game/Blueprints/Interface/BPI_Interract.BPI_Interract_C")
    (Variables|/Game/Game/Blueprints/Characters/Cidara/BP_PlayerCidara.BP_PlayerCidara_C|SetMiroirFocus (Variables|Default|GetAs%20BP%20Player%20Cidara) self)))

(event OnComponentEndOverlap(ZoneProximite)
  (params (OverlappedComponent :type Primitive%20Component%20Object%20Reference) (OtherActor :type Actor%20Object%20Reference) (OtherComp :type Primitive%20Component%20Object%20Reference) (OtherBodyIndex :type Integer))
  (bind _as_bp_player_cidara (Variables|Default|GetAs%20BP%20Player%20Cidara))
  (if (Utilities|DoesObjectImplementInterface OtherActor "/Game/Game/Blueprints/Interface/BPI_Interract.BPI_Interract_C")
    (if (== (Variables|/Game/Game/Blueprints/Characters/Cidara/BP_PlayerCidara.BP_PlayerCidara_C|GetMiroirFocus _as_bp_player_cidara) self)
      (Variables|/Game/Game/Blueprints/Characters/Cidara/BP_PlayerCidara.BP_PlayerCidara_C|SetMiroirFocus _as_bp_player_cidara 0))))

(event Custom|MiroirRotation
  (Variables|Default|SetStartRotation (Transformation|GetWorldRotation (Variables|Default|GetPilier)))
  (Variables|Default|SetTragetRotation (Math|Rotator|MakeRotator 0.0 0.0 (+ (.Yaw (Math|Rotator|BreakRotator (Variables|Default|GetStartRotation))) 45.0)))
  (bind _alpha (Timeline|Timeline PlayFromStart)
    (:Update
      (Transformation|SetWorldRotation (Variables|Default|GetPilier) (Math|Rotator|Lerp(Rotator) (Variables|Default|GetStartRotation) (Variables|Default|GetTragetRotation) _alpha) false false))))

(event Custom|TryMove
  (params (PlayerLookDirection :type Vector))
  (Variables|DeplacementMiroir|SetPlayer%20Look%20Direction PlayerLookDirection)
  (Variables|DeplacementMiroir|SetBestDot 0.5)
  (Variables|DeplacementMiroir|SetBestIndex -1)
  (for (_array_element _array_index) (Variables|DeplacementMiroir|GetPointPosition)
    (if (not (== _array_index (Variables|DeplacementMiroir|GetCurrentIndex)))
      (if (> (Math|Vector|DotProduct (Math|Vector|Normalize (- _array_element (Transformation|GetActorLocation))) (Variables|DeplacementMiroir|GetPlayer%20Look%20Direction)) (Variables|DeplacementMiroir|GetBestDot))
        (Variables|DeplacementMiroir|SetBestDot (Math|Vector|DotProduct (Math|Vector|Normalize (- _array_element (Transformation|GetActorLocation))) (Variables|DeplacementMiroir|GetPlayer%20Look%20Direction)))
        (Variables|DeplacementMiroir|SetBestIndex _array_index))))
  (if (!= (Variables|DeplacementMiroir|GetBestIndex) -1)
    (Variables|DeplacementMiroir|SetCurrentIndex (Variables|DeplacementMiroir|GetBestIndex))
    (Variables|DeplacementMiroir|SetTragetPosition (Utilities|Array|Get(acopy) (Variables|DeplacementMiroir|GetPointPosition) (Variables|DeplacementMiroir|GetBestIndex)))
    (Variables|DeplacementMiroir|SetStartLocation (Transformation|GetActorLocation))
    (bind _alpha (Timeline|MoveTimeline PlayFromStart)
      (:Update
        (Transformation|SetActorLocation (Math|Vector|Lerp(Vector) (Variables|DeplacementMiroir|GetStartLocation) (Variables|DeplacementMiroir|GetTragetPosition) _alpha) false false)))))

(event EventBeginPlay
  (bind _asbp_player_cidara (Utilities|Casting|CastToBP_PlayerCidara (Game|GetPlayerCharacter 0)))
  (Variables|Default|SetAs%20BP%20Player%20Cidara _asbp_player_cidara)
  (if (> (Utilities|Array|Length (Variables|DeplacementMiroir|GetPointPosition)) 0)
    (Variables|DeplacementMiroir|SetCurrentIndex 0)
    (Transformation|SetActorLocation (Utilities|Array|Get(acopy) (Variables|DeplacementMiroir|GetPointPosition)) false false)))

(fn ConstructionScript)

(fn DéplacerMiroir
  (params (Direction :type Vector%202D%20Structure))
  (bind _returnvalue (Game|GetPlayerController 0))
  (bind _returnvalue_2 (Pawn|GetControlRotation _returnvalue :!class /Script/Engine.Controller))
  (bind _yaw (Math|Rotator|BreakRotator _returnvalue_2))
  (bind _returnvalue_3 (Math|Rotator|MakeRotator 0.0 0.0 _yaw))
  (Transformation|SetActorLocation (+ (Transformation|GetActorLocation) (+ (* (* (Math|Float|Round (.x Direction)) (Math|Vector|GetRightVector _returnvalue_3)) (Variables|Default|GetDéplacementPilier)) (* (* (Math|Float|Round (.y Direction)) (Math|Vector|GetForwardVector _returnvalue_3)) (Variables|Default|GetDéplacementPilier)))) false false))