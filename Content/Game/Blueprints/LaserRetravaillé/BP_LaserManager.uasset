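; Laser manager that steps through an array of laser emitters so they switch on in sequence, one room at a time.
; NextRoom deactivates the emitter at the current index, increments the index and activates the next one while it is within the array.
; BeginPlay calls NextRoom once; past the last emitter, nothing new activates.
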(event EventBeginPlay
  (CallFunction|NextRoom))

(fn ConstructionScript)

(fn NextRoom
  (if (and (>= (Variables|Default|GetCurrentIndex) 0) (< (Variables|Default|GetCurrentIndex) (Utilities|Array|Length (Variables|Default|GetEmitters))))
    (Default|Deactivate (Utilities|Array|Get(acopy) (Variables|Default|GetEmitters) (Variables|Default|GetCurrentIndex))))
  (Variables|Default|SetCurrentIndex (+ (Variables|Default|GetCurrentIndex) 1))
  (if (< (Variables|Default|GetCurrentIndex) (Utilities|Array|Length (Variables|Default|GetEmitters)))
    (Default|Activate (Utilities|Array|Get(acopy) (Variables|Default|GetEmitters) (Variables|Default|GetCurrentIndex)))))