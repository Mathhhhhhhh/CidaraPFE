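; BoxDilaogue is a dialogue trigger that plays a sequence of lines on the player's HUD when BP_PlayerCidara overlaps it.
; BPCDialogueComponent supplies each row's character, text and screen time, which the overlap and update events push to WBPHUD.
; DilaogueUpdate reads the next row and loops through a screen-time delay until the dialogue finishes and closes; the C key also triggers an update.
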(event OnComponentBeginOverlap(ActivationDialogue)
  (params (OverlappedComponent :type Primitive%20Component%20Object%20Reference) (OtherActor :type Actor%20Object%20Reference) (OtherComp :type Primitive%20Component%20Object%20Reference) (OtherBodyIndex :type Integer) (bFromSweep :type Boolean) (SweepResult :type Hit%20Result%20Structure%20%28by%20ref%29))
  (bind _bpc_dialoguecomponent (Variables|Default|GetBPC_DialogueComponent))
  (bind _asbp_player_cidara (Utilities|Casting|CastToBP_PlayerCidara OtherActor))
  (Default|GetCurrentDialogueRowData _bpc_dialoguecomponent)
  (bind _character (Default|GetCharacterFormCurrentRow _bpc_dialoguecomponent))
  (bind _long (Default|GetDialogueLongfromCurrentRow _bpc_dialoguecomponent))
  (Default|UpdateDialogue (Variables|/Game/Game/Blueprints/Characters/Cidara/BP_PlayerCidara.BP_PlayerCidara_C|GetWBP_HUD _asbp_player_cidara) _long _character)
  (Default|StartDialogue (Variables|/Game/Game/Blueprints/Characters/Cidara/BP_PlayerCidara.BP_PlayerCidara_C|GetWBP_HUD _asbp_player_cidara))
  (Class|BPIDialogueActivation|DilaogueUpdate(Message) self (stale EventDilaogueUpdate Player)))

(event Custom|DelayEvent
  (bind _readtime (Default|GetScreenTime (Variables|Default|GetBPC_DialogueComponent)))
  (Utilities|FlowControl|Delay _readtime)
  (Class|BPIDialogueActivation|DilaogueUpdate(Message) self (stale EventDilaogueUpdate Player))
  (Development|PrintString "je relance la boucle"))

(event EventDilaogueUpdate
  (params (Player :type BP%20Player%20Cidara%20Object%20Reference))
  (bind _bpc_dialoguecomponent (Variables|Default|GetBPC_DialogueComponent))
  (bind _wbp_hud (Variables|/Game/Game/Blueprints/Characters/Cidara/BP_PlayerCidara.BP_PlayerCidara_C|GetWBP_HUD Player))
  (Development|PrintString "1" true true "(R=0.000000,G=0.660000,B=1.000000,A=1.000000)" 1e+01)
  (bind _isfinished_ (Default|IsDialogueFinished _bpc_dialoguecomponent))
  (if _isfinished_
    (Development|PrintString "c'est fini" true true "(R=1.000000,G=0.830733,B=0.000000,A=1.000000)")
    (Default|EndDialogue _wbp_hud)
    (else
      (Development|PrintString "2" true true "(R=0.000000,G=0.660000,B=1.000000,A=1.000000)" 1e+01)
      (Default|ReadNextRow _bpc_dialoguecomponent)
      (Development|PrintString "3" true true "(R=0.000000,G=0.660000,B=1.000000,A=1.000000)" 1e+01)
      (Default|GetCurrentDialogueRowData _bpc_dialoguecomponent)
      (Development|PrintString "4" true true "(R=0.000000,G=0.660000,B=1.000000,A=1.000000)" 1e+01)
      (bind _character (Default|GetCharacterFormCurrentRow _bpc_dialoguecomponent))
      (Development|PrintString "5" true true "(R=0.000000,G=0.660000,B=1.000000,A=1.000000)" 1e+01)
      (bind _long (Default|GetDialogueLongfromCurrentRow _bpc_dialoguecomponent))
      (Development|PrintString "6" true true "(R=0.000000,G=0.660000,B=1.000000,A=1.000000)" 1e+01)
      (Default|UpdateDialogue _wbp_hud _long _character)
      (CallFunction|DelayEvent)
      (Development|PrintString "je lance delayevent"))))

(event Input|KeyboardEvents|C
  (params (Key :type Key%20Structure))
  (:Pressed
    (Class|BPIDialogueActivation|DilaogueUpdate(Message) self (stale EventDilaogueUpdate Player))))

(fn ConstructionScript)