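; Spectre, a playable shadow-bound character that climbs walls and broadcasts interactions to all interactable actors.
; BPCShadowDetection samples predicted positions to block or axis-filter input leaving shadow, and drives a reversible dissolve timeline that kills Spectre when finished.
; Death teleports it to a random safe spawn, or waits until Cidara stands in shadow to respawn behind her.
; Timed wall traces toggle flying-mode climbing, re-orienting the shadow grid to the wall.
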(event Custom|EvaluateClimb
  ;[0.15 0.15 0.15 0.5] Climbing
  (bind (_wallfound _wallnormalout) (CallFunction|DetectWall))
  (if (== (Variables|Default|GetisClimbing?) false)
    (if _wallfound
      (CallFunction|SnaptoWall)
      (CallFunction|EnterClimbMode _wallnormalout))
    (elif _wallfound
      (Variables|Default|SetWallNormal _wallnormalout)
      (Variables|Default|SetLastValidWallTime (Utilities|Time|GetGameTimeinSeconds))
      (CallFunction|SnaptoWall)
      (CallFunction|UpdateMeshFacing)
      (CallFunction|CheckExittoGround)
      (elif (> (- (Utilities|Time|GetGameTimeinSeconds) (Variables|Default|GetLastValidWallTime)) 0.5)
        (CallFunction|ExitClimbMode)))))

(event Custom|SpectreRespawnNearPlayer
  (bind _cidararef (Variables|Default|GetCidaraRef))
  ;[0.15 0.15 0.15 0.5] Si aucun safe spawn disponible vérifie si le joueur est a l'ombre, quand ce dernier est a l'ombre fait réapparaitre Spectre
  (bind _output_get (Variables|Default|SetSpawnNearPlayerLocation (+ (Transformation|GetActorLocation _cidararef) (* (Math|Vector|NegateVector (Math|Vector|GetForwardVector (Transformation|GetActorRotation _cidararef))) 1.5e+02))))
  (Transformation|SetActorLocation _output_get true false)
  (Variables|Default|SetWaitingForPlayerInShadow false)
  (Variables|Default|SetExposureTime 0.0)
  (CallFunction|SpectreHealUp))

(event Custom|SpectreDeath
  ;[0.15 0.15 0.15 0.5] Système de mort et de respawn pour spectre
  (Variables|Default|SetSunCheckEnabled false)
  (Variables|Default|SetExposureTime 0.0)
  (Utilities|FlowControl|Delay 1.5)
  (bind (_safespawn _foundsafe) (CallFunction|FindSafeSpawnPoint))
  (if _foundsafe
    (Transformation|SetActorLocation (+ (Transformation|GetActorLocation _safespawn) "0.000000,0.000000,50.000000") false true)
    (CallFunction|SpectreHealUp)
    (else
      (Variables|Default|SetWaitingForPlayerInShadow true)
      (Variables|Default|SetWaitingForShadowStartTime (Utilities|Time|GetGameTimeinSeconds))
      (Variables|Default|SetPlayerShadowCheckTimer 0.0))))

(event Custom|SpectreBurning
  ;[0.15 0.15 0.15 0.5] Effets visuels quand Spectre est exposé au soleil et quand elle reviens dans l'ombre
  (bind (_direction _alphadisolve) (Timeline|Timeline PlayFromStart)
    (:Update
      (Rendering|Material|SetScalarParameterValue (Variables|Default|GetSpectreMaterials) "Disolve" (Math|Float|Lerp -0.5 1.0 _alphadisolve) :!class /Script/Engine.MaterialInstanceDynamic))
    (:Finished
      (switch Utilities|FlowControl|Switch|SwitchonETimelineDirection _direction
        (:Forward
          (CallFunction|SpectreDeath))))))

(event Custom|SpectreHealUp
  ;[0.15 0.15 0.15 0.5] Effets visuels quand Spectre est exposé au soleil et quand elle reviens dans l'ombre
  (bind (_direction _alphadisolve) (Timeline|Timeline Reverse)
    (:Update
      (Rendering|Material|SetScalarParameterValue (Variables|Default|GetSpectreMaterials) "Disolve" (Math|Float|Lerp -0.5 1.0 _alphadisolve) :!class /Script/Engine.MaterialInstanceDynamic))
    (:Finished
      (switch Utilities|FlowControl|Switch|SwitchonETimelineDirection _direction
        (:Forward
          (CallFunction|SpectreDeath))))))

(event Custom|CheckPlayerInShadow
  ;[0.15 0.15 0.15 0.5] Si aucun safe spawn disponible vérifie si le joueur est a l'ombre, quand ce dernier est a l'ombre fait réapparaitre Spectre
  (if (Variables|Default|GetWaitingForPlayerInShadow)
    (bind _output_get (Variables|Default|SetPlayerShadowCheckTimer (+ (Variables|Default|GetPlayerShadowCheckTimer) (Utilities|Time|GetWorldDeltaSeconds))))
    (if (>= _output_get (Variables|Default|GetPlayerShadowCheckInterval))
      (Variables|Default|SetPlayerShadowCheckTimer 0.0)
      (if (Utilities|IsValid (Variables|Default|GetCidaraRef))
        (bind _isinshadow (CallFunction|CheckifPlayerIsinShadow (Transformation|GetActorLocation (Variables|Default|GetCidaraRef))))
        (if _isinshadow
          (CallFunction|SpectreRespawnNearPlayer))))))

(event Input|EnhancedActionEvents|EnhancedInputActionIA_SpectreMove
  (params (ActionValue :type Vector%202D%20Structure) (ElapsedSeconds :type Float%20%28double-precision%29) (TriggeredSeconds :type Float%20%28double-precision%29) (InputAction :type Input%20Action%20Object%20Reference :default "/Game/Game/Input/Actions/Spectre/IA_SpectreMove.IA_SpectreMove"))
  ;[1 1 1] Permet a Spectre de bouger
  (bind (_filteredinput _wasblocked) (CallFunction|ValidateMovementInput ActionValue))
  (if (not _wasblocked)
    (if (Variables|Default|GetIsClimbing?)
      (CallFunction|HandleClimbMovement _filteredinput)
      (else
        (CallFunction|HandleGroundedMovement _filteredinput)))))

(event Input|EnhancedActionEvents|EnhancedInputActionIA_SpectreInterract
  (params (ActionValue :type Boolean) (ElapsedSeconds :type Float%20%28double-precision%29) (TriggeredSeconds :type Float%20%28double-precision%29) (InputAction :type Input%20Action%20Object%20Reference :default "/Game/Game/Input/Actions/Spectre/IA_SpectreInterract.IA_SpectreInterract"))
  (:Started
    (bind _outactors (Actor|GetAllActorswithInterface "/Game/Game/Blueprints/Interface/BPI_Interract.BPI_Interract_C"))
    (Class|BPIInterract|Interract(Message) _outactors)))

(event EventBeginPlay
  (bind _bpc_shadowdetection (Variables|Default|GetBPC_ShadowDetection))
  (Utilities|FlowControl|Sequence
    (:then_0
      (bind _returnvalue (Actor|GetActorOfClass "/Game/Game/Blueprints/LightRune/BP_Sun.BP_Sun_C"))
      (Variables|Default|SetSunRef _returnvalue))
    (:then_1
      (bind _returnvalue_2 (Actor|GetActorOfClass "/Game/Game/Blueprints/Characters/Cidara/BP_PlayerCidara.BP_PlayerCidara_C"))
      (Variables|Default|SetCidaraRef _returnvalue_2))
    (:then_2
      (EventDispatchers|BindEventtoOnExitedShadow _bpc_shadowdetection (delegate Custom|SpectreBurning))
      (EventDispatchers|BindEventtoOnEnteredShadow _bpc_shadowdetection (delegate Custom|SpectreHealUp)))
    (:then_3)
    (:then_4
      (Variables|Default|SetLastValidPosition (Transformation|GetActorLocation)))
    (:then_5
      (Utilities|Time|SetTimerbyEvent 0 0.02 true))
    (:then_6
      (Utilities|Time|SetTimerbyEvent (delegate Custom|CheckPlayerInShadow) 0.05 true)
      (Utilities|Time|SetTimerbyEvent (delegate Custom|EvaluateClimb) 0.1 true))
    (:then_7
      (Rendering|SetActorHiddenInGame false)
      (Collision|SetActorEnableCollision true))))

(event EventPossessed
  (params (NewController :type Controller%20Object%20Reference))
  (Default|ResetShadowState (Variables|Default|GetBPC_ShadowDetection)))

(event EventUnpossessed
  (params (OldController :type Controller%20Object%20Reference))
  (Default|CleanUpGraceTimer (Variables|Default|GetBPC_ShadowDetection)))

(fn ConstructionScript)

(fn CheckifPositionIsSafe
  (params (PositionToCheck :type Vector))
  (LocalVariables|SetExposedPoint 0)
  (for _array_element 0
    (LocalVariables|SetTraceStart (+ PositionToCheck _array_element))
    (LocalVariables|SetTraceEnd (* (* (Variables|/Game/Game/Blueprints/LightRune/BP_Sun.BP_Sun_C|GetSunDirection (Variables|Default|GetSunRef)) -1.0) (Variables|Default|GetTraceDistance)))
    (bind _returnvalue (Collision|LineTraceByChannel (LocalVariables|GetTraceStart) (LocalVariables|GetTraceEnd) "TraceTypeQuery1" false 0 "None"))
    (if (not _returnvalue)
      (LocalVariables|SetExposedPoint (+ (LocalVariables|GetExposedPoint) 1))))
  (if (>= (LocalVariables|GetExposedPoint) 4)
    (return false)
    (else
      (return true))))

(fn FindSafeSpawnPoint
  (bind _safespawnpoints (LocalVariables|GetSafeSpawnPoints))
  (bind _returnvalue (Utilities|Array|Length _safespawnpoints))
  (bind _outactors (Actor|GetAllActorsOfClasswithTag "/Game/Game/Blueprints/Characters/Spectre/BP_SafeSpawn.BP_SafeSpawn_C" "SpectreSpawn"))
  (for _array_element _outactors
    (if (== (Variables|/Game/Game/Blueprints/Characters/Spectre/BP_SafeSpawn.BP_SafeSpawn_C|GetIsCurrentlySafe _array_element) true)
      (Utilities|Array|Add (LocalVariables|GetSafeSpawnPoints) _array_element)))
  (if (> _returnvalue 0)
    (return (Utilities|Array|Get(acopy) (LocalVariables|GetSafeSpawnPoints) (Math|Random|RandomIntegerinRange 0 (- _returnvalue 1))) true)
    (else
      (return 0 false))))

(fn CheckifPlayerIsinShadow
  (params (PlayerLocation :type Vector))
  (for _array_element (Utilities|Array|MakeArray "0.000000,0.000000,100.000000" "50.000000,0.000000,80.000000" "-50.000000,0.000000,80.000000" "0.000000,50.000000,80.000000" "0.000000,-50.000000,80.000000")
    (bind _isinligth (Default|IsPointinLigthSimple (Variables|Default|GetBPC_ShadowDetection) (+ PlayerLocation _array_element)))
    (if _isinligth
      (Math|Integer|IncrementInt (LocalVariables|GetExposedPoint))))
  (if (>= (LocalVariables|GetExposedPoint) 2)
    (return false)
    (else
      (return true))))

(fn CalculateNextPosition
  (params (InputVector :type Vector%202D%20Structure))
  (bind _returnvalue (Pawn|GetControlRotation :!class /Script/Engine.Pawn))
  (bind (_x _y) (Math|Vector2D|BreakVector2D InputVector))
  (bind _returnvalue_2 (Math|Rotator|MakeRotator 0.0 0.0 (.yaw _returnvalue)))
  (if (Variables|Default|GetisClimbing?)
    (LocalVariables|SetWorldForward "0.000000,0.000000,1.000000")
    (LocalVariables|SetWorldRight (Variables|/Game/Game/Blueprints/System/Shadows/BPC_ShadowDetection.BPC_ShadowDetection_C|GetGrid%20XAxis (Variables|Default|GetBPC_ShadowDetection)))
    (elif (Utilities|IsValid (Pawn|GetController))
      (LocalVariables|SetWorldForward (Math|Vector|GetForwardVector _returnvalue_2))
      (LocalVariables|SetWorldRight (Math|Vector|GetRightVector _returnvalue_2))
      (else
        (LocalVariables|SetWorldForward (Transformation|GetActorForwardVector))
        (LocalVariables|SetWorldRight (Transformation|GetActorRightVector)))))
  (bind _output_get (LocalVariables|SetMoveDirection (+ (* (LocalVariables|GetWorldForward) _y) (* (LocalVariables|GetWorldRight) _x))))
  (if (< (Math|Vector|VectorLength _output_get) 1.0)
    (return (Transformation|GetActorLocation))
    (else
      (return (+ (Transformation|GetActorLocation) (* (Math|Vector|Normalize _output_get) (Variables|Default|GetPredictionDistanceOffset)))))))

(fn ValidateMovementInput
  (params (RawInput :type Vector%202D%20Structure))
  (bind (_x _y) (Math|Vector2D|BreakVector2D RawInput))
  (bind _bpc_shadowdetection (Variables|Default|GetBPC_ShadowDetection))
  (bind _bpc_shadowdetection_2 (Variables|Default|GetBPC_ShadowDetection))
  (bind _bpc_shadowdetection_3 (Variables|Default|GetBPC_ShadowDetection))
  (LocalVariables|SetRawX _x)
  (LocalVariables|SetRawY _y)
  (bind _predictedlocation (CallFunction|CalculateNextPosition RawInput))
  (if (Variables|Default|GetisClimbing?)
    (bind _isinshadow (Default|IsPointinShadowSamples _bpc_shadowdetection_2 _predictedlocation (Variables|/Game/Game/Blueprints/System/Shadows/BPC_ShadowDetection.BPC_ShadowDetection_C|GetGrid%20Yaxis _bpc_shadowdetection_2) (Variables|/Game/Game/Blueprints/System/Shadows/BPC_ShadowDetection.BPC_ShadowDetection_C|GetGrid%20XAxis _bpc_shadowdetection_2)))
    (if _isinshadow
      (return RawInput false))
    (else
      (bind _isinshadow_2 (Default|IsPointinShadowSamples _bpc_shadowdetection_2 _predictedlocation "1.000000,0.000000,0.000000" "0.000000,1.000000,0.000000"))
      (if _isinshadow_2
        (return RawInput false)
        (else
          (Utilities|FlowControl|Sequence
            (:then_0
              (bind _predictedlocation_2 (CallFunction|CalculateNextPosition (Math|Vector2D|MakeVector2D (LocalVariables|GetRawX) 0.0)))
              (if (Variables|Default|GetisClimbing?)
                (bind _isinshadow_3 (Default|IsPointinShadowSamples _bpc_shadowdetection_3 _predictedlocation_2 (Variables|/Game/Game/Blueprints/System/Shadows/BPC_ShadowDetection.BPC_ShadowDetection_C|GetGrid%20Yaxis _bpc_shadowdetection_3) (Variables|/Game/Game/Blueprints/System/Shadows/BPC_ShadowDetection.BPC_ShadowDetection_C|GetGrid%20XAxis _bpc_shadowdetection_3)))
                (LocalVariables|SetXSafe _isinshadow_3)
                (else
                  (bind _isinshadow_4 (Default|IsPointinShadowSamples _bpc_shadowdetection_3 _predictedlocation_2 "1.000000,0.000000,0.000000" "0.000000,1.000000,0.000000"))
                  (LocalVariables|SetXSafe _isinshadow_4))))
            (:then_1
              (bind _predictedlocation_3 (CallFunction|CalculateNextPosition (Math|Vector2D|MakeVector2D 0.0 (LocalVariables|GetRawY))))
              (if (Variables|Default|GetisClimbing?)
                (bind _isinshadow_5 (Default|IsPointinShadowSamples _bpc_shadowdetection _predictedlocation_3 (Variables|/Game/Game/Blueprints/System/Shadows/BPC_ShadowDetection.BPC_ShadowDetection_C|GetGrid%20Yaxis _bpc_shadowdetection) (Variables|/Game/Game/Blueprints/System/Shadows/BPC_ShadowDetection.BPC_ShadowDetection_C|GetGrid%20XAxis _bpc_shadowdetection)))
                (LocalVariables|SetYSafe _isinshadow_5)
                (else
                  (bind _isinshadow_6 (Default|IsPointinShadowSamples _bpc_shadowdetection _predictedlocation_3 "1.000000,0.000000,0.000000" "0.000000,1.000000,0.000000"))
                  (LocalVariables|SetYSafe _isinshadow_6)))))
          (bind _output_get (LocalVariables|SetLocalBlocked true))
          (return (Math|Vector2D|MakeVector2D (Math|Float|SelectFloat (LocalVariables|GetRawX) 0.0 (LocalVariables|GetXSafe)) (Math|Float|SelectFloat (LocalVariables|GetRawY) 0.0 (LocalVariables|GetYSafe))) _output_get))))))

(fn DetectWall
  (bind _returnvalue (Transformation|GetActorLocation))
  (bind _returnvalue_2 (+ _returnvalue "0.000000,0.000000,50.000000"))
  (if (Utilities|Operators|EqualEqual :A (Transformation|GetVelocity))
    (return false "0, 0, 0" "0, 0, 0")
    (else
      (bind (_outhit _returnvalue_3) (Collision|SphereTraceByChannel _returnvalue_2 (+ _returnvalue_2 (* (Math|Vector|GetForwardVector (Variables|Default|GetArrowCaps)) (Variables|Default|GetWallDetectionDistance))) (Variables|Default|GetWallDetectionRadius) "TraceTypeQuery6" false 0 "None"))
      (if _returnvalue_3
        (Math|Float|CompareFloat (Math|Float|Absolute(Float) (Math|Vector|DotProduct (.ImpactNormal (Collision|BreakHitResult _outhit)) "0.000000,0.000000,1.000000")) (Variables|Default|GetMinClimbDot)
          (:>
            (return false "0, 0, 0" "0, 0, 0"))
          (:<
            (return true (Math|Vector|Normalize (.ImpactNormal (Collision|BreakHitResult _outhit))) (Math|Vector|Normalize (.ImpactPoint (Collision|BreakHitResult _outhit))))))
        (else
          (return false "0, 0, 0" "0, 0, 0"))))))

(fn EnterClimbMode
  (params (WallNormal :type Vector))
  (bind _bpc_shadowdetection (Variables|Default|GetBPC_ShadowDetection))
  (bind _charactermovement (Variables|Character|GetCharacterMovement))
  (Variables|Default|SetWallDetectionDistance 3.5e+02)
  (if (Variables|Default|GetisClimbing?)
    (Variables|Default|SetWallNormal WallNormal)
    (return)
    (else
      (Variables|Default|SetisClimbing? true)
      (Variables|Default|SetWallNormal WallNormal)
      (Pawn|Components|CharacterMovement|SetMovementMode _charactermovement "MOVE_Flying" 0)
      (Variables|/Script/Engine.CharacterMovementComponent|SetGravityScale _charactermovement 0.0)
      (Variables|/Script/Engine.CharacterMovementComponent|SetbOrientRotationToMovement _charactermovement false)
      (Variables|/Game/Game/Blueprints/System/Shadows/BPC_ShadowDetection.BPC_ShadowDetection_C|SetGrid%20Yaxis _bpc_shadowdetection "0.000000,0.000000,1.000000")
      (Variables|/Game/Game/Blueprints/System/Shadows/BPC_ShadowDetection.BPC_ShadowDetection_C|SetGrid%20XAxis _bpc_shadowdetection (Math|Vector|Normalize (Math|Vector|CrossProduct (Variables|Default|GetWallNormal) "0.000000,0.000000,1.000000")))
      (Transformation|SetActorRotation (Math|Interpolation|RInterpTo (Transformation|GetActorRotation) (Math|Rotator|MakeRotationfromAxes (Math|Vector|NegateVector (Variables|Default|GetWallNormal)) (Math|Vector|Normalize (Math|Vector|CrossProduct "0.000000,0.000000,1.000000" (Variables|Default|GetWallNormal))) (Math|Vector|Normalize (Math|Vector|CrossProduct (Variables|Default|GetWallNormal) (Math|Vector|Normalize (Math|Vector|CrossProduct "0.000000,0.000000,1.000000" (Variables|Default|GetWallNormal)))))) (Utilities|Time|GetWorldDeltaSeconds) (Variables|Default|GetRotationInterpSpeed)))
      (Variables|Default|SetClimbStartTime (Utilities|Time|GetGameTimeinSeconds))
      (return))))

(fn ExitClimbMode
  (bind _charactermovement (Variables|Character|GetCharacterMovement))
  (bind _bpc_shadowdetection (Variables|Default|GetBPC_ShadowDetection))
  (Variables|Default|SetWallDetectionDistance 1.5e+02)
  (if (Variables|Default|GetisClimbing?)
    (Variables|Default|SetisClimbing? false)
    (Variables|Default|SetWallNormal "0, 0, 0")
    (Pawn|Components|CharacterMovement|SetMovementMode _charactermovement "MOVE_Walking" 0)
    (Variables|/Script/Engine.CharacterMovementComponent|SetGravityScale _charactermovement 1.0)
    (Variables|/Script/Engine.CharacterMovementComponent|SetbOrientRotationToMovement _charactermovement true)
    (Variables|/Game/Game/Blueprints/System/Shadows/BPC_ShadowDetection.BPC_ShadowDetection_C|SetGrid%20XAxis _bpc_shadowdetection "1.000000,0.000000,0.000000")
    (Variables|/Game/Game/Blueprints/System/Shadows/BPC_ShadowDetection.BPC_ShadowDetection_C|SetGrid%20Yaxis _bpc_shadowdetection "0.000000,1.000000,0.000000")
    (Transformation|SetRelativeRotation (Variables|Character|GetMesh) "0.000000,-90.000000,0.000000" false false)))

(fn GetScreenSpaceInputDirection
  (params (InputAxis :type Vector%202D%20Structure))
  (bind (_x _y) (Math|Vector2D|BreakVector2D InputAxis))
  (bind _output_get (LocalVariables|SetCamRot (Camera|GetCameraRotation (Game|GetPlayerCameraManager 0))))
  (return (Math|Vector|Normalize (+ (* (Math|Vector|GetRightVector _output_get) _x) (* (Math|Vector|GetUpVector _output_get) _y)))))

(fn HandleGroundedMovement
  (params (InputAxis :type Vector%202D%20Structure))
  (bind _screendirection (CallFunction|GetScreenSpaceInputDirection InputAxis))
  (Pawn|Input|AddMovementInput (Math|Vector|Normalize (Math|Vector|MakeVector (.x _screendirection) (.y _screendirection) 0.0)) 1.0 false))

(fn HandleClimbMovement
  (params (InputAxis :type Vector%202D%20Structure))
  (bind _returnvalue (Game|GetPlayerCameraManager 0))
  (bind _wallnormal (Variables|Default|GetWallNormal))
  (bind _returnvalue_2 (Camera|GetCameraRotation _returnvalue))
  (bind _returnvalue_3 (Math|Vector|CrossProduct "0.000000,0.000000,1.000000" _wallnormal))
  (bind _returnvalue_4 (Math|Vector|Normalize _returnvalue_3))
  (bind _returnvalue_5 (Math|Vector|CrossProduct _wallnormal _returnvalue_4))
  (bind _returnvalue_6 (Math|Vector|Normalize _returnvalue_5))
  (bind _screendirection (CallFunction|GetScreenSpaceInputDirection (Math|Vector2D|MakeVector2D (.x InputAxis) (.y InputAxis))))
  (bind _output_get (Variables|Default|SetLastClimbMoveDir (Math|Vector|Normalize (+ (* _returnvalue_4 (* (.x InputAxis) (Math|Float|Sign(Float) (Math|Vector|DotProduct (Math|Vector|GetRightVector _returnvalue_2) _returnvalue_4)))) (* _returnvalue_6 (* (.y InputAxis) (Math|Float|Sign(Float) (Math|Vector|DotProduct (Math|Vector|GetUpVector _returnvalue_2) _returnvalue_6))))))))
  (Pawn|Input|AddMovementInput (+ _screendirection _output_get) 1.0 false))

(fn SnaptoWall
  (bind _returnvalue (Transformation|GetActorLocation))
  (bind _returnvalue_2 (Transformation|GetActorLocation))
  (if (Utilities|Operators|NotEqual(!=) :A (Variables|Default|GetWallNormal) :ErrorTolerance 0.01)
    (bind (_outhit _returnvalue_3) (Collision|LineTraceByChannel _returnvalue_2 (+ _returnvalue_2 (* (* (Variables|Default|GetWallNormal) -1.0) (Variables|Default|GetStickTraceLength))) "TraceTypeQuery6" false 0 "None" true "(R=0.370274,G=0.000000,B=1.000000,A=1.000000)" "(R=1.000000,G=0.000000,B=0.287168,A=1.000000)"))
    (if _returnvalue_3
      (if (not (> (Math|Float|Absolute(Float) (Math|Vector|DotProduct (.ImpactNormal (Collision|BreakHitResult _outhit)) "0.000000,0.000000,1.000000")) 0.7))
        (if (not (< (Math|Vector|DotProduct (.ImpactNormal (Collision|BreakHitResult _outhit)) (Variables|Default|GetWallNormal)) 0.0))
          (if (not (> (Math|Vector|Distance(Vector) (Transformation|GetActorLocation) (+ (.ImpactPoint (Collision|BreakHitResult _outhit)) (* (.ImpactNormal (Collision|BreakHitResult _outhit)) (Variables|Default|GetStickDistance)))) (Variables|Default|GetMaxSnapPerFrame)))
            (Variables|Default|SetWallNormal (.ImpactNormal (Collision|BreakHitResult _outhit)))
            (if (> (Math|Vector|Distance(Vector) "0, 0, 0" "0, 0, 0") 25.0)
              (Transformation|SetActorLocation (Math|Interpolation|VInterpTo _returnvalue (* (+ _returnvalue (Math|Vector|Normalize (- "" ""))) 25.0) (Utilities|Time|GetWorldDeltaSeconds) (Variables|Default|GetStickInterpSpeed)) true false)
              (else
                (Transformation|SetActorLocation (Math|Interpolation|VInterpTo "0, 0, 0" "0, 0, 0" (Utilities|Time|GetWorldDeltaSeconds) (Variables|Default|GetStickInterpSpeed)) true false)))))))))

(fn UpdateMeshFacing
  (bind _wallnormal (Variables|Default|GetWallNormal))
  (bind _mesh (Variables|Character|GetMesh))
  (bind _returnvalue (Math|Vector|CrossProduct "0.000000,0.000000,1.000000" _wallnormal))
  (bind _returnvalue_2 (Math|Vector|Normalize _returnvalue))
  (bind _output_get (LocalVariables|SetVelocity (Variables|/Script/Engine.MovementComponent|GetVelocity (Variables|Character|GetCharacterMovement))))
  (if (> (Math|Vector|VectorLength _output_get) 1e+01)
    (Transformation|SetRelativeRotation _mesh (Math|Interpolation|RInterpTo (Variables|/Script/Engine.SceneComponent|GetRelativeRotation _mesh) (Math|Rotator|MakeRotator 0.0 0.0 (- (* (Math|Trig|Atan2(Radians) (Math|Vector|DotProduct (LocalVariables|GetVelocity) (Math|Vector|Normalize (Math|Vector|CrossProduct _wallnormal _returnvalue_2))) (Math|Vector|DotProduct (LocalVariables|GetVelocity) _returnvalue_2)) (/ 1.8e+02 (Math|Trig|GetPI))) -9e+01)) (Utilities|Time|GetWorldDeltaSeconds) (Variables|Default|GetRotationInterpSpeed)) false false)))

(fn CheckExittoGround
  (bind _returnvalue (Transformation|GetActorLocation))
  (bind _groundexitdistance (Variables|Default|GetGroundExitDistance))
  (if (< (Variables|Default|GetGroundExitMinTimeInClimb) (- (Utilities|Time|GetGameTimeinSeconds) (Variables|Default|GetClimbStartTime)))
    (bind (_outhit _returnvalue_2) (Collision|LineTraceByChannel _returnvalue (+ _returnvalue (Math|Vector|MakeVector 0.0 0.0 (* _groundexitdistance -1e+01))) "TraceTypeQuery1" false 0 "ForDuration"))
    (if _returnvalue_2
      (Development|PrintString (Utilities|String|ToString(Float) (.Distance (Collision|BreakHitResult _outhit))))
      (if (<= (.Distance (Collision|BreakHitResult _outhit)) _groundexitdistance)
        (CallFunction|ExitClimbMode)))))