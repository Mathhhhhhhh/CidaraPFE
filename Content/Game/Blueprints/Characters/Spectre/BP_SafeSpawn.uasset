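; BP_SafeSpawn is a spawn-point actor, filed under Spectre, that tracks whether its location is shaded from the sun.
; On BeginPlay it finds BP_Sun and starts a looping timer that runs CheckIfSafe.
; While active, that check traces toward the sun from a 3x3 grid of points around the actor.
; IsCurrentlySafe turns false when at least two traces are unblocked or the actor is inactive.
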(event EventBeginPlay
  (bind _returnvalue (Actor|GetActorOfClass "/Game/Game/Blueprints/LightRune/BP_Sun.BP_Sun_C"))
  (Variables|Default|SetSunRef _returnvalue)
  (Utilities|Time|SetTimerbyFunctionName 0 "CheckIfSafe" 0.5 true))

(event Collision|EventActorBeginOverlap
  (params (OtherActor :type Actor%20Object%20Reference)))

(event EventTick
  (params (DeltaSeconds :type Float%20%28single-precision%29)))

(fn ConstructionScript)

(fn CheckifSafe
  (if (Variables|Default|GetIsActive)
    (if (Utilities|IsValid (Variables|Default|GetSunRef))
      (for _array_element (Utilities|Array|MakeArray "0, 0, 0" "100.000000,0.000000,0.000000" "-100.000000,0.000000,0.000000" "0.000000,100.000000,0.000000" "0.000000,-100.000000,0.000000" "100.000000,100.000000,0.000000" "-100.000000,100.000000,0.000000" "-100.000000,-100.000000,0.000000" "100.000000,-100.000000,0.000000")
        (bind _returnvalue (Collision|LineTraceByChannel (+ (Transformation|GetActorLocation) _array_element) (+ (+ (Transformation|GetActorLocation) _array_element) (* (Math|Vector|NegateVector (Transformation|GetActorForwardVector (Variables|Default|GetSunRef))) 5e+03)) "TraceTypeQuery5" false 0 "None" true "(R=0.686766,G=1.000000,B=0.000000,A=1.000000)" "(R=1.000000,G=0.000000,B=0.088168,A=1.000000)" 0.5))
        (if (not _returnvalue)
          (Math|Integer|IncrementInt (Variables|Default|GetExposedPoint))))
      (if (>= (Variables|Default|GetExposedPoint) 2)
        (Variables|Default|SetIsCurrentlySafe false)
        (else
          (Variables|Default|SetIsCurrentlySafe true))))
    (else
      (Variables|Default|SetIsCurrentlySafe false))))