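; Base door actor that slides from a start point to an end point when its OpenDoor event is called.
; BeginPlay caches the world locations of the StartPoint and EndPoint components, so the path stays fixed as the actor moves.
; After a short delay, OpenDoor plays a timeline that lerps the whole actor between those locations with sweep enabled.
; The graph contains no closing logic.
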(event Custom|OpenDoor
  ;[0.15 0.15 0.15 0.5] Set la localisation de l'actor
  (Utilities|FlowControl|Delay 0.2)
  (bind _value (Timeline|Timeline Play)
    (:Update
      (Transformation|SetActorLocation (Math|Vector|Lerp(Vector) (Variables|Default|GetStartLocation) (Variables|Default|GetEndLocation) _value) true false))))

(event EventBeginPlay
  ;[0.15 0.15 0.15 0.5] Set le start et end localisation
  (Variables|Default|SetStartLocation (Transformation|GetWorldLocation (Variables|Default|GetStartPoint)))
  (Variables|Default|SetEndLocation (Transformation|GetWorldLocation (Variables|Default|GetEndPoint))))

(fn ConstructionScript)