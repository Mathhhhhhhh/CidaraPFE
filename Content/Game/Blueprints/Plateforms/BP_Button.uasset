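; BP_Button is an interactable button that lowers an elevator platform and opens the labyrinth door.
; Its Interract event checks that the player character is within ActivateRange of the button's root component.
; If so, it calls MovePlateformDown on the referenced platform, then OpenDoor on the referenced door.
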(event EventInterract
  ;[0.15 0.15 0.15 0.5] Faire descendeur l'ascenseur et l'ouvrir la porte du labyrinth
  (if (<= (Math|Vector|Distance(Vector) (Transformation|GetActorLocation (Game|GetPlayerCharacter 0)) (Transformation|GetWorldLocation (Variables|Default|GetDefaultSceneRoot))) (Variables|Default|GetActivateRange))
    (Utilities|FlowControl|Sequence
      (:then_0
        (Default|MovePlateformDown (Variables|Default|GetBP_Plateform)))
      (:then_1
        (Default|OpenDoor (Variables|Default|GetBP_Door))))))

(fn ConstructionScript)