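; Platform block actor that moves between the positions marked by its Start and End components.
; On BeginPlay it caches both world locations and plays a timeline, whose Nav track lerps the actor from start to end without sweep.
; Each timeline update also sets the actor's rotation to End's current world rotation, read live rather than cached or interpolated.
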(event EventBeginPlay
  (Variables|Default|SetStartLocation (Transformation|GetWorldLocation (Variables|Default|GetStart)))
  (Variables|Default|SetEndLocation (Transformation|GetWorldLocation (Variables|Default|GetEnd)))
  (bind _nav (Timeline|Timeline Play)
    (:Update
      (Transformation|SetActorRotation (Transformation|GetWorldRotation (Variables|Default|GetEnd)))
      (Transformation|SetActorLocation (Math|Vector|Lerp(Vector) (Variables|Default|GetStartLocation) (Variables|Default|GetEndLocation) _nav) false false))))

(fn ConstructionScript)