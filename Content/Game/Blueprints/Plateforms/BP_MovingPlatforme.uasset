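; BP_MovingPlatforme is a moving platform that travels along a spline after an interacting actor touches its trigger.
; When the Box overlap begins with an actor implementing BPI_Interract, it waits for a configurable Duration, then plays a timeline.
; The timeline's Nav track scales the spline length, and each update moves the Platform component to that world location along the path without sweeping.
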(event OnComponentBeginOverlap(Box)
  (params (OverlappedComponent :type Primitive%20Component%20Object%20Reference) (OtherActor :type Actor%20Object%20Reference) (OtherComp :type Primitive%20Component%20Object%20Reference) (OtherBodyIndex :type Integer) (bFromSweep :type Boolean) (SweepResult :type Hit%20Result%20Structure%20%28by%20ref%29))
  (if (Utilities|DoesObjectImplementInterface OtherActor "/Game/Game/Blueprints/Interface/BPI_Interract.BPI_Interract_C")
    (Utilities|FlowControl|Delay (Variables|Default|GetDuration))
    (Variables|Default|SetSplineLength (Spline|GetSplineLength (Variables|Default|GetSpline)))
    (bind _nav (Timeline|Timeline_0 Play)
      (:Update
        (Transformation|SetWorldLocation (Variables|Default|GetPlatform) (Spline|GetLocationatDistanceAlongSpline (Variables|Default|GetSpline) (* _nav (Variables|Default|GetSplineLength)) "World") false false)))))

(event EventBeginPlay)

(fn ConstructionScript)