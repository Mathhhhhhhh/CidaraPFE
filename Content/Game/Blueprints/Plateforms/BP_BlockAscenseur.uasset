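; BP_BlockAscenseur is an elevator block platform that travels from a start marker to an end marker.
; BeginPlay caches the world locations of the Start and End components.
; The MovingPlatform event plays a timeline that lerps the actor between them with sweep.
; The same alpha blends rotation from Block's current world rotation, re-read each update, toward Repaire's relative rotation along the shortest path.
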(event Custom|MovingPlatform
  ;[1 1 1 0.5] Faire bouger l'actor
  (bind _nav (Timeline|Timeline Play)
    (:Update
      (Transformation|SetActorLocation (Math|Vector|Lerp(Vector) (Variables|Default|GetStartLocation) (Variables|Default|GetEndLocation) _nav) true false)
      (Transformation|SetActorRotation (Math|Rotator|Lerp(Rotator) (Transformation|GetWorldRotation (Variables|Default|GetBlock)) (Variables|/Script/Engine.SceneComponent|GetRelativeRotation (Variables|Default|GetRepaire)) _nav true)))))

(event EventBeginPlay
  ;[1 1 1 0.5] Set les variables départ et d'arriver
  (Variables|Default|SetStartLocation (Transformation|GetWorldLocation (Variables|Default|GetStart)))
  (Variables|Default|SetEndLocation (Transformation|GetWorldLocation (Variables|Default|GetEnd))))

(fn ConstructionScript)