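; BP_Plateform is a moving platform actor that travels from a start point to an end point.
; On BeginPlay it caches both point components' world locations, then starts moving if MoveOnStart is set.
; The MovePlateformDown event waits a delay, then plays a Timeline whose alpha lerps the actor's location between the cached points, with sweep enabled.
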(event Custom|MovePlateformDown
  ;[0.15 0.15 0.15 0.5] DelayBeforeMove
  (Utilities|FlowControl|Delay (Variables|Default|GetDuration))
  (bind _alpha (Timeline|Timeline Play)
    (:Update
      (Transformation|SetActorLocation (Math|Vector|Lerp(Vector) (Variables|Default|GetStartLocation) (Variables|Default|GetEndLocation) _alpha) true false))))

(event EventBeginPlay
  (Utilities|FlowControl|Sequence
    (:then_0
      (Variables|Default|SetStartLocation (Transformation|GetWorldLocation (Variables|Default|GetStartPont)))
      (Variables|Default|SetEndLocation (Transformation|GetWorldLocation (Variables|Default|GetEndPoint))))
    (:then_1
      (if (Variables|Default|GetMoveOnStart?)
        (CallFunction|MovePlateformDown)))))

(fn ConstructionScript)