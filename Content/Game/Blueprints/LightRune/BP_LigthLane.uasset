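; BP_LigthLane is a LightRune actor with a rect light and a Locked state that selects between fade-out and fade-in.
; On BeginPlay it caches the light's intensity and attenuation radius, then calls SwitchState with its Locked value.
; SwitchState fires fade events that reverse the TL_FadeLigth timeline when locked or play it from start when unlocked.
; The graph shows no timeline update logic applying the fade to the light.
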(event Custom|FAdeoutLigth
  (Timeline|TL_FadeLigth Reverse))

(event Custom|FAdeInLigth
  (Timeline|TL_FadeLigth PlayFromStart))

(event EventBeginPlay
  (bind _rectlight (Variables|Default|GetRectLight))
  (Variables|Default|SetIntensity (Variables|/Script/Engine.LightComponentBase|GetIntensity _rectlight))
  (Variables|Default|SetAttenuation%20Radius (Variables|/Script/Engine.LocalLightComponent|GetAttenuationRadius _rectlight))
  (if (Variables|Default|GetLocked)
    (CallFunction|SwitchState true)
    (else
      (CallFunction|SwitchState false))))

(event Collision|EventActorBeginOverlap
  (params (OtherActor :type Actor%20Object%20Reference)))

(event EventTick
  (params (DeltaSeconds :type Float%20%28single-precision%29)))

(fn ConstructionScript)

(fn SwitchState
  (params (Locked :type Boolean))
  (if Locked
    (CallFunction|FAdeoutLigth)
    (else
      (CallFunction|FAdeinLigth))))