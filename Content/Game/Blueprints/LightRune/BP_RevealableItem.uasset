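; BP_RevealableItem is an item that fades and deforms in and out through its material when reveal is started or stopped.
; On BeginPlay it creates a dynamic instance of M_Revealable on its static mesh, with FadeOpacity and Deform at zero.
; StartReveal plays and StopReveal reverses a timeline that drives both parameters from one track.
; When the timeline finishes, its direction determines whether IsRevealed is set or cleared.
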(event EventBeginPlay
  ;[0.15 0.15 0.15 0.5] Prépare le material utilisé
  (bind _returnvalue (Rendering|Material|CreateDynamicMaterialInstance (Variables|Default|GetStaticMesh) 0 "/Game/Game/Materials/VFX/LightRune/M_Revealable.M_Revealable" "None" :!class /Script/Engine.PrimitiveComponent))
  (bind _output_get (Variables|Default|SetDynamicMaterials _returnvalue))
  (Rendering|Material|SetScalarParameterValue _output_get "FadeOpacity" 0.0 :!class /Script/Engine.MaterialInstanceDynamic)
  (Rendering|Material|SetScalarParameterValue _output_get "Deform" 0.0 :!class /Script/Engine.MaterialInstanceDynamic))

(event EventStartReveal
  (bind _dynamicmaterials (Variables|Default|GetDynamicMaterials))
  ;[0.15 0.15 0.15 0.5] Gère la visibilité de l'objet
  (bind _newtrack_0 (Timeline|TL_Fade Play)
    (:Update
      (Rendering|Material|SetScalarParameterValue _dynamicmaterials "FadeOpacity" _newtrack_0 :!class /Script/Engine.MaterialInstanceDynamic)
      (Rendering|Material|SetScalarParameterValue _dynamicmaterials "Deform" _newtrack_0 :!class /Script/Engine.MaterialInstanceDynamic))
    (:Finished
      (switch Utilities|FlowControl|Switch|SwitchonETimelineDirection "Forward"
        (:Forward
          (CallFunction|OnFullyRevealed))
        (:Backward
          (CallFunction|OnFullyHidden))))))

(event EventStopReveal
  (bind _dynamicmaterials (Variables|Default|GetDynamicMaterials))
  ;[0.15 0.15 0.15 0.5] Gère la visibilité de l'objet
  (bind _newtrack_0 (Timeline|TL_Fade Reverse)
    (:Update
      (Rendering|Material|SetScalarParameterValue _dynamicmaterials "FadeOpacity" _newtrack_0 :!class /Script/Engine.MaterialInstanceDynamic)
      (Rendering|Material|SetScalarParameterValue _dynamicmaterials "Deform" _newtrack_0 :!class /Script/Engine.MaterialInstanceDynamic))
    (:Finished
      (switch Utilities|FlowControl|Switch|SwitchonETimelineDirection "Forward"
        (:Forward
          (CallFunction|OnFullyRevealed))
        (:Backward
          (CallFunction|OnFullyHidden))))))

(event EventOnFullyHidden
  ;[0.15 0.15 0.15 0.5] Gère la visibilité de l'objet
  (Variables|Default|SetIsRevealed? false))

(event EventOnFullyRevealed
  ;[0.15 0.15 0.15 0.5] Gère la visibilité de l'objet
  (Variables|Default|SetIsRevealed? true))

(fn ConstructionScript)