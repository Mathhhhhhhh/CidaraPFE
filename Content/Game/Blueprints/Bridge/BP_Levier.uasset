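; BP_Levier is an interactable lever that raises the BP_Bridge2 bridge, found in the level by class lookup.
; Interacting calls RaiseBridge once through a DoOnce, and focus toggles an outline overlay material on its cube.
; Its box also counts BP_PlayerCidara and BP_Spectre begin-overlaps, calling RaiseBridge when the running count hits three; the count never decreases.
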(event OnComponentBeginOverlap(Box)
  (params (OverlappedComponent :type Primitive%20Component%20Object%20Reference) (OtherActor :type Actor%20Object%20Reference) (OtherComp :type Primitive%20Component%20Object%20Reference) (OtherBodyIndex :type Integer) (bFromSweep :type Boolean) (SweepResult :type Hit%20Result%20Structure%20%28by%20ref%29))
  (Utilities|Casting|CastToBP_PlayerCidara OtherActor
    (:then
      (Development|PrintString "Player"))
    (:CastFailed
      (Utilities|Casting|CastToBP_Spectre OtherActor)
      (Development|PrintString "Spectre")))
  (bind _output_get (Variables|Default|SetNumberOnPlane (+ (Variables|Default|GetNumberOnPlane) 1)))
  (if (== _output_get 3)
    (bind _returnvalue (Actor|GetActorOfClass "/Game/Game/Blueprints/Bridge/BP_Bridge2.BP_Bridge2_C"))
    (Default|RaiseBridge _returnvalue)))

(event EventBeginPlay)

(event Collision|EventActorBeginOverlap
  (params (OtherActor :type Actor%20Object%20Reference)))

(event EventSetFocus
  (params (Focused :type Boolean) (Investigator :type Actor%20Object%20Reference))
  (if Focused
    (Rendering|Material|SetOverlayMaterial (Variables|Default|GetCube) "/Game/Game/Materials/VFX/MI_InteractableOutline.MI_InteractableOutline" :!class /Script/Engine.MeshComponent)
    (else
      (Rendering|Material|SetOverlayMaterial (Variables|Default|GetCube) 0 :!class /Script/Engine.MeshComponent))))

(event EventInterract
  (params (Investigator :type Actor%20Object%20Reference))
  (Utilities|FlowControl|DoOnce false
    (:Completed
      (bind _returnvalue (Actor|GetActorOfClass "/Game/Game/Blueprints/Bridge/BP_Bridge2.BP_Bridge2_C"))
      (Default|RaiseBridge _returnvalue))))

(fn ConstructionScript)