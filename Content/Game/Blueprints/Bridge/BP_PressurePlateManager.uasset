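; BP_PressurePlateManager tracks which actor stands on each plate of a two-plate puzzle and broadcasts solved or reset events.
; SetPlateState updates an index-to-actor map, then CheckActivation tests whether plates 0 and 1 hold different actors.
; The branch compares that result to IsActive: any mismatch sets it true and fires OnPuzzleSolved, even when occupancy is lost.
; A match sets it false and fires OnPuzzleReset.
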(event EventBeginPlay)

(event Collision|EventActorBeginOverlap
  (params (OtherActor :type Actor%20Object%20Reference)))

(event EventTick
  (params (DeltaSeconds :type Float%20%28single-precision%29)))

(fn ConstructionScript)

(fn SetPlateState
  (params (Index :type Integer) (Actor :type Actor%20Object%20Reference))
  (if (Utilities|IsValid Actor)
    (Utilities|Map|Add (Variables|Default|GetActorOnPlate) Index Actor)
    (else
      (Utilities|Map|Remove (Variables|Default|GetActorOnPlate) Index)))
  (CallFunction|CheckActivation)
  (Development|PrintString "Hello"))

(fn CheckActivation
  (bind _actoronplate (Variables|Default|GetActorOnPlate))
  (bind (_value _returnvalue) (Utilities|Map|Find _actoronplate 0))
  (bind (_value_2 _returnvalue_2) (Utilities|Map|Find _actoronplate 1))
  (bind _output_get (Variables|Default|SetbBothPresent (and _returnvalue _returnvalue_2)))
  (bind _output_get_2 (Variables|Default|SetbDifferent (!= _value _value_2)))
  (bind _output_get_3 (Variables|Default|SetbShouldBeActive (and _output_get_2 _output_get)))
  (if (!= _output_get_3 (Variables|Default|GetIsActive))
    (Variables|Default|SetIsActive true)
    (Default|CallOnPuzzleSolved)
    (Development|PrintString "OUI")
    (else
      (Variables|Default|SetIsActive false)
      (Default|CallOnPuzzleReset)
      (Development|PrintString "NON"))))