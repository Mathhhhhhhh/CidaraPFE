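; BP_Platforme is a moving platform that travels between its starting location and that point offset by DirectionVitesse.
; On BeginPlay it computes both endpoints, then a Timeline's Mouvement track drives a swept location lerp between them.
; A BoxInterraction overlap checks the other actor for BPI_PlatformeInteraction but does nothing yet, a placeholder for reactions to entering the platform.
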(event OnComponentBeginOverlap(BoxInterraction)
  (params (OverlappedComponent :type Primitive%20Component%20Object%20Reference) (OtherActor :type Actor%20Object%20Reference) (OtherComp :type Primitive%20Component%20Object%20Reference) (OtherBodyIndex :type Integer) (bFromSweep :type Boolean) (SweepResult :type Hit%20Result%20Structure%20%28by%20ref%29))
  ;[0.15 0.15 0.15 0.5] Si jamais on veut faire en sorte qu'il se passe quelque chose quand on rentre sur la plateform
  (if (Utilities|DoesObjectImplementInterface OtherActor "/Game/Game/Blueprints/Environnement/BPI_PlatformeInteraction.BPI_PlatformeInteraction_C")
    _))

(event EventBeginPlay
  (bind _output_get (Variables|Default|SetStart%20Location (Transformation|GetActorLocation)))
  (Variables|Default|SetEnd%20Location (+ _output_get (Variables|Default|GetDirection%20+%20Vitesse)))
  (bind _mouvement (Timeline|Timeline Play)
    (:Update
      (Transformation|SetActorLocation (Math|Vector|Lerp(Vector) (Variables|Default|GetStart%20Location) (Variables|Default|GetEnd%20Location) _mouvement) true false))))

(fn ConstructionScript)