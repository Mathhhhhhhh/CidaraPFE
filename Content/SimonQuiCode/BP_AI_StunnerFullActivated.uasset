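; Stunner hazard whose electrified spheres kill Cidara and burn the Spectre.
; BeginPlay sizes spheres from SphereScale and, after a delay, plays a randomly timed pulse scaling SphereSpectre and Sphere1 with sound.
; Spheredetect overlap zaps Cidara with Niagara and death, while SphereSpectre burns the Spectre; Deactivate shrinks spheres, optionally sparing the Spectre pair.
; Movement-based Tick detection and AI chase are inactive leftovers.
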(event OnComponentBeginOverlap(CAC)
  (params (OverlappedComponent :type Primitive%20Component%20Object%20Reference) (OtherActor :type Actor%20Object%20Reference) (OtherComp :type Primitive%20Component%20Object%20Reference) (OtherBodyIndex :type Integer) (bFromSweep :type Boolean) (SweepResult :type Hit%20Result%20Structure%20%28by%20ref%29))
  ;[0.15 0.15 0.15 0.5] Si L'IA touche Cidara ou Spectre, il/elle meurt
  (Utilities|FlowControl|Sequence
    (:then_0
      (if (== OtherActor (Variables|Default|GetBP_PlayerRef))
        _))
    (:then_1
      (if (== OtherActor (Variables|Default|GetBP_SpectreRef))
        _))))

(event OnComponentBeginOverlap(SphereSpectre)
  (params (OverlappedComponent :type Primitive%20Component%20Object%20Reference) (OtherActor :type Actor%20Object%20Reference) (OtherComp :type Primitive%20Component%20Object%20Reference) (OtherBodyIndex :type Integer) (bFromSweep :type Boolean) (SweepResult :type Hit%20Result%20Structure%20%28by%20ref%29))
  (bind _asbp_spectre (Utilities|Casting|CastToBP_Spectre OtherActor))
  (Default|SpectreBurning _asbp_spectre))

(event OnComponentEndOverlap(Spheredetect)
  (params (OverlappedComponent :type Primitive%20Component%20Object%20Reference) (OtherActor :type Actor%20Object%20Reference) (OtherComp :type Primitive%20Component%20Object%20Reference) (OtherBodyIndex :type Integer))
  (bind _bp_spectreref (Variables|Default|GetBP_SpectreRef))
  (bind _bp_playerref (Variables|Default|GetBP_PlayerRef))
  ;[0.15 0.15 0.15 0.5] End overlap, vérifie que c'est bien le joueur ou spectre, si oui stock l'info "inside = false"
  (Utilities|FlowControl|Sequence
    (:then_0
      (if (== OtherActor _bp_playerref)
        (if (!= (Utilities|GetClass _bp_playerref) (Utilities|GetClass self))
          (Variables|Default|SetInside false)
          (Actor|Tick|SetActorTickEnabled false :!label _label))))
    (:then_1
      (if (== OtherActor _bp_spectreref)
        (if (!= (Utilities|GetClass _bp_spectreref) (Utilities|GetClass self))
          (Variables|Default|SetSpectreInside false)
          (goto _label))))))

(event OnComponentBeginOverlap(Spheredetect)
  (params (OverlappedComponent :type Primitive%20Component%20Object%20Reference) (OtherActor :type Actor%20Object%20Reference) (OtherComp :type Primitive%20Component%20Object%20Reference) (OtherBodyIndex :type Integer) (bFromSweep :type Boolean) (SweepResult :type Hit%20Result%20Structure%20%28by%20ref%29))
  (bind _bp_playerref (Variables|Default|GetBP_PlayerRef))
  ;[0.15 0.15 0.15 0.5] Si qlq chose est overlap, vérifie que c'est bien cidara ou spectre, stock l'info "inside = true"et pareil pour "spectre inside"
  (Development|PrintString (Utilities|GetDisplayName OtherActor))
  (Utilities|FlowControl|Sequence
    (:then_0
      (if (== _bp_playerref OtherActor)
        (CallFunction|TriggerElectrocution _bp_playerref)
        (Development|PrintString "Cidara")))))

(event Custom|TriggerElectrocution
  (params (Target :type Pawn%20Object%20Reference))
  (if (Utilities|IsValid Target)
    (Niagara|SpawnSystemAttached "/Game/Vefects/Zap_VFX/VFX/Zap/Particles/NS_Zap_02_Blue.NS_Zap_02_Blue" (Variables|/Script/Engine.Actor|GetRootComponent Target) "None" "0.000000,0.000000,-85.000000" "0, 0, 0" "KeepRelativeOffset" false)
    (bind _asbp_player_cidara (Utilities|Casting|CastToBP_PlayerCidara Target)
      (:then
        (Default|Death _asbp_player_cidara))
      (:CastFailed
        (bind _asbp_spectre (Utilities|Casting|CastToBP_Spectre Target))
        (Default|SpectreBurning _asbp_spectre)))))

(event Custom|Deactivate
  (bind _spheredetect (Variables|Default|GetSpheredetect))
  (bind _sphere (Variables|Default|GetSphere))
  (bind _sphere1 (Variables|Default|GetSphere1))
  (bind _spherespectre (Variables|Default|GetSphereSpectre))
  (bind _spheredetect_2 (Variables|Default|GetSpheredetect))
  (bind _sphere_2 (Variables|Default|GetSphere))
  (bind _alpha (Timeline|Destroy Play)
    (:Update
      (if (Variables|Default|GetKeepSpectreUp)
        (Transformation|SetWorldScale3D _spheredetect (Math|Vector|Lerp(Vector) (Transformation|GetWorldScale _spheredetect) "0, 0, 0" _alpha))
        (Transformation|SetWorldScale3D _sphere (Math|Vector|Lerp(Vector) (Transformation|GetWorldScale _sphere) "0, 0, 0" _alpha))
        (else
          (Transformation|SetWorldScale3D _sphere1 (Math|Vector|Lerp(Vector) (Transformation|GetWorldScale _sphere1) "0, 0, 0" _alpha))
          (Transformation|SetWorldScale3D _spherespectre (Math|Vector|Lerp(Vector) (Transformation|GetWorldScale _spherespectre) "0, 0, 0" _alpha))
          (Transformation|SetWorldScale3D _spheredetect_2 (Math|Vector|Lerp(Vector) (Transformation|GetWorldScale _spheredetect_2) "0, 0, 0" _alpha))
          (Transformation|SetWorldScale3D _sphere_2 (Math|Vector|Lerp(Vector) (Transformation|GetWorldScale _sphere_2) "0, 0, 0" _alpha)))))))

(event EventTick
  (params (DeltaSeconds :type Float%20%28single-precision%29))
  (bind _bp_spectreref (Variables|Default|GetBP_SpectreRef))
  (bind _bp_playerref (Variables|Default|GetBP_PlayerRef))
  ;[0.15 0.15 0.15 0.5] Vérifie "le joueur ou spectre sont ils dans le champ de détection ?" puis "est-il en mouvement ?" si oui l'ia fonce sur le joueur.
  (Utilities|FlowControl|Sequence
    (:then_0
      (if (Variables|Default|GetInside)
        (if (> (Math|Vector|VectorLength (Transformation|GetVelocity _bp_playerref)) 1.0)
          (CallFunction|TriggerElectrocution _bp_playerref))))
    (:then_1
      (if (Variables|Default|GetSpectreInside)
        (if (> (Math|Vector|VectorLength (Transformation|GetVelocity _bp_spectreref)) 1.0)
          (CallFunction|TriggerElectrocution _bp_spectreref))))))

(event EventBeginPlay
  (bind _spherescale (Variables|Default|GetSphereScale))
  (bind _spherespectre (Variables|Default|GetSphereSpectre))
  (bind _sphere1 (Variables|Default|GetSphere1))
  ;[0.15 0.15 0.15 0.5] 2 cast, stock la loc puis timelinbe de pulse
  (Utilities|FlowControl|Sequence
    (:then_0
      (bind _returnvalue (Actor|GetActorOfClass "/Game/Game/Blueprints/Characters/Cidara/BP_PlayerCidara.BP_PlayerCidara_C"))
      (Variables|Default|SetBP_PlayerRef _returnvalue))
    (:then_1
      (bind _returnvalue_2 (Actor|GetActorOfClass "/Game/Game/Blueprints/Characters/Spectre/BP_Spectre.BP_Spectre_C"))
      (Variables|Default|SetBP_SpectreRef _returnvalue_2))
    (:then_2
      (Variables|Default|Setloc (Transformation|GetActorLocation)))
    (:then_3
      (Transformation|SetWorldScale3D (Variables|Default|GetSpheredetect) (Math|Conversions|ToVector(Float) (* _spherescale 2.0)))
      (Transformation|SetWorldScale3D (Variables|Default|GetSphere) (Math|Conversions|ToVector(Float) (* _spherescale 1.25)))
      (Components|Timeline|SetPlaybackPosition (Variables|Default|GetTL_Pulse) 0.0 false true)
      (Rendering|Material|SetVectorParameterValue (Variables|Default|GetMat) "Color" "(R=1.000000,G=0.286316,B=0.065224,A=1.000000)" :!class /Script/Engine.MaterialInstanceDynamic)
      (Utilities|FlowControl|Delay (Variables|Default|GetStartPulseTime))
      (bind _scale (Timeline|TL_Pulse PlayFromStart)
        (:Update
          (if (Utilities|IsValid _spherespectre)
            (Transformation|SetWorldScale3D _spherespectre (Math|Conversions|ToVector(Float) (Math|Float|Lerp 0.0 (* (Variables|Default|GetSphereScale) 2.0) _scale)))
            (if (Utilities|IsValid _sphere1)
              (Transformation|SetWorldScale3D _sphere1 (Math|Conversions|ToVector(Float) (Math|Float|Lerp 0.0 (* (Variables|Default|GetSphereScale) 1.25) _scale))))))
        (:Sfx
          (Audio|PlaySoundatLocation "/Game/SimonQuiCode/golemSFX2.golemSFX2" (Transformation|GetActorLocation self) "0, 0, 0" 1.0 1.0 0.0 "/Game/SimonQuiCode/FinalGolem/SFX/Footstep/SA_Sphere.SA_Sphere" 0 0 0))))
    (:then_4
      (Actor|Tick|SetActorTickEnabled false))
    (:then_5
      (bind _returnvalue_3 (Rendering|Material|CreateDynamicMaterialInstance (Variables|Default|GetSphere) 0 0 "None" :!class /Script/Engine.PrimitiveComponent))
      (Variables|Default|SetMat _returnvalue_3))))

(fn ConstructionScript)