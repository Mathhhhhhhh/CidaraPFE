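; Patrolling enemy AI that moves along a spline and hunts BP_PlayerCidara on sight.
; Tick drives the spline patrol and rotations, while a LineOfSight component builds a rotating line-trace vision mesh whose overlaps start AI MoveTo pursuit.
; On losing sight it keeps following briefly, spins in place, then returns to its saved spline distance and eases back into alignment.
; Touching the player through CAC only prints a death message.
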(event OnComponentBeginOverlap(CAC)
  (params (OverlappedComponent :type Primitive%20Component%20Object%20Reference) (OtherActor :type Actor%20Object%20Reference) (OtherComp :type Primitive%20Component%20Object%20Reference) (OtherBodyIndex :type Integer) (bFromSweep :type Boolean) (SweepResult :type Hit%20Result%20Structure%20%28by%20ref%29))
  ;[0.15 0.15 0.15 0.5] Si L'IA touche le joueur, il meurt
  (if (== OtherActor (Variables|Default|GetBP_PlayerRef))
    (Development|PrintString "T'ES MORT")))

(event BeginOverlap(LineOfSight)
  (params (Hit :type Hit%20Result%20Structure%20%28by%20ref%29))
  (bind _bp_playerref (Variables|Default|GetBP_PlayerRef))
  ;[0.15 0.06327 0.01594 0.5] Quand le Player rentre dans le LOS, L'iA le voit, puis le follow
  (if (== (.HitActor (Collision|BreakHitResult Hit)) _bp_playerref)
    ;;[0.15 0.04146 0.1495 0.5] On garde*
    (Variables|Default|SetInVision true)
    (Variables|Default|SetIsRotating false)
    (if (!= (Utilities|GetClass _bp_playerref) (Utilities|GetClass self))
      (Development|PrintString "je te vois")
      (Variables|Default|SetFollowingPlayer true)
      (AI|AIMoveTo self "0, 0, 0" _bp_playerref 5.0 false))))

(event EndOverlap(LineOfSight)
  (params (Hit :type Hit%20Result%20Structure%20%28by%20ref%29))
  (bind _spline (Variables|Default|GetSpline))
  (bind _distancealongspline (Variables|Default|GetDistanceAlongSpline))
  (bind _returnvalue (Spline|GetTransformatDistanceAlongSpline _spline _distancealongspline "Local" false))
  ;[0.15 0.15 0.15 0.5] SI L'IA perd de vue le player
  (if (== (.HitActor (Collision|BreakHitResult Hit)) (Variables|Default|GetBP_PlayerRef))
    ;[0.15 0.15 0.15 0.5] Elle le suit encore 3 secondes
    (Variables|Default|SetInVision false)
    (Development|PrintString "je suis censé te suivre")
    (Variables|Default|SetLaJsuisVif true)
    (AI|AIMoveTo self "0, 0, 0" (Variables|Default|GetBP_PlayerRef) 5.0 false
      (:then
        (Utilities|FlowControl|RetriggerableDelay 3.0)
        ;[0.15 0.15 0.15 0.5] Si elle l'a pas retrouvé, l'IA Fais un tour sur elle même
        (Variables|Default|SetLaJsuisVif false)
        (if (not (Variables|Default|GetInVision))
          (Development|PrintString "Je vais spin frero")
          (AI|Navigation|StopMovement (AI|GetAIController self))
          (Variables|Default|SetIsRotating true)
          (Utilities|FlowControl|RetriggerableDelay 5.0)
          ;[0.15 0.15 0.15 0.5] Puis elle retourne à son spline initial
          (Variables|Default|SetIsRotating false)
          (Development|PrintString "je vois plus")
          (AI|AIMoveTo self (Math|Vector|MakeVector (.x (.location _returnvalue)) (.y (.location _returnvalue)) (+ (.z (.location _returnvalue)) 9e+01)) 0 5.0 false
            (:OnSuccess
              (Variables|Default|SetFollowingPlayer false)
              (Variables|Default|SetImBack true)
              (Development|PrintString "de retour"))))))))

(event EventBeginPlay
  (bind _lineofsight (Variables|Default|GetLineOfSight))
  ;[0.15 0.15 0.15 0.5] Le Line Of Sight Apparait et tourne
  (Utilities|FlowControl|Sequence
    (:then_0
      (bind _asbp_player_cidara (Utilities|Casting|CastToBP_PlayerCidara (Game|Player|GetPlayerPawn 0)))
      (Variables|Default|SetBP_PlayerRef _asbp_player_cidara))
    (:then_1
      (Class|LineOfSightComponent|StartLineTrace _lineofsight "TraceTypeQuery4" 60)
      (Class|LineOfSightComponent|StartBuildMesh _lineofsight)
      (Class|LineOfSightComponent|StartRotateinRangeAxis _lineofsight "X" 9e+01 1e+01 "Relative_Rotation" false))))

(event Collision|EventActorBeginOverlap
  (params (OtherActor :type Actor%20Object%20Reference)))

(event EventTick
  (params (DeltaSeconds :type Float%20%28single-precision%29))
  (bind _self self)
  ;[0.15 0.007812 0.007812 0.5] Parametres de rotations
  ;[0.04591 0.15 0.02398 0.5] L'IA se déplace sur le Spline
  (if (Variables|Default|GetLaJsuisVif)
    (Transformation|SetActorRelativeRotation _self (Math|Interpolation|RInterpTo (Transformation|GetActorRotation self) (Math|Rotator|FindLookatRotation (Transformation|GetActorLocation _self) (Transformation|GetActorLocation)) (Utilities|Time|GetWorldDeltaSeconds) 2.0))
    (elif (Variables|Default|GetIsRotating)
      (Transformation|AddActorLocalRotation self (Variables|Default|GetDelta%20Rotation) false false)
      (elif (not (Variables|Default|GetFollowingPlayer))
        (if (Variables|Default|GetImBack)
          (Development|PrintString "je me met bien")
          ;;[0.15 0.15 0.15 0.5] Quand elle revient dans le spline, l'ia se remet droite sans tp
          (Transformation|SetActorRotation (Math|Interpolation|RInterpTo (Transformation|GetActorRotation) (Spline|GetRotationatDistanceAlongSpline (Variables|Default|GetSpline) (Variables|Default|GetDistanceAlongSpline) "Local") (Utilities|Time|GetWorldDeltaSeconds) 1.0))
          (Utilities|FlowControl|Delay 1.0)
          (Variables|Default|SetImBack false)
          (else
            (Variables|Default|SetDistanceAlongSpline (+ (* DeltaSeconds (Variables|Default|GetSplineSpeed)) (Variables|Default|GetDistanceAlongSpline)))
            (Transformation|SetActorTransform (Math|Transform|MakeTransform (Math|Vector|MakeVector (.x (.location (Spline|GetTransformatDistanceAlongSpline (Variables|Default|GetSpline) (Variables|Default|GetDistanceAlongSpline) "Local" false))) (.y (.location (Spline|GetTransformatDistanceAlongSpline (Variables|Default|GetSpline) (Variables|Default|GetDistanceAlongSpline) "Local" false))) (+ (.z (.location (Spline|GetTransformatDistanceAlongSpline (Variables|Default|GetSpline) (Variables|Default|GetDistanceAlongSpline) "Local" false))) 9e+01)) (Math|Rotator|MakeRotator (.roll (.rotation (Spline|GetTransformatDistanceAlongSpline (Variables|Default|GetSpline) (Variables|Default|GetDistanceAlongSpline) "Local" false))) (.pitch (.rotation (Spline|GetTransformatDistanceAlongSpline (Variables|Default|GetSpline) (Variables|Default|GetDistanceAlongSpline) "Local" false))) (+ (.yaw (.rotation (Spline|GetTransformatDistanceAlongSpline (Variables|Default|GetSpline) (Variables|Default|GetDistanceAlongSpline) "Local" false))) 0.0))))
            (if (Variables|Default|Getloop?)
              (if (> (Variables|Default|GetDistanceAlongSpline) (Spline|GetSplineLength (Variables|Default|GetSpline)))
                (Variables|Default|SetDistanceAlongSpline 0.0)))))))))

(fn ConstructionScript)