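; Golem guard enemy AI that patrols tagged waypoints, chases Cidara or the Spectre, and investigates ball noises.
; AI Perception drives chase speed, music and self-rescheduling growl or angry sounds; lost targets send it through LookAround back to patrol.
; Ball stimuli are line-traced down and projected onto the navmesh.
; The CAC overlap triggers a stomp with a briefly enabled AttackZone, which flags Cidara as dead and ignored when hit.
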(event OnTargetPerceptionUpdated(AIPerception)
  (params (Actor :type Actor%20Object%20Reference) (Stimulus :type AI%20Stimulus%20Structure))
  ;[0.15 0.15 0.15 0.5] Qui j'entends / Qui je vois ? Est ce que faut que je le suive ?
  (if (not (== (.tag Stimulus) "ball"))
    (if (or (== Actor (Variables|Default|GetCidRef)) (== Actor (Variables|Default|GetSpectreRef)))
      (if (not (== Actor (Variables|Default|GetBlockedTarget)))
        (if (not (Utilities|IsValid (Variables|Default|GetCurrentTarget)))
          (Variables|Default|SetCurrentTarget Actor))
        (Variables|Default|SetIsChasing true)
        (Utilities|Time|ClearandInvalidateTimerbyHandle (Variables|Default|GetGrowlTimerHandle))
        (if (Variables|Default|GetSoundIsOn)
          _
          (else
            (Variables|Default|SetSoundIsOn true)
            (Audio|Components|Audio|FadeIn (Variables|Default|GetMusicAudio) 3.0 1.0 0.0 "Linear" :!class /Script/Engine.AudioComponent)
            (CallFunction|PlayAngry)))
        (Variables|/Script/Engine.CharacterMovementComponent|SetMaxWalkSpeed (Variables|Character|GetCharacterMovement) 4.5e+02)
        (if (.bsuccessfullysensed Stimulus)
          (AI|AIMoveTo self (Transformation|GetActorLocation (Variables|Default|GetCurrentTarget)) (Variables|Default|GetCurrentTarget) 5.0 false
            (:OnSuccess
              ;[0.15 0.15 0.15 0.5] C'est mon heure de patrouille michel
              (bind _outactors (Actor|GetAllActorswithTag (Variables|Default|GetTag)))
              (AI|AIMoveTo self (Transformation|GetActorLocation (Utilities|Array|Get(acopy) _outactors (Variables|Default|GetARRAYInt))) (Utilities|Array|Get(acopy) _outactors (Variables|Default|GetARRAYInt)) 5.0 false
                (:OnSuccess
                  (Variables|Default|SetARRAYInt (Math|Integer|%(Integer) (+ (Variables|Default|GetARRAYInt) 1) (Utilities|Array|Length _outactors)))
                  (CallFunction|LookAround)))))
          (else
            (Variables|Default|SetLastKnownLocation (Transformation|GetActorLocation (Variables|Default|GetCurrentTarget)))
            (AI|AIMoveTo self (Variables|Default|GetLastKnownLocation) 0 5.0 false
              (:OnSuccess
                (CallFunction|LookAround)))))))
    (elif (.bsuccessfullysensed Stimulus)
      (if (not (Utilities|IsValid (Variables|Default|GetCurrentTarget)))
        (Variables|Default|SetSoundActorSource Actor)
        (bind (_outhit _returnvalue) (Collision|LineTraceByChannel (+ (.stimuluslocation Stimulus) "0.000000,0.000000,100.000000") (- (.stimuluslocation Stimulus) "0.000000,0.000000,1000.000000") "TraceTypeQuery1" false 0 "None"))
        (if _returnvalue
          (if (.ReturnValue (AI|Navigation|ProjectPointtoNavigation (.ImpactPoint (Collision|BreakHitResult _outhit)) 0 0 "150.000000,150.000000,1000.000000"))
            (AI|AIMoveTo self (.ProjectedLocation (AI|Navigation|ProjectPointtoNavigation (.ImpactPoint (Collision|BreakHitResult _outhit)) 0 0 "150.000000,150.000000,1000.000000")) 0 5.0 false
              (:OnSuccess
                (Variables|Default|SetOrigineSonAtteint true)
                (CallFunction|LookAround)))))))))

(event OnTargetPerceptionForgotten(AIPerception)
  (params (Actor :type Actor%20Object%20Reference))
  ;[0.15 0.15 0.15 0.5] Qui j'oublie ?
  (if (== Actor (Variables|Default|GetCurrentTarget))
    (Variables|Default|SetCurrentTarget 0)
    (CallFunction|LookAround :!label _label)
    (elif (== Actor (Variables|Default|GetSoundActorSource))
      (if (not (Utilities|IsValid (Variables|Default|GetCurrentTarget)))
        (if (not (Variables|Default|GetOrigineSonAtteint))
          (goto _label))))))

(event OnComponentBeginOverlap(CAC)
  (params (OverlappedComponent :type Primitive%20Component%20Object%20Reference) (OtherActor :type Actor%20Object%20Reference) (OtherComp :type Primitive%20Component%20Object%20Reference) (OtherBodyIndex :type Integer) (bFromSweep :type Boolean) (SweepResult :type Hit%20Result%20Structure%20%28by%20ref%29))
  (bind _attackzone (Variables|Default|GetAttackZone))
  ;[0.15 0.15 0.15 0.5] Je tape + si c'est un cadavre bah je l'oublie
  (Utilities|FlowControl|Sequence
    (:then_0
      (if (== OtherActor (Variables|Default|GetCidRef))
        (AI|Navigation|StopMovement (AI|GetAIController self) :!label _label)
        (Transformation|SetActorRotation self (Math|Rotator|MakeRotator 0.0 0.0 (.yaw (Math|Rotator|FindLookatRotation (Transformation|GetActorLocation self) (Transformation|GetActorLocation (Variables|Default|GetCurrentTarget))))))
        (Animation|PlayAnimMontage "/Game/SimonQuiCode/FinalGolem/Anim/Stomp_Montage.Stomp_Montage" 1.0 "None")
        (Utilities|FlowControl|Delay 1.3)
        (Collision|SetCollisionEnabled _attackzone "QueryAndPhysics")
        (Rendering|SetVisibility _attackzone true false)
        (Utilities|FlowControl|Delay 0.2)
        (Collision|SetCollisionEnabled _attackzone "NoCollision")
        (Utilities|FlowControl|Delay 0.7)
        (if (Variables|Default|GetCidaraVivant?)
          (AI|AIMoveTo self "0, 0, 0" (Variables|Default|GetCurrentTarget) -1.0 false
            (:OnSuccess
              (CallFunction|LookAround)))
          (else
            (CallFunction|LookAround)))))
    (:then_1
      (if (== OtherActor (Variables|Default|GetSpectreRef))
        (goto _label)))))

(event OnComponentBeginOverlap(AttackZone)
  (params (OverlappedComponent :type Primitive%20Component%20Object%20Reference) (OtherActor :type Actor%20Object%20Reference) (OtherComp :type Primitive%20Component%20Object%20Reference) (OtherBodyIndex :type Integer) (bFromSweep :type Boolean) (SweepResult :type Hit%20Result%20Structure%20%28by%20ref%29))
  (if (== OtherActor (Variables|Default|GetCidRef))
    (Variables|Default|SetBlockedTarget OtherActor)
    (Variables|Default|SetCurrentTarget 0)
    (Variables|Default|SetCidaraVivant? false)))

(event Custom|OnTargetPerceptionForgotten_Event
  (params (Actor :type Actor%20Object%20Reference))
  ;[0.15 0.15 0.15 0.5] Clicking
)

(event Custom|LookAround
  (bind _musicaudio (Variables|Default|GetMusicAudio))
  (Variables|Default|SetSoundIsOn false)
  ;[0.15 0.15 0.15 0.5] je Look around
  (Variables|Default|SetIsChasing false)
  (Utilities|Time|ClearandInvalidateTimerbyHandle (Variables|Default|GetAngryTimerHandle))
  (Audio|Components|Audio|FadeOut _musicaudio 2.0 0.0 "Linear" :!class /Script/Engine.AudioComponent)
  (Utilities|FlowControl|Delay 2.0)
  (Audio|Components|Audio|Stop _musicaudio)
  (CallFunction|PlayGrowl)
  (Variables|Default|SetCurrentTarget 0)
  (AI|Navigation|StopMovement (AI|GetAIController self))
  (Utilities|FlowControl|Delay 0.2)
  (Variables|/Script/Engine.CharacterMovementComponent|SetMaxWalkSpeed (Variables|Character|GetCharacterMovement) 1.5e+02)
  ;[0.15 0.15 0.15 0.5] C'est mon heure de patrouille michel
  (bind _outactors (Actor|GetAllActorswithTag (Variables|Default|GetTag)))
  (AI|AIMoveTo self (Transformation|GetActorLocation (Utilities|Array|Get(acopy) _outactors (Variables|Default|GetARRAYInt))) (Utilities|Array|Get(acopy) _outactors (Variables|Default|GetARRAYInt)) 5.0 false
    (:OnSuccess
      (Variables|Default|SetARRAYInt (Math|Integer|%(Integer) (+ (Variables|Default|GetARRAYInt) 1) (Utilities|Array|Length _outactors)))
      (CallFunction|LookAround))))

(event Custom|PlayGrowl
  (if (not (Variables|Default|GetIsChasing))
    (Audio|PlaySoundatLocation "/Game/SimonQuiCode/FinalGolem/SFX/SC_Golem_Growl.SC_Golem_Growl" (Transformation|GetActorLocation) "0, 0, 0" 1.0 1.0 0.0 0 0 0 0)
    (bind _returnvalue (Utilities|Time|SetTimerbyEvent (delegate Custom|PlayGrowl) (Math|Random|RandomFloatinRange 5.0 15.0)))
    (Variables|Default|SetGrowlTimerHandle _returnvalue)))

(event Custom|PlayAngry
  (if (Variables|Default|GetIsChasing)
    (Audio|PlaySoundatLocation "/Game/SimonQuiCode/FinalGolem/SFX/SC_Golem_Angry.SC_Golem_Angry" (Transformation|GetActorLocation) "0, 0, 0" 1.0 1.0 0.0 0 0 0 0)
    (bind _returnvalue (Utilities|Time|SetTimerbyEvent (delegate Custom|PlayAngry) (Math|Random|RandomFloatinRange 4.0 1e+01)))
    (Variables|Default|SetAngryTimerHandle _returnvalue)))

(event EventBeginPlay
  (Actor|Tick|SetActorTickEnabled false)
  (Utilities|FlowControl|Sequence
    (:then_0
      ;[0.15 0.15 0.15 0.5] Clicking
      (EventDispatchers|AssignOnTargetPerceptionForgotten (Variables|Default|GetAIPerception) (delegate Custom|OnTargetPerceptionForgotten_Event))
      ;[0.15 0.15 0.15 0.5] C'est mon heure de patrouille michel
      (bind _outactors (Actor|GetAllActorswithTag (Variables|Default|GetTag)))
      (AI|AIMoveTo self (Transformation|GetActorLocation (Utilities|Array|Get(acopy) _outactors (Variables|Default|GetARRAYInt))) (Utilities|Array|Get(acopy) _outactors (Variables|Default|GetARRAYInt)) 5.0 false
        (:OnSuccess
          (Variables|Default|SetARRAYInt (Math|Integer|%(Integer) (+ (Variables|Default|GetARRAYInt) 1) (Utilities|Array|Length _outactors)))
          (CallFunction|LookAround))))
    (:then_1
      ;[0.15 0.15 0.15 0.5] Cast Cidara & Spectre
      (bind _returnvalue (Actor|GetActorOfClass "/Game/Game/Blueprints/Characters/Cidara/BP_PlayerCidara.BP_PlayerCidara_C"))
      (Variables|Default|SetCidRef _returnvalue)
      (Utilities|FlowControl|Delay 0.2)
      (bind _returnvalue_2 (Actor|GetActorOfClass "/Game/Game/Blueprints/Characters/Spectre/BP_Spectre.BP_Spectre_C"))
      (Variables|Default|SetSpectreRef _returnvalue_2)
      (CallFunction|PlayGrowl))))

(fn ConstructionScript)