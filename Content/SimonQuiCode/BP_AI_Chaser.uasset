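; AI chaser enemy that patrols a spline and hunts the player (Cidara) or the Spectre.
; Tick moves it along the spline, while a rotating LineOfSight trace mesh triggers AIMoveTo pursuit of the first target spotted.
; Losing sight starts a retriggerable delay, then a spin in place if the player stays unseen.
; It then returns to its saved spline distance, as it does after CAC overlap flags a target dead.
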(event OnComponentBeginOverlap(CAC)
  (params (OverlappedComponent :type Primitive%20Component%20Object%20Reference) (OtherActor :type Actor%20Object%20Reference) (OtherComp :type Primitive%20Component%20Object%20Reference) (OtherBodyIndex :type Integer) (bFromSweep :type Boolean) (SweepResult :type Hit%20Result%20Structure%20%28by%20ref%29))
  ;[0.15 0.15 0.15 0.5] Si L'IA touche le joueur, il meurt
  (Utilities|FlowControl|Sequence
    (:then_0
      (if (== OtherActor (Variables|Default|GetBP_PlayerRef))
        (Variables|Default|SetCidaraVivant false)
        (CallFunction|Retour :!label _label)))
    (:then_1
      (if (== OtherActor (Variables|Default|GetBP_SpectreRef))
        (Variables|Default|Setspectrevivant false)
        (goto _label)))))

(event BeginOverlap(LineOfSight)
  (params (Hit :type Hit%20Result%20Structure%20%28by%20ref%29))
  (bind _hitactor (Collision|BreakHitResult Hit))
  ;[0.15 0.06327 0.01594 0.5] Quand le Player rentre dans le LOS, L'iA le voit, puis le follow
  (Utilities|FlowControl|Sequence
    (:then_0
      (if (== _hitactor (Variables|Default|GetBP_PlayerRef))
        (if (Variables|Default|GetCidaraVivant)
          (Variables|Default|SetInVision true)
          (Variables|Default|SetFollowingCidara true)
          (if (not (Variables|Default|GetFollowingSpectre))
            (CallFunction|FollowCIdara)
            (Variables|Default|SetIsRotating false :!label _label)
            (Variables|Default|SetOnTrack? false)))))
    (:then_1
      (if (== _hitactor (Variables|Default|GetBP_SpectreRef))
        (if (Variables|Default|Getspectrevivant)
          (Variables|Default|SetSpetreInvision true)
          (Variables|Default|SetFollowingSpectre true)
          (if (not (Variables|Default|GetFollowingCidara))
            (CallFunction|FollowSpectre)
            (goto _label)))))))

(event EndOverlap(LineOfSight)
  (params (Hit :type Hit%20Result%20Structure%20%28by%20ref%29))
  (bind _hitactor (Collision|BreakHitResult Hit))
  ;[0.15 0.15 0.15 0.5] SI L'IA perd de vue le player
  (Utilities|FlowControl|Sequence
    (:then_0
      (if (== _hitactor (Variables|Default|GetBP_PlayerRef))
        (Variables|Default|SetInVision false)
        (Utilities|FlowControl|RetriggerableDelay 5.0 :!label _label)
        ;[0.15 0.15 0.15 0.5] Si elle l'a pas retrouvé, l'IA Fais un tour sur elle même
        (if (not (Variables|Default|GetInVision))
          (AI|Navigation|StopMovement (AI|GetAIController self))
          (Variables|Default|SetIsRotating true)
          ;[0.15 0.15 0.15 0.5] décidement, je vois plus degun
          (Utilities|FlowControl|RetriggerableDelay 5.0)
          (Variables|Default|SetIsRotating false)
          (CallFunction|Retour))))
    (:then_1
      (if (== _hitactor (Variables|Default|GetBP_SpectreRef))
        (Variables|Default|SetSpetreInvision false)
        (goto _label)))))

(event Custom|Retour
  (bind _spline (Variables|Default|GetSpline))
  (bind _distancealongspline (Variables|Default|GetDistanceAlongSpline))
  (bind _returnvalue (Spline|GetTransformatDistanceAlongSpline _spline _distancealongspline "Local" false))
  ;[0.15 0.15 0.15 0.5] retour
  (Variables|Default|SetFollowingSpectre false)
  (Variables|Default|SetFollowingCidara false)
  (AI|AIMoveTo self (Math|Vector|MakeVector (.x (.location _returnvalue)) (.y (.location _returnvalue)) (+ (.z (.location _returnvalue)) 9e+01)) 0 5.0 false
    (:OnSuccess
      (Variables|Default|SetOnTrack? true)
      (Variables|Default|SetImBack true))))

(event Custom|Follow%20CIdara
  (AI|AIMoveTo self "0, 0, 0" (Variables|Default|GetBP_PlayerRef) 5.0 false))

(event Custom|Follow%20Spectre
  (AI|AIMoveTo self "0, 0, 0" (Variables|Default|GetBP_SpectreRef) 5.0 false))

(event EventBeginPlay
  (bind _lineofsight (Variables|Default|GetLineOfSight))
  ;[0.15 0.15 0.15 0.5] Le Line Of Sight Apparait et tourne
  (Utilities|FlowControl|Sequence
    (:then_0
      (bind _asbp_player_cidara (Utilities|Casting|CastToBP_PlayerCidara (Game|Player|GetPlayerPawn 0)))
      (Variables|Default|SetBP_PlayerRef _asbp_player_cidara))
    (:then_1
      (Class|LineOfSightComponent|StartLineTrace _lineofsight "TraceTypeQuery4" 60)
      (Class|LineOfSightComponent|StartBuildMesh _lineofsight)
      (Class|LineOfSightComponent|StartRotateinRangeAxis _lineofsight "X" 9e+01 1e+01 "Relative_Rotation" false))
    (:then_2
      (bind _returnvalue (Actor|GetActorOfClass "/Game/Game/Blueprints/Characters/Spectre/BP_Spectre.BP_Spectre_C"))
      (Variables|Default|SetBP_SpectreRef _returnvalue))))

(event Collision|EventActorBeginOverlap
  (params (OtherActor :type Actor%20Object%20Reference)))

(event EventTick
  (params (DeltaSeconds :type Float%20%28single-precision%29))
  ;[0.15 0.007812 0.007812 0.5] Parametres de rotations
  ;;[0.15 0 0 0.5] EventTick
  ;[0.04591 0.15 0.02398 0.5] L'IA se déplace sur le Spline
  (if (Variables|Default|GetIsRotating)
    (Transformation|AddActorLocalRotation self (Variables|Default|GetDelta%20Rotation) false false)
    (elif (Variables|Default|GetOnTrack?)
      (if (Variables|Default|GetImBack)
        ;;[0.15 0.15 0.15 0.5] Quand elle revient dans le spline, l'ia se remet droite sans tp
        (Transformation|SetActorRotation (Math|Interpolation|RInterpTo (Transformation|GetActorRotation) (Spline|GetRotationatDistanceAlongSpline (Variables|Default|GetSpline) (Variables|Default|GetDistanceAlongSpline) "Local") (Utilities|Time|GetWorldDeltaSeconds) 1.0))
        (Utilities|FlowControl|Delay 1.0)
        (Variables|Default|SetImBack false)
        (else
          (Variables|Default|SetDistanceAlongSpline (+ (* DeltaSeconds (Variables|Default|GetSplineSpeed)) (Variables|Default|GetDistanceAlongSpline)))
          (Transformation|SetActorTransform (Math|Transform|MakeTransform (Math|Vector|MakeVector (.x (.location (Spline|GetTransformatDistanceAlongSpline (Variables|Default|GetSpline) (Variables|Default|GetDistanceAlongSpline) "Local" false))) (.y (.location (Spline|GetTransformatDistanceAlongSpline (Variables|Default|GetSpline) (Variables|Default|GetDistanceAlongSpline) "Local" false))) (+ (.z (.location (Spline|GetTransformatDistanceAlongSpline (Variables|Default|GetSpline) (Variables|Default|GetDistanceAlongSpline) "Local" false))) 9e+01)) (Math|Rotator|MakeRotator (.roll (.rotation (Spline|GetTransformatDistanceAlongSpline (Variables|Default|GetSpline) (Variables|Default|GetDistanceAlongSpline) "Local" false))) (.pitch (.rotation (Spline|GetTransformatDistanceAlongSpline (Variables|Default|GetSpline) (Variables|Default|GetDistanceAlongSpline) "Local" false))) (+ (.yaw (.rotation (Spline|GetTransformatDistanceAlongSpline (Variables|Default|GetSpline) (Variables|Default|GetDistanceAlongSpline) "Local" false))) 0.0))))
          (if (Variables|Default|Getloop?)
            (if (> (Variables|Default|GetDistanceAlongSpline) (Spline|GetSplineLength (Variables|Default|GetSpline)))
              (Variables|Default|SetDistanceAlongSpline 0.0))))))))

(fn ConstructionScript)

(fn CheckinVision
  (if (Variables|Default|GetInVision)
    (return true)
    (else
      (return false))))