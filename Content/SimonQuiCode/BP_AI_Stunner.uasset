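; BP_AI_Stunner is a stunner enemy with a pulsing detection sphere that reacts to movement by the player (Cidara) or the Spectre.
; A randomly offset timeline scales the sphere and triggers a golem sound.
; Overlaps toggle Tick, which spawns a zap effect on the player pawn every frame either target moves inside.
; Chase, return-to-start and color-pulse logic are disconnected, and the contact overlap has no effect.
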(event OnComponentBeginOverlap(CAC)
  (params (OverlappedComponent :type Primitive%20Component%20Object%20Reference) (OtherActor :type Actor%20Object%20Reference) (OtherComp :type Primitive%20Component%20Object%20Reference) (OtherBodyIndex :type Integer) (bFromSweep :type Boolean) (SweepResult :type Hit%20Result%20Structure%20%28by%20ref%29))
  ;[0.15 0.15 0.15 0.5] Si L'IA touche Cidara ou Spectre, il/elle meurt
  (Utilities|FlowControl|Sequence
    (:then_0
      (if (== OtherActor (Variables|Default|GetBP_PlayerRef))
        _))
    (:then_1
      (if (== OtherActor (Variables|Default|GetBP_SpectreRef))
        _))))

(event OnComponentEndOverlap(Spheredetect)
  (params (OverlappedComponent :type Primitive%20Component%20Object%20Reference) (OtherActor :type Actor%20Object%20Reference) (OtherComp :type Primitive%20Component%20Object%20Reference) (OtherBodyIndex :type Integer))
  (bind _bp_spectreref (Variables|Default|GetBP_SpectreRef))
  (bind _bp_playerref (Variables|Default|GetBP_PlayerRef))
  ;[0.15 0.15 0.15 0.5] End overlap, vérifie que c'est bien le joueur ou spectre, si oui stock l'info "inside = false"
  (Utilities|FlowControl|Sequence
    (:then_0
      (if (== OtherActor _bp_playerref)
        (if (!= (Utilities|GetClass _bp_playerref) (Utilities|GetClass self))
          (Variables|Default|SetInside false)
          (Actor|Tick|SetActorTickEnabled false :!label _label))))
    (:then_1
      (if (== OtherActor _bp_spectreref)
        (if (!= (Utilities|GetClass _bp_spectreref) (Utilities|GetClass self))
          (Variables|Default|SetSpectreInside false)
          (goto _label))))))

(event OnComponentBeginOverlap(Spheredetect)
  (params (OverlappedComponent :type Primitive%20Component%20Object%20Reference) (OtherActor :type Actor%20Object%20Reference) (OtherComp :type Primitive%20Component%20Object%20Reference) (OtherBodyIndex :type Integer) (bFromSweep :type Boolean) (SweepResult :type Hit%20Result%20Structure%20%28by%20ref%29))
  (bind _bp_playerref (Variables|Default|GetBP_PlayerRef))
  (bind _bp_spectreref (Variables|Default|GetBP_SpectreRef))
  ;[0.15 0.15 0.15 0.5] Si qlq chose est overlap, vérifie que c'est bien cidara ou spectre, stock l'info "inside = true"et pareil pour "spectre inside"
  (Utilities|FlowControl|Sequence
    (:then_0
      (if (== _bp_playerref OtherActor)
        (Variables|Default|SetInside true)
        (Variables|Default|SetcurrentTarget _bp_playerref)
        (Actor|Tick|SetActorTickEnabled true :!label _label)))
    (:then_1
      (if (== _bp_spectreref OtherActor)
        (Variables|Default|SetSpectreInside true)
        (Variables|Default|SetcurrentTarget _bp_spectreref)
        (goto _label)))))

(event Custom|TriggerElectrocution
  (Niagara|SpawnSystemAttached "/Game/Vefects/Zap_VFX/VFX/Zap/Particles/NS_Zap_02_Blue.NS_Zap_02_Blue" (Variables|/Script/Engine.Actor|GetRootComponent (Game|Player|GetPlayerPawn 0)) "None" "0.000000,0.000000,-85.000000" "0, 0, 0" "KeepRelativeOffset" false))

(event EventTick
  (params (DeltaSeconds :type Float%20%28single-precision%29))
  ;[0.15 0.15 0.15 0.5] Vérifie "le joueur ou spectre sont ils dans le champ de détection ?" puis "est-il en mouvement ?" si oui l'ia fonce sur le joueur.
  (Utilities|FlowControl|Sequence
    (:then_0
      (if (Variables|Default|GetInside)
        (if (> (Math|Vector|VectorLength (Transformation|GetVelocity (Variables|Default|GetBP_PlayerRef))) 1.0)
          (CallFunction|TriggerElectrocution :!label _label))))
    (:then_1
      (if (Variables|Default|GetSpectreInside)
        (if (> (Math|Vector|VectorLength (Transformation|GetVelocity (Variables|Default|GetBP_SpectreRef))) 1.0)
          (goto _label))))))

(event EventBeginPlay
  ;[0.15 0.15 0.15 0.5] 2 cast, stock la loc puis timelinbe de pulse
  (Utilities|FlowControl|Sequence
    (:then_0
      (bind _returnvalue (Actor|GetActorOfClass "/Game/Game/Blueprints/Characters/Cidara/BP_PlayerCidara.BP_PlayerCidara_C"))
      (Variables|Default|SetBP_PlayerRef _returnvalue))
    (:then_1
      (bind _returnvalue_2 (Actor|GetActorOfClass "/Game/Game/Blueprints/Characters/Spectre/BP_Spectre.BP_Spectre_C"))
      (Variables|Default|SetBP_SpectreRef _returnvalue_2))
    (:then_2
      (Variables|Default|Setloc (Transformation|GetActorLocation)))
    (:then_3
      (Components|Timeline|SetPlaybackPosition (Variables|Default|GetTL_Pulse) (Math|Random|RandomFloatinRange 0.0 4.5) false true)
      (bind (_direction _scale _color) (Timeline|TL_Pulse Play)
        (:Update
          (Transformation|SetWorldScale3D (Variables|Default|GetSpheredetect) (Math|Conversions|ToVector(Float) _scale)))
        (:Sfx
          (Audio|PlaySoundatLocation "/Game/SimonQuiCode/golemSFX2.golemSFX2" (Transformation|GetActorLocation self) "0, 0, 0" 1.0 1.0 0.0 "/Game/SimonQuiCode/FinalGolem/SFX/Footstep/SA_Sphere.SA_Sphere" 0 0 0))))
    (:then_4
      (Actor|Tick|SetActorTickEnabled false))
    (:then_5
      (bind _returnvalue_3 (Rendering|Material|CreateDynamicMaterialInstance (Variables|Default|GetSphere) 0 0 "None" :!class /Script/Engine.PrimitiveComponent))
      (Variables|Default|SetMat _returnvalue_3))))

(fn ConstructionScript)