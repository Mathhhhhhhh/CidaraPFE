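; Stunner AI hazard that burns only BP_Spectre, through a pulsing sphere.
; On BeginPlay it tints its material and plays a randomized timeline that scales SphereSpectre and Sphere1 with a golem sound, then disables tick.
; SphereSpectre overlaps and TriggerElectrocution call SpectreBurning on the Spectre; Deactivate destroys both spheres.
; CAC overlap checks for Cidara or Spectre do nothing, and the AIMoveTo chains are unconnected.
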(event OnComponentBeginOverlap(CAC)
  (params (OverlappedComponent :type Primitive%20Component%20Object%20Reference) (OtherActor :type Actor%20Object%20Reference) (OtherComp :type Primitive%20Component%20Object%20Reference) (OtherBodyIndex :type Integer) (bFromSweep :type Boolean) (SweepResult :type Hit%20Result%20Structure%20%28by%20ref%29))
  ;[0.15 0.15 0.15 0.5] Si L'IA touche Cidara ou Spectre, il/elle meurt
  (Utilities|FlowControl|Sequence
    (:then_0
      (if (== OtherActor (Variables|Default|GetBP_PlayerRef))
        _))
    (:then_1
      (if (== OtherActor (Variables|Default|GetBP_SpectreRef))
        _))))

(event OnComponentBeginOverlap(SphereSpectre)
  (params (OverlappedComponent :type Primitive%20Component%20Object%20Reference) (OtherActor :type Actor%20Object%20Reference) (OtherComp :type Primitive%20Component%20Object%20Reference) (OtherBodyIndex :type Integer) (bFromSweep :type Boolean) (SweepResult :type Hit%20Result%20Structure%20%28by%20ref%29))
  (bind _asbp_spectre (Utilities|Casting|CastToBP_Spectre OtherActor))
  (Default|SpectreBurning _asbp_spectre))

(event Custom|TriggerElectrocution
  (params (Target :type Pawn%20Object%20Reference))
  (if (Utilities|IsValid Target)
    (bind _asbp_spectre (Utilities|Casting|CastToBP_Spectre Target))
    (Default|SpectreBurning _asbp_spectre)))

(event Custom|Deactivate
  (Components|DestroyComponent (Variables|Default|GetSphere1))
  (Components|DestroyComponent (Variables|Default|GetSphereSpectre)))

(event EventBeginPlay
  (bind _spherespectre (Variables|Default|GetSphereSpectre))
  (bind _sphere1 (Variables|Default|GetSphere1))
  ;[0.15 0.15 0.15 0.5] 2 cast, stock la loc puis timelinbe de pulse
  (Utilities|FlowControl|Sequence
    (:then_0
      (bind _returnvalue (Actor|GetActorOfClass "/Game/Game/Blueprints/Characters/Cidara/BP_PlayerCidara.BP_PlayerCidara_C"))
      (Variables|Default|SetBP_PlayerRef _returnvalue))
    (:then_1
      (bind _returnvalue_2 (Actor|GetActorOfClass "/Game/Game/Blueprints/Characters/Spectre/BP_Spectre.BP_Spectre_C"))
      (Variables|Default|SetBP_SpectreRef _returnvalue_2))
    (:then_2
      (Variables|Default|Setloc (Transformation|GetActorLocation)))
    (:then_3
      (Components|Timeline|SetPlaybackPosition (Variables|Default|GetTL_Pulse) 0.0 false true)
      (Rendering|Material|SetVectorParameterValue (Variables|Default|GetMat) "Color" "(R=1.000000,G=0.286316,B=0.065224,A=1.000000)" :!class /Script/Engine.MaterialInstanceDynamic)
      (bind _scale (Timeline|TL_Pulse Play)
        (:Update
          (if (Utilities|IsValid _spherespectre)
            (Transformation|SetWorldScale3D _spherespectre (Math|Conversions|ToVector(Float) (Math|Float|Lerp 0.0 (* (Variables|Default|GetSphereScale) 2.0) _scale)))
            (if (Utilities|IsValid _sphere1)
              (Transformation|SetWorldScale3D _sphere1 (Math|Conversions|ToVector(Float) (Math|Float|Lerp 0.0 (* (Variables|Default|GetSphereScale) 1.25) _scale))))))
        (:Sfx
          (Audio|PlaySoundatLocation "/Game/SimonQuiCode/golemSFX2.golemSFX2" (Transformation|GetActorLocation self) "0, 0, 0" 1.0 1.0 0.0 "/Game/SimonQuiCode/FinalGolem/SFX/Footstep/SA_Sphere.SA_Sphere" 0 0 0))))
    (:then_4
      (Actor|Tick|SetActorTickEnabled false))))

(fn ConstructionScript)