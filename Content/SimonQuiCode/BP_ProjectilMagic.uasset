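; BP_ProjectilMagic is an interactable magic projectile pickup that gives BP_PlayerCidara ammunition.
; While still available, an interaction within 300 units hides the actor, increments Munitions and disables further pickup.
; A DoOnce per instance then shows the HUD's aim (Viser) and throw (Jeter) widgets in timed succession.
; That HUD sequence sits outside the distance check, so an out-of-range interaction also triggers it.
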(event EventBeginPlay
  (|CallParentFunction))

(event EventInteract
  (params (Investigator :type Actor%20Object%20Reference))
  (if (Variables|Default|GetCanInteract)
    (bind _asbp_player_cidara (Utilities|Casting|CastToBP_PlayerCidara Investigator))
    (Utilities|FlowControl|Sequence
      (:then_0
        (if (<= (Math|Vector|Distance(Vector) (Transformation|GetActorLocation _asbp_player_cidara) (Transformation|GetActorLocation)) 3e+02)
          (Rendering|SetActorHiddenInGame true)
          (Math|Integer|IncrementInt (Variables|/Game/Game/Blueprints/Characters/Cidara/BP_PlayerCidara.BP_PlayerCidara_C|GetMunitions _asbp_player_cidara)
            (:%20%20
              (Variables|Default|SetCanInteract false)))))
      (:then_1
        (Utilities|FlowControl|DoOnce false
          (:Completed
            (Widget|SetVisibility (Variables|/Game/Game/Blueprints/Widget/WBP_HUD.WBP_HUD_C|GetSW_Viser (Variables|/Game/Game/Blueprints/Characters/Cidara/BP_PlayerCidara.BP_PlayerCidara_C|GetWBP_HUD _asbp_player_cidara)) "Visible")
            (Utilities|FlowControl|Delay 4.0)
            (Widget|SetVisibility (Variables|/Game/Game/Blueprints/Widget/WBP_HUD.WBP_HUD_C|GetSW_Viser (Variables|/Game/Game/Blueprints/Characters/Cidara/BP_PlayerCidara.BP_PlayerCidara_C|GetWBP_HUD _asbp_player_cidara)) "Collapsed")
            (Utilities|FlowControl|Delay 1.0)
            (Widget|SetVisibility (Variables|/Game/Game/Blueprints/Widget/WBP_HUD.WBP_HUD_C|GetSW_Jeter (Variables|/Game/Game/Blueprints/Characters/Cidara/BP_PlayerCidara.BP_PlayerCidara_C|GetWBP_HUD _asbp_player_cidara)) "Visible")
            (Utilities|FlowControl|Delay 4.0)
            (Widget|SetVisibility (Variables|/Game/Game/Blueprints/Widget/WBP_HUD.WBP_HUD_C|GetSW_Jeter (Variables|/Game/Game/Blueprints/Characters/Cidara/BP_PlayerCidara.BP_PlayerCidara_C|GetWBP_HUD _asbp_player_cidara)) "Hidden")))))))

(fn ConstructionScript
  (|CallParentFunction))